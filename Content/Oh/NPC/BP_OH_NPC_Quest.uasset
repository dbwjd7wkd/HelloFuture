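; Quest-giver NPC Blueprint that offers quests to the player on interaction.
; Interact checks that quests exist and the first can be accepted, then calls AskForQuest on the player's Oh_HelloFutureCharacter with itself.
; BeginPlay and EndPlay are empty; disconnected logic would link quest names and steps to their triggers and load or save NPC quests through the game instance's quest save.
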(event `self.ReceiveBeginPlay`)

(event `self.ReceiveEndPlay`
  (params (EndPlayReason :type "EEndPlayReason Enum" :default "Destroyed")))

(event `/Game/Oh/NPC/BP_OH_NPC_Interface.Interact`
  (bind _quests_quests (break `/Game/Oh/Quest/Oh_NPC_Quest_Holder` (`self.Quests`)))
  (bind _quests_quests_2 (break `/Game/Oh/Quest/Oh_NPC_Quest_Holder` (`self.Quests`)))
  (bind (_output_name _output_description _output_queststeps _output_primary _output_canbeaccepted) (break `/Game/Oh/Quest/OH_NPC_Quest` (`|GetArrayItem` _quests_quests)))
  (if (`KismetMathLibrary.Conv_IntToBool` (`KismetArrayLibrary.Array_Length` _quests_quests_2))
    (if _output_canbeaccepted
      (bind _asoh_hello_future_character (cast `/Game/Oh/Player/Oh_HelloFutureCharacter` (`GameplayStatics.GetPlayerCharacter` 0)))
      (`/Game/Oh/Player/Oh_HelloFutureCharacter.Ask For Quest` _asoh_hello_future_character self))))

(fn `UserConstructionScript`
  (`parent.UserConstructionScript`))