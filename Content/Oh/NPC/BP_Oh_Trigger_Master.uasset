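; BP_Oh_Trigger_Master is a quest trigger actor, named as a master class, that can complete a step of the player's active quest.
; On BeginPlay it caches the player character's OHQuestComponent.
; FinishStep completes the step and returns true only if the active quest matches QuestName and its first step's Trigger is this actor.
; Overlap and Tick are empty, and nothing here calls FinishStep.
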(event `self.ReceiveBeginPlay`
  (bind _asoh_hello_future_character (cast `/Game/Oh/Player/Oh_HelloFutureCharacter` (`GameplayStatics.GetPlayerCharacter` 0)))
  (set `self.Quest Ref` (`/Game/Oh/Player/Oh_HelloFutureCharacter.OH_Quest_Component` _asoh_hello_future_character)))

(fn `Finish Step`
  (returns (Return :type Boolean))
  (bind (_active_quest_name _active_quest_description _active_quest_queststeps) (break `/Game/Oh/Quest/Oh_Quest_Struct` (`/Game/Oh/Quest/OH_Quest_Component.Active Quest` (`self.Quest Ref`))))
  (bind (_output_description _output_trigger) (break `/Game/Oh/Quest/OH_Quest_Step` (`|GetArrayItem` _active_quest_queststeps)))
  (if (`KismetMathLibrary.Conv_IntToBool` (`KismetArrayLibrary.Array_Length` _active_quest_queststeps))
    (if (and (`KismetStringLibrary.EqualEqual_StrStr` _active_quest_name (`self.Quest Name`)) (== _output_trigger self))
      (`/Game/Oh/Quest/OH_Quest_Component.Complete Step` (`self.Quest Ref`))
      (return true)
      (else
        (return false)))))

(fn `UserConstructionScript`)