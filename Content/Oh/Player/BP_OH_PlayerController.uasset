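; Player controller Blueprint for the OH player, holding a leftover hook into the OhQuestUI dialogue system.
; A custom event prints a debug string when the current dialogue is the intro dialogue.
; The code that would bind it to dialogue completion, gated by a StartPlay flag on the game instance, is disconnected, and Tick is empty.
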(event `self.ReceiveTick`
  (params (DeltaSeconds :type "Float (single-precision)")))

(event `CustomEvent_0`
  (if (`KismetStringLibrary.EqualEqual_StrStr` (`KismetSystemLibrary.GetDisplayName` (`OH_QuestUI.curDialog` (`self.oh_QuestUI`))) "IntroDialogue")
    (`KismetSystemLibrary.PrintString` "2")))

(fn `UserConstructionScript`)