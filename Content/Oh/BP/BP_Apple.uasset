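; BP_Apple is an apple shop item that shows its price and opens a purchase widget when clicked.
; Entering or leaving the collision component shows or hides the Price component.
; Clicking any of five body components toggles the BP_purchase widget created at BeginPlay.
; Opening shows the cursor and sets UI-only input; closing only removes the widget and clears the flag, without restoring input mode or cursor.
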(event `self.ReceiveBeginPlay`
  (`SceneComponent.SetVisibility` (`self.Price`) false false)
  (bind _returnvalue (`|CreateWidget` "/Game/Oh/BP/BP_purchase.BP_purchase_C"))
  (set `self.Purchase UI` _returnvalue))

(event `self.collision.OnComponentBeginOverlap`
  (params (OverlappedComponent :type "PrimitiveComponent Object Reference") (OtherActor :type "Actor Object Reference") (OtherComp :type "PrimitiveComponent Object Reference") (OtherBodyIndex :type Integer) (bFromSweep :type Boolean) (SweepResult :type "HitResult Structure (by ref)"))
  (`SceneComponent.SetVisibility` (`self.Price`) true false))

(event `self.collision.OnComponentEndOverlap`
  (params (OverlappedComponent :type "PrimitiveComponent Object Reference") (OtherActor :type "Actor Object Reference") (OtherComp :type "PrimitiveComponent Object Reference") (OtherBodyIndex :type Integer))
  (`SceneComponent.SetVisibility` (`self.Price`) false false))

(event `self.body.OnClicked`
  (params (TouchedComponent :type "PrimitiveComponent Object Reference") (ButtonPressed :type "Key Structure"))
  (bind _returnvalue (`GameplayStatics.GetPlayerController` 0))
  (if (== (`self.is Show UI`) false) :!label _label
    (set `PlayerController.bShowMouseCursor` true _returnvalue)
    (`WidgetBlueprintLibrary.SetInputMode_UIOnlyEx` _returnvalue null)
    (`UserWidget.AddToViewport` (`self.Purchase UI`) 0)
    (set `self.is Show UI` true)
    (else
      (`Widget.RemoveFromParent` (`self.Purchase UI`))
      (set `self.is Show UI` false))))

(event `self.Bpdy2.OnClicked`
  (params (TouchedComponent :type "PrimitiveComponent Object Reference") (ButtonPressed :type "Key Structure"))
  (goto _label))

(event `self.Bpdy3.OnClicked`
  (params (TouchedComponent :type "PrimitiveComponent Object Reference") (ButtonPressed :type "Key Structure"))
  (goto _label))

(event `self.Bpdy4.OnClicked`
  (params (TouchedComponent :type "PrimitiveComponent Object Reference") (ButtonPressed :type "Key Structure"))
  (goto _label))

(event `self.Bpdy1.OnClicked`
  (params (TouchedComponent :type "PrimitiveComponent Object Reference") (ButtonPressed :type "Key Structure"))
  (goto _label))

(fn `UserConstructionScript`)