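; Shop pickup actor for daikon radish that shows a purchase UI while something overlaps its collision.
; On BeginPlay it creates a WBP_purchase widget and fills in the fruit name and price.
; Overlap start adds the widget, switches to game-and-UI input and constructs a BP_Daikon, outered to the player pawn, as the widget's inventory item.
; Overlap end removes the widget without restoring input mode; neither event checks the overlapping actor.
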(event `self.ReceiveBeginPlay`
  (bind _returnvalue (`|CreateWidget` "/Game/Oh/BP/WBP_purchase.WBP_purchase_C"))
  (set `self.Purchase UI` _returnvalue)
  ;[1 1 1] UI에 값 넘겨주기
  (set `/Game/Oh/BP/WBP_purchase.FruitName` "무" (`self.Purchase UI`))
  (set `/Game/Oh/BP/WBP_purchase.FruitPrice` 1250 (`self.Purchase UI`)))

(event `self.collision.OnComponentBeginOverlap`
  (params (OverlappedComponent :type "PrimitiveComponent Object Reference") (OtherActor :type "Actor Object Reference") (OtherComp :type "PrimitiveComponent Object Reference") (OtherBodyIndex :type Integer) (bFromSweep :type Boolean) (SweepResult :type "HitResult Structure (by ref)"))
  (if (== (`self.is Show UI`) false)
    (`WidgetBlueprintLibrary.SetInputMode_GameAndUIEx` (`GameplayStatics.GetPlayerController` 0) null)
    (`UserWidget.AddToViewport` (`self.Purchase UI`) 0)
    (set `self.is Show UI` true)
    ;[1 1 1] 현재 아이템 종류 인벤토리에 넣기
    (bind _returnvalue (`|GenericCreateObject` "/Game/YJ/Blueprints/Inventory/BP_Daikon.BP_Daikon_C" (`GameplayStatics.GetPlayerPawn` 0)))
    (set `/Game/Oh/BP/WBP_purchase.InventoryItem` _returnvalue (`self.Purchase UI`))))

(event `self.collision.OnComponentEndOverlap`
  (params (OverlappedComponent :type "PrimitiveComponent Object Reference") (OtherActor :type "Actor Object Reference") (OtherComp :type "PrimitiveComponent Object Reference") (OtherBodyIndex :type Integer))
  (`Widget.RemoveFromParent` (`self.Purchase UI`))
  (set `self.is Show UI` false))

(fn `UserConstructionScript`)