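; Interactive dialogue Blueprint that reacts when the farm selling dialogue completes in the quest UI.
; Tick casts to OH_PlayerController and binds a handler to OhQuestUI's OnDialogueCompleted every frame.
; When the current dialogue is FarmSellDialogue, the handler shows the cursor and sets Game and UI input focused on SellingInventoryUI.
; The nodes that create that selling widget and destroy the actor are disconnected and never run.
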(event `self.ReceiveTick`
  (params (DeltaSeconds :type "Float (single-precision)"))
  (bind _asoh_player_controller (cast `OH_PlayerController` (`GameplayStatics.GetPlayerController` 0)))
  (add `OH_QuestUI.OnDialogueCompleted` (`OH_PlayerController.oh_QuestUI` _asoh_player_controller) (delegate `CustomEvent_0`)))

(event `CustomEvent_0`
  (bind _returnvalue (`GameplayStatics.GetPlayerController` 0))
  (if (`KismetStringLibrary.EqualEqual_StrStr` (`KismetSystemLibrary.GetDisplayName` (`OH_QuestUI.curDialog` (`OH_PlayerController.oh_QuestUI` (stale `self.ReceiveTick` _asoh_player_controller)))) "FarmSellDialogue")
    (set `PlayerController.bShowMouseCursor` true _returnvalue)
    (`WidgetBlueprintLibrary.SetInputMode_GameAndUIEx` _returnvalue (`self.SellingInventoryUI`))))

(fn `UserConstructionScript`)