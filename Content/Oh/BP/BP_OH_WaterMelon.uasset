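; BP_OH_WaterMelon is a watermelon shop actor that shows a purchase widget when something overlaps its collision.
; BeginPlay creates WBP_purchase and fills in the fruit's name and price.
; Overlap begin switches input to Game and UI and adds the widget to the viewport; overlap end removes it.
; Logic that sets IsShowUI true and assigns a BP_WaterMelon as the widget's inventory item is disconnected and never runs.
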(event `self.ReceiveBeginPlay`
  (bind _returnvalue (`|CreateWidget` "/Game/Oh/BP/WBP_purchase.WBP_purchase_C"))
  (set `self.PurchaseUI_0` _returnvalue)
  ;[1 1 1] UI에 값 넘겨주기
  (set `/Game/Oh/BP/WBP_purchase.FruitName` "수박" (`self.PurchaseUI_0`))
  (set `/Game/Oh/BP/WBP_purchase.FruitPrice` 1000 (`self.PurchaseUI_0`)))

(event `self.collision.OnComponentBeginOverlap`
  (params (OverlappedComponent :type "PrimitiveComponent Object Reference") (OtherActor :type "Actor Object Reference") (OtherComp :type "PrimitiveComponent Object Reference") (OtherBodyIndex :type Integer) (bFromSweep :type Boolean) (SweepResult :type "HitResult Structure (by ref)"))
  (if (== (`self.is Show UI`) false)
    (`WidgetBlueprintLibrary.SetInputMode_GameAndUIEx` (`GameplayStatics.GetPlayerController` 0) null)
    (`UserWidget.AddToViewport` (`self.PurchaseUI_0`) 0)))

(event `self.collision.OnComponentEndOverlap`
  (params (OverlappedComponent :type "PrimitiveComponent Object Reference") (OtherActor :type "Actor Object Reference") (OtherComp :type "PrimitiveComponent Object Reference") (OtherBodyIndex :type Integer))
  (`Widget.RemoveFromParent` (`self.PurchaseUI_0`))
  (set `self.is Show UI` false))

(fn `UserConstructionScript`)