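; Interactive dialogue actor that offers or turns in a quest when its InteractQuest flag is raised.
; Tick polls and clears the flag, then, if the player's "2" flag is set, checks the owner of InteractMessage's attach parent for interaction.
; A returned quest shows turn-in if already in the QuestLog, otherwise the quest display.
; Both quest and plain-interact results call Interact2Message on that owner; debug prints remain.
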(event `self.ReceiveTick`
  (params (DeltaSeconds :type "Float (single-precision)"))
  (if (== (`self.interactQuest`) true)
    (set `self.interactQuest` false)
    (`KismetSystemLibrary.PrintString` "Hello")
    (bind _asyj_hello_future_character (cast `/Game/Map/YJ_HelloFutureCharacter` (`GameplayStatics.GetPlayerCharacter` 0)))
    (if (== (`/Game/Map/YJ_HelloFutureCharacter.2` _asyj_hello_future_character) true)
      (`KismetSystemLibrary.PrintString` "22")
      (bind _asyj_hello_future_character_2 (cast `/Game/Map/YJ_HelloFutureCharacter` (`GameplayStatics.GetPlayerCharacter` 0)))
      (bind _returnvalue (`ActorComponent.GetOwner` (`SceneComponent.GetAttachParent` (`/Game/Map/YJ_HelloFutureCharacter.InteractMessage` _asyj_hello_future_character_2))))
      (bind _quest (`/Game/Oh/RealQuest/QuestMacro.CheakForInteraction` _returnvalue)
        (:`True`
          (if (`KismetArrayLibrary.Array_Contains` (`/Game/Oh/RealQuest/QuestLog.Quests` (`/Game/Map/YJ_HelloFutureCharacter.QuestLog` (cast `/Game/Map/YJ_HelloFutureCharacter` (`GameplayStatics.GetPlayerCharacter` 0) :!pure true))) _quest)
            (`/Game/Oh/RealQuest/QuestMacro.DisplayTurnIn` _quest
              (:`out`
                _))
            (else
              (`/Game/Oh/RealQuest/QuestMacro.DisplayQuest` _quest
                (:`Out`
                  _)))))
        (:`Interact`
          _))
      (message `/Game/Oh/RealQuest/InteractInterface.Interact2` _returnvalue))))

(fn `UserConstructionScript`)