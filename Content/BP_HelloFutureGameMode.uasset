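; Game mode that sets up the HUD and picks player spawn points by portal name.
; BeginPlay creates the HUD widget for player controller 0, adds it to the viewport and stores its canvas.
; ChoosePlayerStart returns the PlayerStart whose tag matches PotalName in realCharGameInstance, falling back to the first one found.
; The HUD rep-notifies are empty, and an authority check is left unconnected.
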(event `self.ReceiveBeginPlay`
  (bind _returnvalue (`|CreateWidget` "/Game/Oh/RealQuest/QuestUI/HUD_UI.HUD_UI_C" (`GameplayStatics.GetPlayerController` 0)))
  (bind _output_get (set `self.HUD_Widget` _returnvalue))
  (`UserWidget.AddToViewport` _output_get 0)
  (set `self.HUD Canvas` (`/Game/Oh/RealQuest/QuestUI/HUD_UI.HUD_Canvas` _output_get)))

(fn `ChoosePlayerStart`
  (params (Player :type "Controller Object Reference"))
  (returns (ReturnValue :type "Actor Object Reference"))
  (bind _asreal_char_game_instance (cast `/Game/Map/realCharGameInstance` (`GameplayStatics.GetGameInstance`)))
  (bind _outactors (`GameplayStatics.GetAllActorsOfClass` "/Script/Engine.PlayerStart"))
  (for _array_element _outactors
    (if (== (`PlayerStart.PlayerStartTag` _array_element) (`/Game/Map/realCharGameInstance.Potal Name` _asreal_char_game_instance))
      (return _array_element)))
  (return (`|GetArrayItem` _outactors)))

(fn `OnRep_HUD Canvas`)

(fn `OnRep_HUD_Widget`)

(fn `UserConstructionScript`)