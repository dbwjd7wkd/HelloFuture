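; BP_Apple is a farm pickup that adds an Apple to the inventory of an overlapping HelloFutureCharacter.
; Its Seed component stops simulating physics one second after BeginPlay.
; A Box overlap plays the fruit-picking montage, waits a second, plays a sound, adds the item and destroys the actor.
; It then casts player 0 to YJ_HelloFutureCharacter and reports the collected Apple to every quest in its QuestLog.
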(event `self.ReceiveBeginPlay`
  (`KismetSystemLibrary.Delay` 1.0)
  (`PrimitiveComponent.SetSimulatePhysics` (`self.Seed`) false))

(event `self.Box.OnComponentBeginOverlap`
  (params (OverlappedComponent :type "PrimitiveComponent Object Reference") (OtherActor :type "Actor Object Reference") (OtherComp :type "PrimitiveComponent Object Reference") (OtherBodyIndex :type Integer) (bFromSweep :type Boolean) (SweepResult :type "HitResult Structure (by ref)"))
  (bind _ashello_future_character (cast `HelloFutureCharacter` OtherActor))
  (`Character.PlayAnimMontage` _ashello_future_character "/Game/Map/Animation/Pick_Fruit_Montage.Pick_Fruit_Montage" 1.0 "None")
  (`KismetSystemLibrary.Delay` 1.0)
  (`GameplayStatics.PlaySound2D` "/Game/NewAssets/Game_UI_Bundle/Cartoon_Funny_Item_UI/Cue/Item/Item_UI_014_Cue.Item_UI_014_Cue" 1.0 1.0 0.0 null null)
  ;[1 1 1] CornItem 아이템 추가
  (`YJ_InventoryComponent.AddItem2` (`HelloFutureCharacter.Inventory` _ashello_future_character) "Apple")
  (`self.K2_DestroyActor`)
  (bind _asyj_hello_future_character (cast `/Game/Map/YJ_HelloFutureCharacter` (`GameplayStatics.GetPlayerCharacter` 0)))
  (for _array_element (`/Game/Oh/RealQuest/QuestLog.Quests` (`/Game/Map/YJ_HelloFutureCharacter.QuestLog` _asyj_hello_future_character))
    (`/Game/Oh/RealQuest/Quests/OH_RealQuest.CollectedItem` _array_element "Apple")))

(fn `UserConstructionScript`)