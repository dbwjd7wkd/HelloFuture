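; Farm tree actor that spawns fruit when the player holds the Shake input nearby.
; Box overlap by HelloFutureCharacter toggles actor input and a gate, and shows or removes a WBP_Hold widget.
; A press starts a retriggerable delay of MaxHoldTime, then spawns fruit and removes the widget if still held.
; A parallel timer, polled by a self-calling delayed event, feeds elapsed hold time to the widget until release.
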(event `InputAction|Shake`
  (params (Key :type "Key Structure"))
  (:`Pressed`
    (set `self.Is Held?` true)
    (`/Engine/EditorBlueprintResources/StandardMacros.Gate` true :!label _label
      (:`Exit`
        (`|ExecutionSequence`
          (:`then_0`
            (`KismetSystemLibrary.RetriggerableDelay` (`self.MaxHoldTime`))
            (if (`self.Is Held?`)
              (`self.SpawnFruit`)
              (`Widget.RemoveFromParent` (stale `self.Box.OnComponentBeginOverlap` _output_get))))
          (:`then_1`
            (`self.Timer`)
            (`self.Update Timer`))))))
  (:`Released`
    (set `self.Is Held?` false)))

(event `self.Box.OnComponentBeginOverlap`
  (params (OverlappedComponent :type "PrimitiveComponent Object Reference") (OtherActor :type "Actor Object Reference") (OtherComp :type "PrimitiveComponent Object Reference") (OtherBodyIndex :type Integer) (bFromSweep :type Boolean) (SweepResult :type "HitResult Structure (by ref)"))
  (cast `HelloFutureCharacter` OtherActor)
  (`self.EnableInput` (`GameplayStatics.GetPlayerController` 0))
  (bind _returnvalue (`|CreateWidget` "/Game/Minsu/Farm/BP/WBP_Hold.WBP_Hold_C"))
  (bind _output_get (set `self.Hold Widget` _returnvalue))
  (`UserWidget.AddToViewport` _output_get 0)
  (set `/Game/Minsu/Farm/BP/WBP_Hold.MaxTimeHeld` (`self.MaxHoldTime`) _output_get)
  (goto _label :!via `Open`))

(event `Stop Timer`
  (`KismetSystemLibrary.K2_PauseTimerHandle` (stale `Timer` _returnvalue)))

(event `self.Box.OnComponentEndOverlap`
  (params (OverlappedComponent :type "PrimitiveComponent Object Reference") (OtherActor :type "Actor Object Reference") (OtherComp :type "PrimitiveComponent Object Reference") (OtherBodyIndex :type Integer))
  (cast `HelloFutureCharacter` OtherActor)
  (`self.DisableInput` (`GameplayStatics.GetPlayerController` 0))
  (`Widget.RemoveFromParent` (stale `self.Box.OnComponentBeginOverlap` _returnvalue))
  (goto _label :!via `Close`))

(event `Timer`
  (bind _returnvalue (`KismetSystemLibrary.K2_SetTimerDelegate` (delegate `Timer`) (`self.MaxHoldTime`))))

(event `Update Timer`
  (bind _hold_widget (`self.Hold Widget`))
  (if (`self.Is Held?`)
    (set `/Game/Minsu/Farm/BP/WBP_Hold.TimeHeld` (`KismetSystemLibrary.K2_GetTimerElapsedTimeHandle` (stale `Timer` _returnvalue)) _hold_widget)
    (`KismetSystemLibrary.Delay` 0.1)
    (`self.Update Timer`)
    (else
      (`self.Stop Timer`)
      (set `/Game/Minsu/Farm/BP/WBP_Hold.TimeHeld` 0.0 _hold_widget))))

(fn `UserConstructionScript`)