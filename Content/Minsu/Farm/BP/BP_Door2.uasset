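; Door actor that shows a NewWBP_Door2 UI widget when the HelloFutureCharacter enters either of its two sphere triggers.
; Each sphere creates its own widget with a reference to this door, then switches to Game and UI input with the mouse cursor shown.
; Leaving a sphere removes its widget and restores game-only input, but does not reset the cursor flag.
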(event `self.Sphere.OnComponentBeginOverlap`
  (params (OverlappedComponent :type "PrimitiveComponent Object Reference") (OtherActor :type "Actor Object Reference") (OtherComp :type "PrimitiveComponent Object Reference") (OtherBodyIndex :type Integer) (bFromSweep :type Boolean) (SweepResult :type "HitResult Structure (by ref)"))
  (bind _returnvalue (`GameplayStatics.GetPlayerController` 0))
  (cast `HelloFutureCharacter` OtherActor)
  (bind _returnvalue_2 (`|CreateWidget` "/Game/Minsu/NewWBP_Door2.NewWBP_Door2_C" null self))
  (`UserWidget.AddToViewport` _returnvalue_2 0)
  (`UserWidget.SetDesiredSizeInViewport` _returnvalue_2 (0.0 0.0))
  (`WidgetBlueprintLibrary.SetInputMode_GameAndUIEx` _returnvalue _returnvalue_2)
  (set `PlayerController.bShowMouseCursor` true _returnvalue))

(event `self.Sphere.OnComponentEndOverlap`
  (params (OverlappedComponent :type "PrimitiveComponent Object Reference") (OtherActor :type "Actor Object Reference") (OtherComp :type "PrimitiveComponent Object Reference") (OtherBodyIndex :type Integer))
  (cast `HelloFutureCharacter` OtherActor)
  (`Widget.RemoveFromParent` (stale `self.Sphere.OnComponentBeginOverlap` _returnvalue_2))
  (`WidgetBlueprintLibrary.SetInputMode_GameOnly` (`GameplayStatics.GetPlayerController` 0)))

(event `self.Sphere1.OnComponentBeginOverlap`
  (params (OverlappedComponent :type "PrimitiveComponent Object Reference") (OtherActor :type "Actor Object Reference") (OtherComp :type "PrimitiveComponent Object Reference") (OtherBodyIndex :type Integer) (bFromSweep :type Boolean) (SweepResult :type "HitResult Structure (by ref)"))
  (bind _returnvalue (`GameplayStatics.GetPlayerController` 0))
  (cast `HelloFutureCharacter` OtherActor)
  (bind _returnvalue_2 (`|CreateWidget` "/Game/Minsu/NewWBP_Door2.NewWBP_Door2_C" null self))
  (`UserWidget.AddToViewport` _returnvalue_2 0)
  (`UserWidget.SetDesiredSizeInViewport` _returnvalue_2 (0.0 0.0))
  (`WidgetBlueprintLibrary.SetInputMode_GameAndUIEx` _returnvalue null)
  (set `PlayerController.bShowMouseCursor` true _returnvalue))

(event `self.Sphere1.OnComponentEndOverlap`
  (params (OverlappedComponent :type "PrimitiveComponent Object Reference") (OtherActor :type "Actor Object Reference") (OtherComp :type "PrimitiveComponent Object Reference") (OtherBodyIndex :type Integer))
  (cast `HelloFutureCharacter` OtherActor)
  (`Widget.RemoveFromParent` (stale `self.Sphere1.OnComponentBeginOverlap` _returnvalue_2))
  (`WidgetBlueprintLibrary.SetInputMode_GameOnly` (`GameplayStatics.GetPlayerController` 0)))

(fn `UserConstructionScript`)