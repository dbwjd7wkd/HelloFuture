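; Farm tile actor that grows wheat, corn or pumpkin from the player's selected seed and spawns loose produce on harvest.
; BPIPlantSeed consumes a seed from the player's inventory, then swaps static mesh components through three growth stages, timed by a Text3D countdown.
; Corn and pumpkin risk disease at each stage, which halts growth with a disease material and yields no produce.
; BPIActivate harvests finished or diseased crops, freeing the tile.
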(event `self.ReceiveBeginPlay`
  (`Text3DComponent.SetText` (`self.Text3D`) (`self.Value`)))

(event `Plant Wheat`
  (bind _returnvalue (`AddComponent|NODE_AddStaticMeshComponent-0` :`RelativeTransform` (`KismetMathLibrary.MakeTransform` (`self.Relative Transfrom Location`))))
  (`self.GrowTime` (`self.WheatGrowTime`)
    (:`Out`
      (`ActorComponent.K2_DestroyComponent` _returnvalue)
      (bind _returnvalue_2 (`AddComponent|NODE_AddStaticMeshComponent-1` :`RelativeTransform` (`KismetMathLibrary.MakeTransform` (`self.Relative Transfrom Location`))))
      (`self.GrowTime` (`self.WheatGrowTime`)
        (:`Out`
          (`ActorComponent.K2_DestroyComponent` _returnvalue_2)
          (bind _returnvalue_3 (`AddComponent|NODE_AddStaticMeshComponent-2` :`RelativeTransform` (`KismetMathLibrary.MakeTransform` (`self.Relative Transfrom Location`))))
          (set `self.FullyGrown?` true)
          (set `self.CurrentMesh` _returnvalue_3)
          (set `self.WhatCanBeHarvested` "Wheat"))))))

(event `/Game/Minsu/Farm/BPI_PlantSeed.BPI_PlantSeed`
  (if (not (`self.IsSomethingPlanted?`))
    (bind _asyj_hello_future_character (cast `/Game/YJ/Blueprints/YJ_HelloFutureCharacter` (`GameplayStatics.GetPlayerCharacter` 0)))
    (switch `int` (`/Game/YJ/Blueprints/YJ_HelloFutureCharacter.Seed` _asyj_hello_future_character)
      (:`0`
        (`self.DoWeHaveWheatSeed`
          (:`Output`
            (`self.Plant Wheat`))))
      (:`1`
        (`self.DoWeHaveCornSeed`
          (:`Output`
            (`self.Plant Corn`))))
      (:`2`
        (`self.DoWeHavePumpkinSeed`
          (:`Output`
            (`self.Plant Pumpkin`)))))
    (set `self.IsSomethingPlanted?` true)))

(event `/Game/Minsu/Farm/BPI_Activate.BPI_Activate`
  (`self.Harvest`))

(event `Plant Corn`
  (bind _returnvalue (`AddComponent|NODE_AddStaticMeshComponent-3` :`RelativeTransform` (`KismetMathLibrary.MakeTransform` (`self.Relative Transfrom Location`))))
  (`self.GrowTime` (`self.CornGrowTime`)
    (:`Out`
      (`self.ChanceOfDisease` _returnvalue
        (:`NoDisease`
          (`ActorComponent.K2_DestroyComponent` _returnvalue)
          (bind _returnvalue_2 (`AddComponent|NODE_AddStaticMeshComponent-4`))
          (`self.GrowTime` (`self.CornGrowTime`)
            (:`Out`
              (`self.ChanceOfDisease` _returnvalue_2
                (:`NoDisease`
                  (`ActorComponent.K2_DestroyComponent` _returnvalue_2)
                  (bind _returnvalue_3 (`AddComponent|NODE_AddStaticMeshComponent-5`))
                  (`self.ChanceOfDisease` _returnvalue_3
                    (:`NoDisease`
                      (set `self.FullyGrown?` true)
                      (set `self.CurrentMesh` _returnvalue_3)
                      (set `self.WhatCanBeHarvested` "Corn"))))))))))))

(event `Plant Pumpkin`
  (bind _returnvalue (`AddComponent|NODE_AddStaticMeshComponent-6` :`RelativeTransform` (`KismetMathLibrary.MakeTransform` (`self.Relative Transfrom Location`))))
  (`self.GrowTime` (`self.PumpkinGrowTime`)
    (:`Out`
      (`self.ChanceOfDisease` _returnvalue
        (:`NoDisease`
          (`ActorComponent.K2_DestroyComponent` _returnvalue)
          (bind _returnvalue_2 (`AddComponent|NODE_AddStaticMeshComponent-7`))
          (`self.GrowTime` (`self.PumpkinGrowTime`)
            (:`Out`
              (`self.ChanceOfDisease` _returnvalue_2
                (:`NoDisease`
                  (`ActorComponent.K2_DestroyComponent` _returnvalue_2)
                  (bind _returnvalue_3 (`AddComponent|NODE_AddStaticMeshComponent-8`))
                  (`self.ChanceOfDisease` _returnvalue_3
                    (:`NoDisease`
                      (set `self.FullyGrown?` true)
                      (set `self.CurrentMesh` _returnvalue_3)
                      (set `self.WhatCanBeHarvested` "Pumpkin"))))))))))))

(fn `Harvest`
  (bind _returnvalue (`KismetMathLibrary.Conv_VectorToTransform` (`SceneComponent.K2_GetComponentLocation` (`self.Text3D`))))
  (if (`self.FullyGrown?`)
    (`ActorComponent.K2_DestroyComponent` (`self.CurrentMesh`))
    (switch `string` (`self.WhatCanBeHarvested`)
      (:`Default`
        _)
      (:`Wheat`
        (`|SpawnActorFromClass` "/Game/Minsu/Farm/BP/BP_WheatLoose.BP_WheatLoose_C" _returnvalue "Undefined" "OverrideRootScale" null null))
      (:`Corn`
        (`|SpawnActorFromClass` "/Game/Minsu/Farm/BP/BP_CornLoose.BP_CornLoose_C" _returnvalue "Undefined" "OverrideRootScale" null null))
      (:`Pumpkin`
        (`|SpawnActorFromClass` "/Game/Minsu/Farm/BP/BP_PumpkinLoose.BP_PumpkinLoose_C" _returnvalue "Undefined" "OverrideRootScale" null null)))
    (set `self.FullyGrown?` false)
    (set `self.CurrentMesh` null)
    (set `self.IsSomethingPlanted?` false)
    (set `self.WhatCanBeHarvested` "")))

(fn `UserConstructionScript`)