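; BP_CornSeed is a pickup actor that gives the player a corn seed when touched.
; When its Box is overlapped by a YJ_HelloFutureCharacter, it increments that character's corn seed count.
; It then adds the corn seed entry from the game instance's AllItems list, looked up by fixed index, to the character's inventory and destroys itself.
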(event `self.Box.OnComponentBeginOverlap`
  (params (OverlappedComponent :type "PrimitiveComponent Object Reference") (OtherActor :type "Actor Object Reference") (OtherComp :type "PrimitiveComponent Object Reference") (OtherBodyIndex :type Integer) (bFromSweep :type Boolean) (SweepResult :type "HitResult Structure (by ref)"))
  (bind _asyj_hello_future_character (cast `/Game/YJ/Blueprints/YJ_HelloFutureCharacter` OtherActor))
  (bind _result (`/Engine/EditorBlueprintResources/StandardMacros.IncrementInt` (`/Game/YJ/Blueprints/YJ_HelloFutureCharacter.AmountOfCornSeed` _asyj_hello_future_character))
    (:`  `
      (set `/Game/YJ/Blueprints/YJ_HelloFutureCharacter.AmountOfCornSeed` _result _asyj_hello_future_character)
      ;[1 1 1] CornSeedItem 아이템 추가
      (`YJ_InventoryComponent.AddItem` (`HelloFutureCharacter.Inventory` _asyj_hello_future_character) (`|GetArrayItem` (`YJ_GameInstance.AllItems` (cast `YJ_GameInstance` (`GameplayStatics.GetGameInstance`) :!pure true)) 4))
      (`self.K2_DestroyActor`))))

(fn `UserConstructionScript`)