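; BP_Gem is a collectible gem pickup in the farm content that feeds the player's inventory and quest progress.
; After BeginPlay, a short delay lets its Seed component settle before physics simulation is switched off.
; On box overlap, an overlapping YJ_HelloFutureCharacter runs the reused apple-grab server call and montage, then receives a Gem item.
; Separately, any overlap reports a collected Gem to every quest in player 0's quest log.
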(event `self.ReceiveBeginPlay`
  (`KismetSystemLibrary.Delay` 1.5)
  (`PrimitiveComponent.SetSimulatePhysics` (`self.Seed`) false))

(event `self.Box.OnComponentBeginOverlap`
  (params (OverlappedComponent :type "PrimitiveComponent Object Reference") (OtherActor :type "Actor Object Reference") (OtherComp :type "PrimitiveComponent Object Reference") (OtherBodyIndex :type Integer) (bFromSweep :type Boolean) (SweepResult :type "HitResult Structure (by ref)"))
  (`|ExecutionSequence`
    (:`then_0`
      ;[1 1 1] 사과 줍기 애니메이션 및 사운드
      (bind _asyj_hello_future_character (cast `/Game/Map/YJ_HelloFutureCharacter` OtherActor))
      (`/Game/Map/YJ_HelloFutureCharacter.Grab Apple On Server` _asyj_hello_future_character "/Game/Map/Animation/Plant2_Montage1.Plant2_Montage1" self)
      ;[1 1 1] Apple 아이템 추가
      (`YJ_InventoryComponent.AddItem2` (`HelloFutureCharacter.Inventory` _asyj_hello_future_character) "Gem"))
    (:`then_1`
      (bind _asyj_hello_future_character_2 (cast `/Game/Map/YJ_HelloFutureCharacter` (`GameplayStatics.GetPlayerCharacter` 0)))
      (for _array_element (`/Game/Oh/RealQuest/QuestLog.Quests` (`/Game/Map/YJ_HelloFutureCharacter.QuestLog` _asyj_hello_future_character_2))
        (`/Game/Oh/RealQuest/Quests/OH_RealQuest.CollectedItem` _array_element "Gem")))))

(fn `UserConstructionScript`)