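; Farm tile where the player plants, fertilizes and harvests wheat, corn, pumpkin or radish through interface events.
; Planting consumes a seed, then swaps three stage meshes on GrowTime countdowns shown by a TextRender.
; Corn, pumpkin and radish roll ChanceOfDisease each stage; wheat skips it.
; Fertilizers shorten growth, tonic zeroes disease odds and magic powder may yield "Gold", which Harvest spawns as a pumpkin seed instead of the crop.
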(event `self.ReceiveBeginPlay`
  ;[1 1 1] 타이머 표시
  (`TextRenderComponent.K2_SetText` (`self.TextRender`) (`self.Value`)))

(event `Blue`
  (bind _farmtile (`self.FarmTile`))
  ;[1 1 1] 선택된건 파랑
  (`PrimitiveComponent.SetMaterial` _farmtile 0 "/Game/Minsu/Farm/BP/M_Select.M_Select")
  (`KismetSystemLibrary.Delay` 0.2)
  (`PrimitiveComponent.SetMaterial` _farmtile 0 "/Game/Import/Village/Materials/Village_Base_Village_Base_0_MatInstnace.Village_Base_Village_Base_0_MatInstnace"))

(event `/Game/Minsu/Farm/BPI_Fertilizer.BPI_Fertilizer`
  ;[1 1 1] 비료뿌리기 BPI
  (if (`self.IsSomethingPlanted?`)
    (`self.Red`)
    (elif (`self.Is Fertilizer?`)
      (`self.Red`)
      (else
        (bind _asyj_hello_future_character (cast `/Game/Map/YJ_HelloFutureCharacter` (`GameplayStatics.GetPlayerCharacter` 0)))
        (switch `int` (`/Game/Map/YJ_HelloFutureCharacter.Item` _asyj_hello_future_character)
          (:`0`
            (`self.Fertilizer`))
          (:`1`
            (`self.Fertilizer2`))
          (:`2`
            (`self.MagicPowder`))
          (:`3`
            (`self.Tonic`)))))))

(event `Red`
  (bind _farmtile (`self.FarmTile`))
  ;[1 1 1] 이미 있는건 빨강색
  (`PrimitiveComponent.SetMaterial` _farmtile 0 "/Game/Minsu/Farm/BP/M_Planted.M_Planted")
  (`KismetSystemLibrary.Delay` 1.0)
  (`PrimitiveComponent.SetMaterial` _farmtile 0 "/Game/Import/Village/Materials/Village_Base_Village_Base_0_MatInstnace.Village_Base_Village_Base_0_MatInstnace"))

(event `/Game/Minsu/Farm/BPI_Activate.BPI_Activate`
  ;[1 1 1] 수확하기 BPI
  (`self.Harvest`))

(event `Plant Wheat`
  ;[1 1 1] 밀 심기
  (bind _returnvalue (`AddComponent|NODE_AddStaticMeshComponent-0` :`RelativeTransform` (`KismetMathLibrary.MakeTransform` (`self.Relative Transfrom Location`))))
  (`self.GrowTime` (`self.WheatGrowTime`)
    (:`Out`
      (`ActorComponent.K2_DestroyComponent` _returnvalue)
      (bind _returnvalue_2 (`AddComponent|NODE_AddStaticMeshComponent-1` :`RelativeTransform` (`KismetMathLibrary.MakeTransform` (`self.Relative Transfrom Location`))))
      (`self.GrowTime` (`self.WheatGrowTime`)
        (:`Out`
          (`ActorComponent.K2_DestroyComponent` _returnvalue_2)
          (bind _returnvalue_3 (`AddComponent|NODE_AddStaticMeshComponent-2` :`RelativeTransform` (`KismetMathLibrary.MakeTransform` (`self.Relative Transfrom Location`))))
          (set `self.FullyGrown?` true)
          (set `self.Is Fertilizer?` false)
          (set `self.CurrentMesh` _returnvalue_3)
          (set `self.DiseaseValue` 20)
          (if (`self.Is Magic?`)
            (set `self.WhatCanBeHarvested` "Gold")
            (else
              (set `self.WhatCanBeHarvested` "Wheat")))
          (set `self.Is Magic?` false))))))

(event `/Game/Minsu/Farm/BPI_PlantSeed.BPI_PlantSeed`
  ;[1 1 1] 씨앗 심기 BPI
  (if (`self.IsSomethingPlanted?`)
    (`self.Red`)
    (else
      (`self.Blue`)
      (bind _asyj_hello_future_character (cast `/Game/Map/YJ_HelloFutureCharacter` (`GameplayStatics.GetPlayerCharacter` 0)))
      (switch `int` (`/Game/Map/YJ_HelloFutureCharacter.Seed` _asyj_hello_future_character)
        (:`0`
          (`self.DoWeHaveWheatSeed`
            (:`Output`
              (`self.Plant Wheat`))))
        (:`1`
          (`self.DoWeHaveCornSeed`
            (:`Output`
              (`self.Plant Corn`))))
        (:`2`
          (`self.DoWeHavePumpkinSeed`
            (:`Output`
              (`self.Plant Pumpkin`))))
        (:`3`
          (`self.DoWeHaveRadishSeed`
            (:`Output`
              (`self.Plant Radish`)))))
      (set `self.IsSomethingPlanted?` true)
      (set `self.Is Fertilizer?` false))))

(event `Plant Corn`
  ;[1 1 1] 옥수수 심기
  (bind _returnvalue (`AddComponent|NODE_AddStaticMeshComponent-3` :`RelativeTransform` (`KismetMathLibrary.MakeTransform` (`self.Relative Transfrom Location`))))
  (`self.GrowTime` (`self.CornGrowTime`)
    (:`Out`
      (`self.ChanceOfDisease` _returnvalue
        (:`NoDisease`
          (`ActorComponent.K2_DestroyComponent` _returnvalue)
          (bind _returnvalue_2 (`AddComponent|NODE_AddStaticMeshComponent-4`))
          (`self.GrowTime` (`self.CornGrowTime`)
            (:`Out`
              (`self.ChanceOfDisease` _returnvalue_2
                (:`NoDisease`
                  (`ActorComponent.K2_DestroyComponent` _returnvalue_2)
                  (bind _returnvalue_3 (`AddComponent|NODE_AddStaticMeshComponent-5`))
                  (`self.ChanceOfDisease` _returnvalue_3
                    (:`NoDisease`
                      (set `self.FullyGrown?` true)
                      (set `self.Is Fertilizer?` false)
                      (set `self.CurrentMesh` _returnvalue_3)
                      (set `self.DiseaseValue` 20)
                      (if (`self.Is Magic?`)
                        (set `self.WhatCanBeHarvested` "Gold")
                        (else
                          (set `self.WhatCanBeHarvested` "Corn")))
                      (set `self.Is Magic?` false))))))))))))

(event `Plant Pumpkin`
  ;[1 1 1] 호박 심기
  (bind _returnvalue (`AddComponent|NODE_AddStaticMeshComponent-6` :`RelativeTransform` (`KismetMathLibrary.MakeTransform` (`self.Relative Transfrom Location`))))
  (`self.GrowTime` (`self.PumpkinGrowTime`)
    (:`Out`
      (`self.ChanceOfDisease` _returnvalue
        (:`NoDisease`
          (`ActorComponent.K2_DestroyComponent` _returnvalue)
          (bind _returnvalue_2 (`AddComponent|NODE_AddStaticMeshComponent-7`))
          (`self.GrowTime` (`self.PumpkinGrowTime`)
            (:`Out`
              (`self.ChanceOfDisease` _returnvalue_2
                (:`NoDisease`
                  (`ActorComponent.K2_DestroyComponent` _returnvalue_2)
                  (bind _returnvalue_3 (`AddComponent|NODE_AddStaticMeshComponent-8`))
                  (`self.ChanceOfDisease` _returnvalue_3
                    (:`NoDisease`
                      (set `self.FullyGrown?` true)
                      (set `self.Is Fertilizer?` false)
                      (set `self.CurrentMesh` _returnvalue_3)
                      (set `self.DiseaseValue` 20)
                      (if (`self.Is Magic?`)
                        (set `self.WhatCanBeHarvested` "Gold")
                        (else
                          (set `self.WhatCanBeHarvested` "Pumpkin")))
                      (set `self.Is Magic?` false))))))))))))

(event `Plant Radish`
  (bind (_relative_transfrom_location_x _relative_transfrom_location_y _relative_transfrom_location_z) (`KismetMathLibrary.BreakVector` (`self.Relative Transfrom Location`)))
  (bind (_relative_transfrom_location_x_2 _relative_transfrom_location_y_2 _relative_transfrom_location_z_2) (`KismetMathLibrary.BreakVector` (`self.Relative Transfrom Location`)))
  ;[1 1 1] 무심기
  (bind _returnvalue (`AddComponent|NODE_AddStaticMeshComponent-9` :`RelativeTransform` (`KismetMathLibrary.MakeTransform` (`self.Relative Transfrom Location`))))
  (`self.GrowTime` (`self.RadishGrowTime`)
    (:`Out`
      (`self.ChanceOfDisease` _returnvalue
        (:`NoDisease`
          (`ActorComponent.K2_DestroyComponent` _returnvalue)
          (bind _returnvalue_2 (`AddComponent|NODE_AddStaticMeshComponent-10` :`RelativeTransform` (`KismetMathLibrary.MakeTransform` (`KismetMathLibrary.MakeVector` _relative_transfrom_location_x _relative_transfrom_location_y (+ _relative_transfrom_location_z 15.0)))))
          (`self.GrowTime` (`self.RadishGrowTime`)
            (:`Out`
              (`self.ChanceOfDisease` _returnvalue_2
                (:`NoDisease`
                  (`ActorComponent.K2_DestroyComponent` _returnvalue_2)
                  (bind _returnvalue_3 (`AddComponent|NODE_AddStaticMeshComponent-11` :`RelativeTransform` (`KismetMathLibrary.MakeTransform` (`KismetMathLibrary.MakeVector` _relative_transfrom_location_x_2 _relative_transfrom_location_y_2 (+ _relative_transfrom_location_z_2 30.0)))))
                  (`self.ChanceOfDisease` _returnvalue_3
                    (:`NoDisease`
                      (set `self.FullyGrown?` true)
                      (set `self.Is Fertilizer?` false)
                      (set `self.CurrentMesh` _returnvalue_3)
                      (set `self.DiseaseValue` 20)
                      (if (`self.Is Magic?`)
                        (set `self.WhatCanBeHarvested` "Gold")
                        (else
                          (set `self.WhatCanBeHarvested` "Radish")))
                      (set `self.Is Magic?` false))))))))))))

(fn `Fertilizer`
  (bind (_relative_transfrom_location_x _relative_transfrom_location_y _relative_transfrom_location_z) (`KismetMathLibrary.BreakVector` (`self.Relative Transfrom Location`)))
  (bind _inventory (`HelloFutureCharacter.Inventory` (cast `HelloFutureCharacter` (`GameplayStatics.GetPlayerCharacter` 0) :!pure true)))
  ;[1 1 1] 아이템 지우기
  (for _array_element (`YJ_InventoryComponent.Items` _inventory)
    (bind _asbp_fertilizer_item (cast `/Game/YJ/Blueprints/Inventory/BP_FertilizerItem` _array_element))
    (if (not (<= (`YJ_Item.Count` _asbp_fertilizer_item) 0))
      (`|ExecutionSequence`
        (:`then_0`
          (`YJ_InventoryComponent.RemoveItem2` _inventory "Fertilizer"))
        (:`then_1`
          (`self.Blue`)
          (bind _returnvalue (`AddComponent|NODE_AddStaticMeshComponent-16` :`RelativeTransform` (`KismetMathLibrary.MakeTransform` (`KismetMathLibrary.MakeVector` _relative_transfrom_location_x _relative_transfrom_location_y (+ _relative_transfrom_location_z 3.0)))))
          (set `self.FertilizerComponent` _returnvalue)
          (`|ExecutionSequence`
            (:`then_0`
              (set `self.WheatGrowTime` (/ (`self.WheatGrowTime`) 2)))
            (:`then_1`
              (set `self.CornGrowTime` (/ (`self.CornGrowTime`) 2)))
            (:`then_2`
              (set `self.PumpkinGrowTime` (/ (`self.PumpkinGrowTime`) 2)))
            (:`then_3`
              (set `self.RadishGrowTime` (/ (`self.RadishGrowTime`) 2))))
          (set `self.Is Fertilizer?` true))))))

(fn `Fertilizer2`
  (bind (_relative_transfrom_location_x _relative_transfrom_location_y _relative_transfrom_location_z) (`KismetMathLibrary.BreakVector` (`self.Relative Transfrom Location`)))
  (bind _inventory (`HelloFutureCharacter.Inventory` (cast `HelloFutureCharacter` (`GameplayStatics.GetPlayerCharacter` 0) :!pure true)))
  ;[1 1 1] 아이템 지우기
  (for _array_element (`YJ_InventoryComponent.Items` _inventory)
    (bind _asbp_fertilizer_2item (cast `/Game/YJ/Blueprints/Inventory/BP_Fertilizer2Item` _array_element))
    (if (not (<= (`YJ_Item.Count` _asbp_fertilizer_2item) 0))
      (`|ExecutionSequence`
        (:`then_0`
          (`YJ_InventoryComponent.RemoveItem2` _inventory "Fertilizer2"))
        (:`then_1`
          (`self.Blue`)
          (bind _returnvalue (`AddComponent|NODE_AddStaticMeshComponent-17` :`RelativeTransform` (`KismetMathLibrary.MakeTransform` (`KismetMathLibrary.MakeVector` _relative_transfrom_location_x _relative_transfrom_location_y (+ _relative_transfrom_location_z 3.0)))))
          (set `self.FertilizerComponent` _returnvalue)
          (`|ExecutionSequence`
            (:`then_0`
              (set `self.WheatGrowTime` (/ (`self.WheatGrowTime`) 4)))
            (:`then_1`
              (set `self.CornGrowTime` (/ (`self.CornGrowTime`) 4)))
            (:`then_2`
              (set `self.PumpkinGrowTime` (/ (`self.PumpkinGrowTime`) 4)))
            (:`then_3`
              (set `self.RadishGrowTime` (/ (`self.RadishGrowTime`) 4))))
          (set `self.Is Fertilizer?` true))))))

(fn `Harvest`
  (bind _farmtile (`self.FarmTile`))
  (bind _fertilizercomponent (`self.FertilizerComponent`))
  (bind (_returnvalue_x _returnvalue_y _returnvalue_z) (`KismetMathLibrary.BreakVector` (`SceneComponent.K2_GetComponentLocation` (`self.TextRender`))))
  (bind _returnvalue (`KismetMathLibrary.Conv_VectorToTransform` (`SceneComponent.K2_GetComponentLocation` (`self.TextRender`))))
  (if (`self.FullyGrown?`)
    (`/Engine/EditorBlueprintResources/StandardMacros.IsValid` _fertilizercomponent
      (:`Is Valid`
        (`ActorComponent.K2_DestroyComponent` _fertilizercomponent))
      (:`Is Not Valid`
        _))
    (`PrimitiveComponent.SetMaterial` _farmtile 0 "/Game/Minsu/Farm/BP/M_Select.M_Select")
    (`PrimitiveComponent.SetMaterial` _farmtile 0 "/Game/Import/Village/Materials/Village_Base_Village_Base_0_MatInstnace.Village_Base_Village_Base_0_MatInstnace")
    (`ActorComponent.K2_DestroyComponent` (`self.CurrentMesh`))
    (switch `string` (`self.WhatCanBeHarvested`)
      (:`Default`
        _)
      (:`Wheat`
        (`|SpawnActorFromClass` "/Game/Minsu/Farm/BP/BP_WheatLoose.BP_WheatLoose_C" _returnvalue "Undefined" "OverrideRootScale" null null))
      (:`Corn`
        (`|SpawnActorFromClass` "/Game/Minsu/Farm/BP/BP_CornLoose.BP_CornLoose_C" _returnvalue "Undefined" "OverrideRootScale" null null))
      (:`Pumpkin`
        (`|SpawnActorFromClass` "/Game/Minsu/Farm/BP/BP_PumpkinLoose.BP_PumpkinLoose_C" _returnvalue "Undefined" "OverrideRootScale" null null))
      (:`Radish`
        (`|ExecutionSequence`
          (:`then_0`
            (`|SpawnActorFromClass` "/Game/Minsu/Farm/BP/BP_Radish.BP_Radish_C" (`KismetMathLibrary.MakeTransform` (`KismetMathLibrary.MakeVector` (- _returnvalue_x 25.0) _returnvalue_y _returnvalue_z) (struct :`Roll` 10.0)) "Undefined" "OverrideRootScale" null null))
          (:`then_1`
            (`|SpawnActorFromClass` "/Game/Minsu/Farm/BP/BP_Radish.BP_Radish_C" (`KismetMathLibrary.MakeTransform` (`KismetMathLibrary.MakeVector` (+ _returnvalue_x 25.0) _returnvalue_y _returnvalue_z) (struct :`Pitch` 45.0)) "Undefined" "OverrideRootScale" null null))
          (:`then_2`
            (`|SpawnActorFromClass` "/Game/Minsu/Farm/BP/BP_Radish.BP_Radish_C" (`KismetMathLibrary.MakeTransform` (`KismetMathLibrary.MakeVector` _returnvalue_x (+ _returnvalue_y 25.0) _returnvalue_z) (struct :`Yaw` 80.0)) "Undefined" "OverrideRootScale" null null))
          (:`then_3`
            (`|SpawnActorFromClass` "/Game/Minsu/Farm/BP/BP_Radish.BP_Radish_C" (`KismetMathLibrary.MakeTransform` (`KismetMathLibrary.MakeVector` _returnvalue_x (- _returnvalue_y 25.0) _returnvalue_z) (struct :`Pitch` 30.0)) "Undefined" "OverrideRootScale" null null))))
      (:`Gold`
        (`|SpawnActorFromClass` "/Game/Minsu/Farm/BP/BP_PumpkinSeed.BP_PumpkinSeed_C" _returnvalue "Undefined" "OverrideRootScale" null null)))
    (set `self.FullyGrown?` false)
    (set `self.CurrentMesh` null)
    (set `self.IsSomethingPlanted?` false)
    (set `self.WhatCanBeHarvested` "")
    (`|ExecutionSequence`
      (:`then_0`
        (set `self.WheatGrowTime` 5))
      (:`then_1`
        (set `self.CornGrowTime` 15))
      (:`then_2`
        (set `self.PumpkinGrowTime` 30))
      (:`then_3`
        (set `self.RadishGrowTime` 3)))
    (set `self.Is Fertilizer?` false)))

(fn `MagicPowder`
  (bind (_relative_transfrom_location_x _relative_transfrom_location_y _relative_transfrom_location_z) (`KismetMathLibrary.BreakVector` (`self.Relative Transfrom Location`)))
  (bind _inventory (`HelloFutureCharacter.Inventory` (cast `HelloFutureCharacter` (`GameplayStatics.GetPlayerCharacter` 0) :!pure true)))
  ;[1 1 1] 아이템 지우기
  (for _array_element (`YJ_InventoryComponent.Items` _inventory)
    (bind _asbp_magic_powder_item (cast `/Game/YJ/Blueprints/Inventory/BP_MagicPowderItem` _array_element))
    (if (not (<= (`YJ_Item.Count` _asbp_magic_powder_item) 0))
      (`|ExecutionSequence`
        (:`then_0`
          (`YJ_InventoryComponent.RemoveItem2` _inventory "MagicPowder"))
        (:`then_1`
          (`self.Blue`)
          (bind _returnvalue (`AddComponent|NODE_AddStaticMeshComponent-18` :`RelativeTransform` (`KismetMathLibrary.MakeTransform` (`KismetMathLibrary.MakeVector` _relative_transfrom_location_x _relative_transfrom_location_y (+ _relative_transfrom_location_z 3.0)))))
          (set `self.FertilizerComponent` _returnvalue)
          (if (< (`KismetMathLibrary.RandomIntegerInRange` 1 100) 51)
            (set `self.Is Magic?` true)
            (else
              (set `self.Is Magic?` false)))
          (set `self.Is Fertilizer?` true))))))

(fn `ReturnBoxes`
  (returns (Boxes :type "Array of BoxComponent Object Reference"))
  (return (`|MakeArray` (`self.Box1`) (`self.Box2`) (`self.Box3`) (`self.Box`))))

(fn `Tonic`
  (bind _inventory (`HelloFutureCharacter.Inventory` (cast `HelloFutureCharacter` (`GameplayStatics.GetPlayerCharacter` 0) :!pure true)))
  ;[1 1 1] 아이템 지우기
  (for _array_element (`YJ_InventoryComponent.Items` _inventory)
    (bind _asbp_tonic_item (cast `/Game/YJ/Blueprints/Inventory/BP_TonicItem` _array_element))
    (if (not (<= (`YJ_Item.Count` _asbp_tonic_item) 0))
      (`|ExecutionSequence`
        (:`then_0`
          (`YJ_InventoryComponent.RemoveItem2` _inventory "Tonic"))
        (:`then_1`
          (`self.Blue`)
          (bind _returnvalue (`AddComponent|NODE_AddStaticMeshComponent-20` :`RelativeTransform` (`KismetMathLibrary.MakeTransform` (`self.Relative Transfrom Location`))))
          (set `self.FertilizerComponent` _returnvalue)
          (set `self.DiseaseValue` 0)
          (set `self.Is Fertilizer?` true))))))

(fn `UserConstructionScript`)