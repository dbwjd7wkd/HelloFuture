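; BP_Cow is a farm cow that the player can feed wheat through the BPIFeed event.
; If IsFeed is set it flashes a red material, otherwise it flashes a selection material and, for item 0, checks the player's inventory for wheat and removes it.
; EatWheat then adds a temporary mesh, plays the eat montage and pauses movement before restoring NavWalking.
; Overlap events are empty, leaving the look-at and feed-widget logic disconnected.
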(event `self.boxComp.OnComponentBeginOverlap`
  (params (OverlappedComponent :type "PrimitiveComponent Object Reference") (OtherActor :type "Actor Object Reference") (OtherComp :type "PrimitiveComponent Object Reference") (OtherBodyIndex :type Integer) (bFromSweep :type Boolean) (SweepResult :type "HitResult Structure (by ref)")))

(event `self.boxComp.OnComponentEndOverlap`
  (params (OverlappedComponent :type "PrimitiveComponent Object Reference") (OtherActor :type "Actor Object Reference") (OtherComp :type "PrimitiveComponent Object Reference") (OtherBodyIndex :type Integer)))

(event `/Game/Minsu/Farm/Animal/BP/BPI_Feed.BPI_Feed`
  (if (`self.Is Feed?`)
    (`self.Red`)
    (else
      (`self.Blue`)
      (bind _asyj_hello_future_character (cast `/Game/Map/YJ_HelloFutureCharacter` (`GameplayStatics.GetPlayerCharacter` 0)))
      (switch `int` (`/Game/Map/YJ_HelloFutureCharacter.Item` _asyj_hello_future_character)
        (:`0`
          (`self.DoWeHaveWheat?`
            (:`Output`
              (`self.Eat Wheat`))))))))

(event `Eat Wheat`
  (bind _charactermovement (`self.CharacterMovement`))
  (`|ExecutionSequence`
    (:`then_0`
      (bind _returnvalue (`AddComponent|NODE_AddStaticMeshComponent-0` :`RelativeTransform` (`KismetMathLibrary.MakeTransform` (`self.Relative Location`))))
      (`self.PlayAnimMontage` "/Game/Minsu/Farm/Animal/Anim_LowPoly_Cow_Eat_loop_Montage.Anim_LowPoly_Cow_Eat_loop_Montage")
      (`CharacterMovementComponent.SetMovementMode` _charactermovement "MOVE_None" 0)
      (`CharacterMovementComponent.DisableMovement` _charactermovement)
      (`KismetSystemLibrary.Delay` 3.33)
      (`ActorComponent.K2_DestroyComponent` _returnvalue)
      (`CharacterMovementComponent.SetMovementMode` _charactermovement "MOVE_NavWalking" 0))))

(event `Blue`
  (bind _mesh (`self.Mesh`))
  ;[1 1 1] 선택된건 파랑
  (`PrimitiveComponent.SetMaterial` _mesh 0 "/Game/Minsu/Farm/BP/M_Select.M_Select")
  (`KismetSystemLibrary.Delay` 0.2)
  (`PrimitiveComponent.SetMaterial` _mesh 0 "/Game/NewAssets/LowPoly_Farm_animals/Materials/M_LowPoly_Cows_color.M_LowPoly_Cows_color"))

(event `Red`
  (bind _mesh (`self.Mesh`))
  ;[1 1 1] 선택된건 파랑
  (`PrimitiveComponent.SetMaterial` _mesh 0 "/Game/Minsu/Farm/BP/M_Planted.M_Planted")
  (`KismetSystemLibrary.Delay` 1.0)
  (`PrimitiveComponent.SetMaterial` _mesh 0 "/Game/NewAssets/LowPoly_Farm_animals/Materials/M_LowPoly_Cows_color.M_LowPoly_Cows_color"))

(fn `UserConstructionScript`)