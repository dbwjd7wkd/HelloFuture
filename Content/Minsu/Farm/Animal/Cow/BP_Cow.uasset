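; Farm cow character that the player feeds wheat, corn, pumpkin or radish through the BPIFeed interface event.
; BPIFeed flashes a material for accepted or busy, then macros consume the selected crop from the player's inventory.
; Per-crop events show a food mesh and eat montage while movement stops, then randomly lead to sleep or idle.
; A camera-facing widget hides for a random cooldown after feeding; proximity UI, random-sleep and sound logic are unwired.
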(event `EatRadish`
  (bind _charactermovement (`self.CharacterMovement`))
  (bind _returnvalue (`AddComponent|NODE_AddStaticMeshComponent-3` :`RelativeTransform` (`KismetMathLibrary.MakeTransform` (`self.Relative Location`))))
  (`self.PlayAnimMontage` "/Game/Minsu/Farm/Animal/Cow/Anim_LowPoly_Cow_Eat_loop_Montage.Anim_LowPoly_Cow_Eat_loop_Montage")
  (set `CharacterMovementComponent.MaxWalkSpeed` 0.0 _charactermovement)
  (`CharacterMovementComponent.SetMovementMode` _charactermovement "MOVE_None" 0)
  (set `CharacterMovementComponent.RotationRate` (struct) _charactermovement)
  (set `self.Is Feed?` true)
  (`KismetSystemLibrary.Delay` 5.0)
  (`ActorComponent.K2_DestroyComponent` _returnvalue)
  (set `self.Is Feed?` false)
  (if (< (`KismetMathLibrary.RandomIntegerInRange` 0 100) 30)
    (`self.Sleep`)
    (else
      (set `self.m_state` "Idle")
      (`CharacterMovementComponent.SetMovementMode` (`self.CharacterMovement`) "MOVE_NavWalking" 0))))

(event `self.boxComp.OnComponentBeginOverlap`
  (params (OverlappedComponent :type "PrimitiveComponent Object Reference") (OtherActor :type "Actor Object Reference") (OtherComp :type "PrimitiveComponent Object Reference") (OtherBodyIndex :type Integer) (bFromSweep :type Boolean) (SweepResult :type "HitResult Structure (by ref)")))

(event `Eat Pumpkin`
  (bind _charactermovement (`self.CharacterMovement`))
  (bind _returnvalue (`AddComponent|NODE_AddStaticMeshComponent-2` :`RelativeTransform` (`KismetMathLibrary.MakeTransform` (`self.Relative Location`))))
  (`self.PlayAnimMontage` "/Game/Minsu/Farm/Animal/Cow/Anim_LowPoly_Cow_Eat_loop_Montage.Anim_LowPoly_Cow_Eat_loop_Montage")
  (set `CharacterMovementComponent.MaxWalkSpeed` 0.0 _charactermovement)
  (`CharacterMovementComponent.SetMovementMode` _charactermovement "MOVE_None" 0)
  (set `CharacterMovementComponent.RotationRate` (struct) _charactermovement)
  (set `self.Is Feed?` true)
  (`KismetSystemLibrary.Delay` 5.0)
  (`ActorComponent.K2_DestroyComponent` _returnvalue)
  (set `self.Is Feed?` false)
  (if (< (`KismetMathLibrary.RandomIntegerInRange` 0 100) 30)
    (`self.Sleep`)
    (else
      (set `self.m_state` "Idle")
      (`CharacterMovementComponent.SetMovementMode` (`self.CharacterMovement`) "MOVE_NavWalking" 0))))

(event `self.boxComp.OnComponentEndOverlap`
  (params (OverlappedComponent :type "PrimitiveComponent Object Reference") (OtherActor :type "Actor Object Reference") (OtherComp :type "PrimitiveComponent Object Reference") (OtherBodyIndex :type Integer)))

(event `Eat Corn`
  (bind _charactermovement (`self.CharacterMovement`))
  (bind _returnvalue (`AddComponent|NODE_AddStaticMeshComponent-1` :`RelativeTransform` (`KismetMathLibrary.MakeTransform` (`self.Relative Location`))))
  (`self.PlayAnimMontage` "/Game/Minsu/Farm/Animal/Cow/Anim_LowPoly_Cow_Eat_loop_Montage.Anim_LowPoly_Cow_Eat_loop_Montage")
  (set `CharacterMovementComponent.MaxWalkSpeed` 0.0 _charactermovement)
  (`CharacterMovementComponent.SetMovementMode` _charactermovement "MOVE_None" 0)
  (set `CharacterMovementComponent.RotationRate` (struct) _charactermovement)
  (set `self.Is Feed?` true)
  (`KismetSystemLibrary.Delay` 5.0)
  (`ActorComponent.K2_DestroyComponent` _returnvalue)
  (set `self.Is Feed?` false)
  (if (< (`KismetMathLibrary.RandomIntegerInRange` 0 100) 30)
    (`self.Sleep`)
    (else
      (set `self.m_state` "Idle")
      (`CharacterMovementComponent.SetMovementMode` (`self.CharacterMovement`) "MOVE_NavWalking" 0))))

(event `/Game/Minsu/Farm/Animal/BP/BPI_Feed.BPI_Feed`
  (bind _widget (`self.Widget`))
  (if (`self.Is Feed?`)
    (`self.Red`)
    (else
      (`self.Blue`)
      (bind _asyj_hello_future_character (cast `/Game/Map/YJ_HelloFutureCharacter` (`GameplayStatics.GetPlayerCharacter` 0)))
      (switch `int` (`/Game/Map/YJ_HelloFutureCharacter.Item` _asyj_hello_future_character)
        (:`0`
          (`self.DoWeHaveWheat?`
            (:`Output`
              (`self.Eat Wheat`))))
        (:`1`
          (`self.DoWeHaveCorn?`
            (:`Output`
              (`self.Eat Corn`))))
        (:`2`
          (`self.DoWeHavePumpkin?`
            (:`Output`
              (`self.Eat Pumpkin`))))
        (:`3`
          (`self.DoWeHaveRadish?`
            (:`Output`
              (`self.EatRadish`)))))
      (`SceneComponent.SetVisibility` _widget false false)
      (`KismetSystemLibrary.Delay` (`KismetMathLibrary.RandomFloatInRange` 7.0 50.0))
      (`SceneComponent.SetVisibility` _widget true false))))

(event `Eat Wheat`
  (bind _charactermovement (`self.CharacterMovement`))
  (bind _returnvalue (`AddComponent|NODE_AddStaticMeshComponent-0` :`RelativeTransform` (`KismetMathLibrary.MakeTransform` (`self.Relative Location`))))
  (`self.PlayAnimMontage` "/Game/Minsu/Farm/Animal/Cow/Anim_LowPoly_Cow_Eat_loop_Montage.Anim_LowPoly_Cow_Eat_loop_Montage")
  (set `CharacterMovementComponent.MaxWalkSpeed` 0.0 _charactermovement)
  (`CharacterMovementComponent.SetMovementMode` _charactermovement "MOVE_None" 0)
  (set `CharacterMovementComponent.RotationRate` (struct) _charactermovement)
  (set `self.Is Feed?` true)
  (`KismetSystemLibrary.Delay` 5.0)
  (`ActorComponent.K2_DestroyComponent` _returnvalue)
  (set `self.Is Feed?` false)
  (if (< (`KismetMathLibrary.RandomIntegerInRange` 0 100) 30)
    (`self.Sleep`)
    (else
      (set `self.m_state` "Idle")
      (`CharacterMovementComponent.SetMovementMode` (`self.CharacterMovement`) "MOVE_NavWalking" 0)
      (set `CharacterMovementComponent.RotationRate` (struct :`Yaw` 360.0) (`self.CharacterMovement`)))))

(event `Blue`
  (bind _mesh (`self.Mesh`))
  ;[1 1 1] 선택된건 파랑
  (`PrimitiveComponent.SetMaterial` _mesh 0 "/Game/Minsu/Farm/BP/M_Select.M_Select")
  (`KismetSystemLibrary.Delay` 0.2)
  (`PrimitiveComponent.SetMaterial` _mesh 0 "/Game/NewAssets/LowPoly_Farm_animals/Materials/M_LowPoly_Cows_color.M_LowPoly_Cows_color"))

(event `Red`
  (bind _mesh (`self.Mesh`))
  ;[1 1 1] 선택된건 파랑
  (`PrimitiveComponent.SetMaterial` _mesh 0 "/Game/Minsu/Farm/BP/M_Planted.M_Planted")
  (`KismetSystemLibrary.Delay` 1.0)
  (`PrimitiveComponent.SetMaterial` _mesh 0 "/Game/NewAssets/LowPoly_Farm_animals/Materials/M_LowPoly_Cows_color.M_LowPoly_Cows_color"))

(event `Sleep`
  (`self.PlayAnimMontage` "/Game/Minsu/Farm/Animal/Cow/COW_SleepMontage.COW_SleepMontage")
  (`KismetSystemLibrary.Delay` 11.25)
  (set `self.m_state` "Idle")
  (`CharacterMovementComponent.SetMovementMode` (`self.CharacterMovement`) "MOVE_NavWalking" 0)
  (set `CharacterMovementComponent.RotationRate` (struct :`Yaw` 360.0) (`self.CharacterMovement`)))

(event `self.ReceiveBeginPlay`)

(event `self.ReceiveTick`
  (params (DeltaSeconds :type "Float (single-precision)"))
  (bind _widget (`self.Widget`))
  (`SceneComponent.K2_SetWorldRotation` _widget (`KismetMathLibrary.FindLookAtRotation` (`SceneComponent.K2_GetComponentLocation` _widget) (`SceneComponent.K2_GetComponentLocation` (`PlayerCameraManager.TransformComponent` (`GameplayStatics.GetPlayerCameraManager` 0)))) false false))

(fn `UserConstructionScript`)