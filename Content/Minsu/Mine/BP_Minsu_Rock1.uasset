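; BP_Minsu_Rock1 is a mineable rock that calls SpawnFruit after the player holds Shake inside its box for MaxHoldTime.
; Box overlap enables input, shows WBP_Hold and opens a gate; a retriggerable delay completes the hold while a polled timer feeds widget progress.
; Tick toggles Mine_Montage on player 0.
; The Shake handler is marked for removal, having moved to YJ_HelloFutrueCharacter; SpawnActorOnServer also calls SpawnFruit.
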(event `Spawn Actor On Server`
  (`self.SpawnFruit`))

(event `InputAction|Shake`
  (params (Key :type "Key Structure"))
  ;[1 1 1] 삭제 예정(YJ_HelloFutrueCharacter에 구현함)
  (:`Pressed`
    (set `self.Is Held?` true)
    (`/Engine/EditorBlueprintResources/StandardMacros.Gate` true :!label _label
      (:`Exit`
        (`|ExecutionSequence`
          (:`then_0`
            (`KismetSystemLibrary.RetriggerableDelay` (`self.MaxHoldTime`))
            (if (`self.Is Held?`)
              (`self.SpawnFruit`)
              (`Widget.RemoveFromParent` (`self.Hold Widget`))))
          (:`then_1`
            (`self.Timer`)
            (`self.Update Timer`))))))
  (:`Released`
    (set `self.Is Held?` false)))

(event `self.Box.OnComponentBeginOverlap`
  (params (OverlappedComponent :type "PrimitiveComponent Object Reference") (OtherActor :type "Actor Object Reference") (OtherComp :type "PrimitiveComponent Object Reference") (OtherBodyIndex :type Integer) (bFromSweep :type Boolean) (SweepResult :type "HitResult Structure (by ref)"))
  ;[1 1 1] 삭제 예정(YJ_HelloFutrueCharacter에 구현함)
  (cast `HelloFutureCharacter` OtherActor)
  (set `self.Is Held Overlap?` true)
  (`self.EnableInput` (`GameplayStatics.GetPlayerController` 0))
  (bind _returnvalue (`|CreateWidget` "/Game/Minsu/Farm/BP/WBP_Hold.WBP_Hold_C" null null))
  (bind _output_get (set `self.Hold Widget` _returnvalue))
  (`UserWidget.AddToViewport` _output_get 0)
  (set `/Game/Minsu/Farm/BP/WBP_Hold.MaxTimeHeld` (`self.MaxHoldTime`) _output_get)
  (goto _label :!via `Open`))

(event `Stop Timer`
  ;[1 1 1] 삭제 예정(YJ_HelloFutrueCharacter에 구현함)
  (`KismetSystemLibrary.K2_PauseTimerHandle` (stale `Timer` _returnvalue)))

(event `self.Box.OnComponentEndOverlap`
  (params (OverlappedComponent :type "PrimitiveComponent Object Reference") (OtherActor :type "Actor Object Reference") (OtherComp :type "PrimitiveComponent Object Reference") (OtherBodyIndex :type Integer))
  ;[1 1 1] 삭제 예정(YJ_HelloFutrueCharacter에 구현함)
  (cast `HelloFutureCharacter` OtherActor)
  (set `self.Is Held Overlap?` false)
  (`self.DisableInput` (`GameplayStatics.GetPlayerController` 0))
  (`/Engine/EditorBlueprintResources/StandardMacros.IsValid` (stale `self.Box.OnComponentBeginOverlap` _returnvalue)
    (:`Is Valid`
      (`Widget.RemoveFromParent` (stale `self.Box.OnComponentBeginOverlap` _returnvalue))
      (goto _label :!via `Close`))))

(event `Timer`
  ;[1 1 1] 삭제 예정(YJ_HelloFutrueCharacter에 구현함)
  (bind _returnvalue (`KismetSystemLibrary.K2_SetTimerDelegate` (delegate `Timer`) (`self.MaxHoldTime`))))

(event `Update Timer`
  (bind _hold_widget (`self.Hold Widget`))
  ;[1 1 1] 삭제 예정(YJ_HelloFutrueCharacter에 구현함)
  (if (`self.Is Held?`)
    (set `/Game/Minsu/Farm/BP/WBP_Hold.TimeHeld` (`KismetSystemLibrary.K2_GetTimerElapsedTimeHandle` (stale `Timer` _returnvalue)) _hold_widget)
    (`KismetSystemLibrary.Delay` 0.1)
    (`self.Update Timer`)
    (else
      (`self.Stop Timer`)
      (set `/Game/Minsu/Farm/BP/WBP_Hold.TimeHeld` 0.0 _hold_widget))))

(event `self.ReceiveTick`
  (params (DeltaSeconds :type "Float (single-precision)"))
  (bind _returnvalue (`GameplayStatics.GetPlayerCharacter` 0))
  ;[1 1 1] 삭제 예정(YJ_HelloFutrueCharacter에 구현함)
  (if (`self.Is Held?`)
    (`/Engine/EditorBlueprintResources/StandardMacros.DoOnce` false :!label _label_2
      (:`Completed`
        (`Character.PlayAnimMontage` _returnvalue "/Game/Minsu/Mine/Mine_Montage.Mine_Montage" 1.0 "None")))
    (else
      (`Character.StopAnimMontage` _returnvalue "/Game/Minsu/Mine/Mine_Montage.Mine_Montage")
      (goto _label_2 :!via `Reset`))))

(fn `UserConstructionScript`)