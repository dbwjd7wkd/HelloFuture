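; BP_Chair is a chair actor that shows a chair UI while a HelloFutureCharacter overlaps its Collision component.
; Begin overlap creates a WBP_Chair widget with a reference to this chair, adds it to the viewport and sets IsSit true.
; End overlap removes that widget and clears IsSit.
; Both paths set player 0's input mode to Game and UI, so leaving does not restore game-only input.
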(event `self.collision.OnComponentBeginOverlap`
  (params (OverlappedComponent :type "PrimitiveComponent Object Reference") (OtherActor :type "Actor Object Reference") (OtherComp :type "PrimitiveComponent Object Reference") (OtherBodyIndex :type Integer) (bFromSweep :type Boolean) (SweepResult :type "HitResult Structure (by ref)"))
  (cast `HelloFutureCharacter` OtherActor)
  (bind _returnvalue (`|CreateWidget` "/Game/Minsu/Hall/WBP_Chair.WBP_Chair_C" null self))
  (`UserWidget.AddToViewport` _returnvalue 0)
  (set `self.isSit` true)
  (`WidgetBlueprintLibrary.SetInputMode_GameAndUIEx` (`GameplayStatics.GetPlayerController` 0) null :!label _label))

(event `self.collision.OnComponentEndOverlap`
  (params (OverlappedComponent :type "PrimitiveComponent Object Reference") (OtherActor :type "Actor Object Reference") (OtherComp :type "PrimitiveComponent Object Reference") (OtherBodyIndex :type Integer))
  (cast `HelloFutureCharacter` OtherActor)
  (`Widget.RemoveFromParent` (stale `self.collision.OnComponentBeginOverlap` _returnvalue))
  (set `self.isSit` false)
  (goto _label))

(fn `UserConstructionScript`)