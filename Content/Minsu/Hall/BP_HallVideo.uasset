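; BP_HallVideo is a proximity trigger that shows the Hall_Video widget when a HelloFutureCharacter enters its Capsule.
; On entry it creates and positions the widget on screen, also assigns it to the URLHall component, and enables Game-and-UI input with a mouse cursor.
; On exit it removes the widget and restores game-only input, without hiding the cursor.
; The web browser URL-loading code is unconnected.
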(event `self.Capsule.OnComponentBeginOverlap`
  (params (OverlappedComponent :type "PrimitiveComponent Object Reference") (OtherActor :type "Actor Object Reference") (OtherComp :type "PrimitiveComponent Object Reference") (OtherBodyIndex :type Integer) (bFromSweep :type Boolean) (SweepResult :type "HitResult Structure (by ref)"))
  (bind _returnvalue (`GameplayStatics.GetPlayerController` 0))
  (cast `HelloFutureCharacter` OtherActor)
  (bind _returnvalue_2 (`|CreateWidget` "/Game/Minsu/Hall/Hall_Video.Hall_Video_C"))
  (`UserWidget.SetDesiredSizeInViewport` _returnvalue_2 (1600.0 900.0))
  (`Widget.SetRenderTranslation` _returnvalue_2 (225.0 100.0))
  (`UserWidget.AddToViewport` _returnvalue_2 0)
  (`WidgetComponent.SetWidget` (`self.URLHall`) _returnvalue_2)
  (`WidgetBlueprintLibrary.SetInputMode_GameAndUIEx` _returnvalue (`WidgetComponent.GetUserWidgetObject` (`self.URLHall`)))
  (set `PlayerController.bShowMouseCursor` true _returnvalue))

(event `self.Capsule.OnComponentEndOverlap`
  (params (OverlappedComponent :type "PrimitiveComponent Object Reference") (OtherActor :type "Actor Object Reference") (OtherComp :type "PrimitiveComponent Object Reference") (OtherBodyIndex :type Integer))
  (cast `HelloFutureCharacter` OtherActor)
  (`Widget.RemoveFromParent` (stale `self.Capsule.OnComponentBeginOverlap` _returnvalue_2))
  (`WidgetBlueprintLibrary.SetInputMode_GameOnly` (`GameplayStatics.GetPlayerController` 0)))

(fn `UserConstructionScript`)