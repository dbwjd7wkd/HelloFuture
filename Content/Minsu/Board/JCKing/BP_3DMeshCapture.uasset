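; BP_3DMeshCapture is a capture actor pairing a skeletal mesh with a SceneCaptureComponent2D, apparently to show an animated character through a render target.
; On BeginPlay the mesh loops a hip-hop dance animation.
; ChangeMesh swaps in a given skeletal mesh, resetting its pose, and assigns Minsu_MeshRenderTarget as the capture's texture target.
; Unconnected graph leftovers for cycling or randomly picking other dances never run.
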(event `self.ReceiveBeginPlay`
  (`SkeletalMeshComponent.PlayAnimation` (`self.SkeletalMesh`) "/Game/MainCharacter/Animation/Wave_Hip_Hop_Dance.Wave_Hip_Hop_Dance" true))

(event `self.ReceiveTick`
  (params (DeltaSeconds :type "Float (single-precision)")))

(fn `ChangeMesh`
  (params (NewMesh :type "SkeletalMesh Object Reference"))
  (bind _scenecapturecomponent2d (`self.SceneCaptureComponent2D`))
  (`SkinnedMeshComponent.SetSkinnedAssetAndUpdate` (`self.SkeletalMesh`) NewMesh true)
  (bind _output_get (set `SceneCaptureComponent2D.TextureTarget` "/Game/Minsu/Board/JCKing/Minsu_MeshRenderTarget.Minsu_MeshRenderTarget" _scenecapturecomponent2d))
  (set `SceneCaptureComponent2D.TextureTarget` _output_get _scenecapturecomponent2d)
  (return))

(fn `UserConstructionScript`)