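; Notice board actor with three overlap zones that open screen widgets for JeoChuckKing, a newspaper web browser and a quiz.
; The JC zone also spawns a 3D mesh capture actor far below the level and destroys it on exit.
; The quiz zone alone filters for HelloFutureCharacter and picks its widget from IsQuiz.
; Zones remove or fade widgets on exit, but JC never restores game-only input.
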(event `self.JC.OnComponentBeginOverlap`
  (params (OverlappedComponent :type "PrimitiveComponent Object Reference") (OtherActor :type "Actor Object Reference") (OtherComp :type "PrimitiveComponent Object Reference") (OtherBodyIndex :type Integer) (bFromSweep :type Boolean) (SweepResult :type "HitResult Structure (by ref)"))
  (bind _returnvalue (`GameplayStatics.GetPlayerController` 0))
  ;[1 1 1] JeoChuckKing
  (set `self.IS JC?` true)
  (bind _returnvalue_2 (`|CreateWidget` "/Game/Minsu/Board/JCKing/WBP_JCKing.WBP_JCKing_C" _returnvalue))
  (`UserWidget.AddToViewport` _returnvalue_2 0)
  (`WidgetBlueprintLibrary.SetInputMode_GameAndUIEx` _returnvalue _returnvalue_2 "DoNotLock" false)
  (bind _returnvalue_3 (`|SpawnActorFromClass` "/Game/Minsu/Board/JCKing/BP_3DMeshCapture.BP_3DMeshCapture_C" (`KismetMathLibrary.MakeTransform` (0.0 0.0 -8000000.0)) "Undefined" "OverrideRootScale" null null)))

(event `self.ReceiveTick`
  (params (DeltaSeconds :type "Float (single-precision)")))

(event `self.JC.OnComponentEndOverlap`
  (params (OverlappedComponent :type "PrimitiveComponent Object Reference") (OtherActor :type "Actor Object Reference") (OtherComp :type "PrimitiveComponent Object Reference") (OtherBodyIndex :type Integer))
  ;[1 1 1] JeoChuckKing
  (set `self.IS JC?` false)
  (`/Game/Minsu/Board/JCKing/WBP_JCKing.Fade Out` (stale `self.JC.OnComponentBeginOverlap` _returnvalue_2))
  (`self.K2_DestroyActor` (stale `self.JC.OnComponentBeginOverlap` _returnvalue_3)))

(event `InputAction|InteractBoard`
  (params (Key :type "Key Structure")))

(event `self.NS.OnComponentBeginOverlap`
  (params (OverlappedComponent :type "PrimitiveComponent Object Reference") (OtherActor :type "Actor Object Reference") (OtherComp :type "PrimitiveComponent Object Reference") (OtherBodyIndex :type Integer) (bFromSweep :type Boolean) (SweepResult :type "HitResult Structure (by ref)"))
  (bind _returnvalue (`GameplayStatics.GetPlayerController` 0))
  ;[1 1 1] NewsPaper
  (set `self.IS NS?` true)
  (bind _returnvalue_2 (`|CreateWidget` "/Game/Minsu/Board/PC/WebBrowser.WebBrowser_C" _returnvalue))
  (`UserWidget.AddToViewport` _returnvalue_2 0)
  (`WidgetBlueprintLibrary.SetInputMode_GameAndUIEx` _returnvalue _returnvalue_2 "DoNotLock" false))

(event `self.NS.OnComponentEndOverlap`
  (params (OverlappedComponent :type "PrimitiveComponent Object Reference") (OtherActor :type "Actor Object Reference") (OtherComp :type "PrimitiveComponent Object Reference") (OtherBodyIndex :type Integer))
  ;[1 1 1] NewsPaper
  (set `self.IS NS?` false)
  (`/Game/Minsu/Board/PC/WebBrowser.Fade Out` (stale `self.NS.OnComponentBeginOverlap` _returnvalue_2))
  (`WidgetBlueprintLibrary.SetInputMode_GameOnly` (`GameplayStatics.GetPlayerController` 0)))

(event `self.QZ.OnComponentBeginOverlap`
  (params (OverlappedComponent :type "PrimitiveComponent Object Reference") (OtherActor :type "Actor Object Reference") (OtherComp :type "PrimitiveComponent Object Reference") (OtherBodyIndex :type Integer) (bFromSweep :type Boolean) (SweepResult :type "HitResult Structure (by ref)"))
  ;[1 1 1] Quiz
  (bind _ashello_future_character (cast `HelloFutureCharacter` OtherActor))
  (if (`HelloFutureCharacter.isQuiz` _ashello_future_character)
    (bind _returnvalue (`|CreateWidget` "/Game/Minsu/Board/Quiz/QuizArray/WBP_QuizJB.WBP_QuizJB_C"))
    (`UserWidget.AddToViewport` _returnvalue 0)
    (else
      (bind _returnvalue_2 (`|CreateWidget` "/Game/Minsu/Board/WBP_QZ.WBP_QZ_C"))
      (`UserWidget.AddToViewport` _returnvalue_2 0)
      (`WidgetBlueprintLibrary.SetInputMode_GameAndUIEx` (`GameplayStatics.GetPlayerController` 0) _returnvalue_2 "DoNotLock" false))))

(event `self.QZ.OnComponentEndOverlap`
  (params (OverlappedComponent :type "PrimitiveComponent Object Reference") (OtherActor :type "Actor Object Reference") (OtherComp :type "PrimitiveComponent Object Reference") (OtherBodyIndex :type Integer))
  ;[1 1 1] Quiz
  (cast `HelloFutureCharacter` OtherActor)
  (`/Engine/EditorBlueprintResources/StandardMacros.IsValid` (stale `self.QZ.OnComponentBeginOverlap` _returnvalue)
    (:`Is Valid`
      (`Widget.RemoveFromParent` (stale `self.QZ.OnComponentBeginOverlap` _returnvalue)))
    (:`Is Not Valid`
      (`Widget.RemoveFromParent` (stale `self.QZ.OnComponentBeginOverlap` _returnvalue_2))
      (`WidgetBlueprintLibrary.SetInputMode_GameOnly` (`GameplayStatics.GetPlayerController` 0)))))

(fn `UserConstructionScript`)