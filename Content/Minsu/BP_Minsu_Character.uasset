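; Player character Blueprint that adds a crosshair widget to the screen and carries unfinished logic for interacting with a notice board.
; The InteractBoard input raises a short-lived pressed flag that clears after a brief delay.
; A Newspaper event copies the notice board's ISNS state to the player and checks that flag, but triggers nothing.
; Nodes to open and close a web browser widget with mouse cursor are left disconnected.
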(event `self.ReceiveBeginPlay`
  (bind _returnvalue (`|CreateWidget` "/Game/Minsu/WBP_Crosshair.WBP_Crosshair_C"))
  (`UserWidget.AddToViewport` _returnvalue 0))

(event `InputAction|InteractBoard`
  (params (Key :type "Key Structure"))
  (:`Pressed`
    (set `self.IS E Pressed?` true)
    (`KismetSystemLibrary.Delay` 0.3)
    (set `self.IS E Pressed?` false)))

(event `self.ReceiveTick`
  (params (DeltaSeconds :type "Float (single-precision)")))

(event `Newspaper`
  (bind _returnvalue (`GameplayStatics.GetActorOfClass` "/Game/Minsu/Board/BP_Minsu_NoticeBoard.BP_Minsu_NoticeBoard_C"))
  (if (`/Game/Minsu/Board/BP_Minsu_NoticeBoard.IS NS?` _returnvalue)
    (set `self.IS NS Player?` true)
    (if (`self.IS E Pressed?`)
      _)
    (else
      (set `self.IS NS Player?` false))))

(fn `UserConstructionScript`)