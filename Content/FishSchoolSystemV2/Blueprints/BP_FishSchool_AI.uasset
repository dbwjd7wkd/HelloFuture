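; Actor that drives a Niagara particle school of fish, configured through flocking presets, shallow-water mode and animation type.
; Niagara exports the leader particle's position, which Tick uses to steer the school at box bounds or set an avoidance point from player, camera or custom actor.
; It manually advances the paused simulation to vary swim speed in alternating fast and slow phases, and throttles ticking when not recently rendered.
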(event `self.ReceiveBeginPlay`
  (bind _fish (`self.Fish`))
  (`self.CaluclateSwimmingBounds from Box Transform`)
  (`NiagaraComponent.SetVariableObject` (`self.Fish`) "ExportHandler" self)
  (`self.Adjust_School_Settings`)
  (`NiagaraComponent.SetPaused` _fish false)
  (`NiagaraComponent.SetAgeUpdateMode` _fish "TickDeltaTime")
  (set `self.DynamicSpeed_SpeedingUp?` (`KismetMathLibrary.RandomBool`))
  (`self.DynamicSpeed_Set_Slow` :!label _label ; Slow down the Speed
    (:`Completed`
      (`self.DynamicSpeed_Set_Fast` ; Speed up the Speed
        (:`Completed`
          (goto _label))))))

(event `Event_ResetSystem`
  (`NiagaraComponent.ResetSystem` (`self.Fish`)))

(event `self.ReceiveTick`
  (params (DeltaSeconds :type "Float (single-precision)"))
  (bind _dynamicspeed___acceleration (`self.DynamicSpeed - Acceleration`))
  (bind _fish (`self.Fish`))
  (bind _returnvalue (`KismetMathLibrary.SelectFloat` (* _dynamicspeed___acceleration 5.0) _dynamicspeed___acceleration (< (/ (`KismetMathLibrary.Vector_Distance` (`self.AvoidThisPosition`) (`self.SchoolLeaderPosition`)) (`self.Fish Swim Away From - Detection Distance`)) 1.0)))
  (if (`PrimitiveComponent.WasRecentlyRendered` (`self.Fish`) 0.2)
    (`self.SetActorTickInterval` 0.0)
    (`self.Make Fish Swim Away From ___`)
    (`NiagaraComponent.SetPaused` _fish false)
    (`NiagaraComponent.AdvanceSimulation` _fish 1 (`KismetMathLibrary.SelectFloat` (* DeltaSeconds (`KismetMathLibrary.Lerp` (`self.MovementSpeed_Min`) (`self.MovementSpeed_Max`) (`self.DynamicSpeed - Speed`))) (* DeltaSeconds (`self.Non-Dynamic_MovementSpeed`)) (`self.Use Dynamic Speed`)))
    (`NiagaraComponent.SetPaused` _fish true)
    (switch `/Game/FishSchoolSystemV2/Blueprints/Enum_AnimationType` (`self.Animation Type`)
      (:`NewEnumerator0`
        _)
      (:`NewEnumerator3`
        (`NiagaraComponent.SetVariableVec4` (`self.Fish`) "MaterialMod" (`KismetMathLibrary.MakeVector4` 100.0 (`self.VertexAnim Intensity`) 1.0 (`KismetMathLibrary.Lerp` (`self.Dynamic Vertex Anim Speed Min`) (`self.Dynamic Vertex Anim Speed Max`) (`self.DynamicSpeed_AnimScale`))))))
    (if (`self.Use Dynamic Speed`)
      (if (`self.DynamicSpeed_SpeedingUp?`)
        (set `self.DynamicSpeed - Speed` (`KismetMathLibrary.FInterpTo` (`self.DynamicSpeed - Speed`) (`self.DynamicSpeed - Desired_Speed`) (`GameplayStatics.GetWorldDeltaSeconds`) _returnvalue))
        (set `self.DynamicSpeed_AnimScale` (`KismetMathLibrary.FInterpTo` (`self.DynamicSpeed_AnimScale`) (`self.DynamicSpeed_Desired_AnimScale`) (`GameplayStatics.GetWorldDeltaSeconds`) _returnvalue))
        (else
          (set `self.DynamicSpeed - Speed` (`KismetMathLibrary.FInterpTo` (`self.DynamicSpeed - Speed`) (`self.DynamicSpeed - Desired_Speed`) (`GameplayStatics.GetWorldDeltaSeconds`) (`self.DynamicSpeed - Deceleration`)))
          (set `self.DynamicSpeed_AnimScale` (`KismetMathLibrary.FInterpTo` (`self.DynamicSpeed_AnimScale`) (`self.DynamicSpeed_Desired_AnimScale`) (`GameplayStatics.GetWorldDeltaSeconds`) (`self.DynamicSpeed - Acceleration`))))))
    (else
      (`NiagaraComponent.SetPaused` (`self.Fish`) true)
      (`self.SetActorTickInterval` 0.2))))

(event `self.ReceiveParticleData`
  (params (Data :type "Array of BasicParticleData Structure (by ref)") (NiagaraSystem :type "NiagaraSystem Object Reference"))
  ;[1 1 1] Receive Particle Position Data from Niagara Particle System
  (for (_array_element _array_index) Data
    (if (== _array_index 0)
      (set `self.SchoolLeaderPosition` (`.Position` (break `BasicParticleData` _array_element))))))

(fn `Adjust_School_Settings`
  (bind _shallowwaters (`self.ShallowWaters`))
  (bind _fish (`self.Fish`))
  (`NiagaraComponent.SetAsset` (`self.Fish`) (`self.NiagaraFishParticle`))
  (`NiagaraComponent.SetVariableInt` _fish "Number of Fish" (`self.Number of Fish`))
  (`NiagaraComponent.SetVariableFloat` _fish "AI_DetectionDistance" (`self.Fish Swim Away From - Detection Distance`))
  (`NiagaraComponent.SetVariableFloat` _fish "Mesh Scale Maximum" (`self.Fish Scale Maximum`))
  (`NiagaraComponent.SetVariableFloat` _fish "Mesh Scale Minimum" (`self.Fish Scale Minimum`))
  (`NiagaraComponent.SetVariableLinearColor` _fish "Color" (`self.Color`))
  (`NiagaraComponent.SetVariableVec3` _fish "InitialVelocity" (`KismetMathLibrary.SelectVector` (200.0 200.0 0.0) (0.0 0.0 0.0) _shallowwaters))
  (`NiagaraComponent.SetVariableFloat` _fish "AvoidanceStrength" (`KismetMathLibrary.SelectFloat` -20.0 1000.0 _shallowwaters))
  (`NiagaraComponent.SetVariableFloat` _fish "CurlNoiseMask" (`KismetMathLibrary.SelectFloat` 0.0 10000000000.0 _shallowwaters))
  (switch `/Game/FishSchoolSystemV2/Blueprints/Enum_AnimationType` (`self.Animation Type`)
    (:`NewEnumerator0`
      (`NiagaraComponent.SetVariableVec4` (`self.Fish`) "MaterialMod" (`KismetMathLibrary.MakeVector4` (`self.Auto Animation Frequency`) (`self.AutoAnimation Intensity`) 1.0 1.0)))
    (:`NewEnumerator3`
      (`NiagaraComponent.SetVariableVec4` (`self.Fish`) "MaterialMod" (`KismetMathLibrary.MakeVector4` 100.0 (`self.VertexAnim Intensity`) 1.0 (`self.Non-Dynamic Vertex Anim Speed`)))))
  (switch `/Game/FishSchoolSystemV2/Blueprints/Enum_FishFlockPresets` (`self.SchoolFlockPreset`)
    (:`NewEnumerator0`
      (`self.SetNiagaraSchoolVariables` (`self.CurNoiseForce_1_Strength`) (`self.CurNoiseForce_1_Size`) (`self.CurNoiseForce_2_Strength`) (`self.CurNoiseForce_2_Size`) (`self.CurNoiseForce_3_Strength`) (`self.CurNoiseForce_3_Size`) (`KismetMathLibrary.SelectFloat` 0.0 (`self.Wandering Randomness`) (`self.ShallowWaters`)) (`self.Drag`) (`self.Attraction_Min`) (`self.Attraction_Max`)))
    (:`NewEnumerator3`
      (`self.SetNiagaraSchoolVariables` 400.0 0.01 300.0 0.012 300.0 0.006 300.0 2.0 2.0 8.0))
    (:`NewEnumerator1`
      (`self.SetNiagaraSchoolVariables` 450.0 0.01 200.0 0.007 500.0 0.005 300.0 2.0 3.0 6.0))
    (:`NewEnumerator2`
      (`self.SetNiagaraSchoolVariables` 100.0 0.006 1500.0 0.002 500.0 0.002 100.0 1.0 0.0 3.0))
    (:`NewEnumerator4`
      (`self.SetNiagaraSchoolVariables` 100.0 0.006 500.0 0.002 5001.0 0.006 100.0 1.0 0.0 5.0))
    (:`NewEnumerator5`
      (`self.SetNiagaraSchoolVariables` 250.0 0.02 100.0 0.014 250.0 0.003 300.0 2.0 2.0 8.0))))

(fn `CaluclateSwimmingBounds from Box Transform`
  (bind _swimming_area_box (`self.Swimming Area Box`))
  (bind _returnvalue (`self.GetTransform` _swimming_area_box))
  (bind _x (.x (.location _returnvalue)))
  (bind _z (.z (.location _returnvalue)))
  (bind _y (.y (.location _returnvalue)))
  (bind _x_2 (.x (* (.scale _returnvalue) 100.0)))
  (bind _z_2 (.z (* (.scale _returnvalue) 100.0)))
  (bind _y_2 (.y (* (.scale _returnvalue) 100.0)))
  (`/Engine/EditorBlueprintResources/StandardMacros.IsValid` _swimming_area_box
    (:`Is Valid`
      (set `self.Maximum_Z_Bounds` (+ _z _z_2))
      (set `self.Minimum_Z_Bounds` (- _z _z_2))
      (set `self.Maximum_Y_Bounds` (+ _y _y_2))
      (set `self.Minimum_Y_Bounds` (- _y _y_2))
      (set `self.Maximim_X_Bounds` (+ _x _x_2))
      (set `self.Minimum_X_Bounds` (- _x _x_2)))))

(fn `Make Fish Swim Away From ___`
  (bind _z (.z (`self.SchoolLeaderPosition`)))
  (bind _returnvalue (`PlayerCameraManager.GetCameraLocation` (`GameplayStatics.GetPlayerCameraManager` 0)))
  (if (`self.ShallowWaters`)
    (if (>= (.z (`self.SchoolLeaderPosition`)) (`self.Maximum_Z_Bounds`))
      (`NiagaraComponent.SetVariableVec3` (`self.Fish`) "FollowMe_AttractorPosition" (`KismetMathLibrary.MakeVector` (+ (.x (`self.SchoolLeaderPosition`)) 50.0) (+ (.y (`self.SchoolLeaderPosition`)) 50.0) (.z (`self.K2_GetActorLocation`))) :!label _label)
      (elif (<= (.z (`self.SchoolLeaderPosition`)) (`self.Minimum_Z_Bounds`))
        (goto _label)))
    (else
      ;[1 1 1] Avoid Bounds of Swimming Area Box
      (if (>= (.z (`self.SchoolLeaderPosition`)) (`self.Maximum_Z_Bounds`))
        (`self.PushFishAwayFrom` 0.0 0.0 50.0)
        (elif (<= (.z (`self.SchoolLeaderPosition`)) (`self.Minimum_Z_Bounds`))
          (`self.PushFishAwayFrom` 0.0 0.0 -50.0)
          (elif (>= (.y (`self.SchoolLeaderPosition`)) (`self.Maximum_Y_Bounds`))
            (`self.PushFishAwayFrom` 0.0 50.0)
            (elif (<= (.y (`self.SchoolLeaderPosition`)) (`self.Minimum_Y_Bounds`))
              (`self.PushFishAwayFrom` 0.0 -50.0)
              (elif (>= (.x (`self.SchoolLeaderPosition`)) (`self.Maximim_X_Bounds`))
                (`self.PushFishAwayFrom` 50.0)
                (elif (<= (.x (`self.SchoolLeaderPosition`)) (`self.Minimum_X_Bounds`))
                  (`self.PushFishAwayFrom` -50.0)
                  (else
                    ;[1 1 1] Set location to Swim Away From
                    (switch `/Game/FishSchoolSystemV2/Blueprints/Enum_SwimAwayFrom` (`self.SwimAwayFrom`)
                      (:`NewEnumerator3`
                        (set `self.AvoidThisPosition` (`KismetMathLibrary.SelectVector` (`KismetMathLibrary.MakeVector` (.x (`self.K2_GetActorLocation` (`GameplayStatics.GetPlayerPawn` 0))) (.y (`self.K2_GetActorLocation` (`GameplayStatics.GetPlayerPawn` 0))) _z) (`self.K2_GetActorLocation` (`GameplayStatics.GetPlayerPawn` 0)) (`self.ShallowWaters`))))
                      (:`NewEnumerator1`
                        (set `self.AvoidThisPosition` (`KismetMathLibrary.SelectVector` (`KismetMathLibrary.MakeVector` (.x _returnvalue) (.y _returnvalue) _z) _returnvalue (`self.ShallowWaters`))))
                      (:`NewEnumerator5`
                        (set `self.AvoidThisPosition` (`KismetMathLibrary.SelectVector` (0.0 0.0 0.0) (`self.K2_GetActorLocation` (`self.CustomActor to Swim Away From`)) (`self.ShallowWaters`)))))
                    (`NiagaraComponent.SetVariableVec3` (`self.Fish`) "AvoidThis_Position" (`self.AvoidThisPosition`))))))))))))

(fn `UserConstructionScript`
  (`PrimitiveComponent.SetCastShadow` (`self.Fish`) (`self.Cast Shadow`))
  (`self.Adjust_School_Settings`)
  ;[1 1 1] if in shallow waters, rotate the fish randomly because its direction is now set by its initial velocity, and we need to randomize direction without randomizing its velocity
  (if (`self.ShallowWaters`)
    (`SceneComponent.K2_AddLocalRotation` (`self.Fish`) (`KismetMathLibrary.MakeRotator` 0.0 0.0 (`KismetMathLibrary.RandomFloatInRange` 0.0 360.0)) false false)))