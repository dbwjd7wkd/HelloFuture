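; Quest component that tracks a list of quests and one active quest with ordered steps.
; SelectQuest activates a quest by name, or the first one for an empty name.
; CompleteStep pops the first step, removing the quest when none remain and selecting the first remaining one.
; UpdateCache writes active steps back and rebuilds the name-keyed map after additions or step progress; auto-select on add is hard-disabled.
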(event `UpdateCache`
  (bind (_activequest_name _activequest_description _activequest_queststeps) (break `/Game/YJ/QuestSystem/Quest_Struct` (`self.ActiveQuest`)))
  (`BlueprintMapLibrary.Map_Clear` (`self.QuestCache`))
  (`|ExecutionSequence`
    (:`then_0`
      (if (!= (`self.CurrentQusetID`) -1)
        (setmembers `/Game/YJ/QuestSystem/Quest_Struct` :`StructRef` (`|GetArrayItem` (`self.Quests`) (`self.CurrentQusetID`)) :`Quest Steps` _activequest_queststeps)))
    (:`then_1`
      (for _array_element (`self.Quests`)
        (`BlueprintMapLibrary.Map_Add` (`self.QuestCache`) (`.Name_6_A8C5765242A0D43E903C23BBADD40D0F` (break `/Game/YJ/QuestSystem/Quest_Struct` _array_element)) _array_element)))))

(event `self.ReceiveBeginPlay`
  (add `self.Added/Removed Quest` (delegate `UpdateCache`)))

(event `AddQuest`
  (params (Quest :type "/Game/YJ/QuestSystem/NPC_Quest Structure"))
  (`KismetArrayLibrary.Array_Add` (`self.Quests`))
  (`self.Added/Removed Quest`)
  (if (and false (`self.CanChageQuest`))
    (`self.SelectQuest` "")))

(event `RemoveQuest`
  (`KismetArrayLibrary.Array_Remove` (`self.Quests`) (`self.CurrentQusetID`))
  (`self.SelectQuest` "")
  (set `self.CanChageQuest` true))

(event `CompleteStep`
  (bind (_activequest_name _activequest_description _activequest_queststeps) (break `/Game/YJ/QuestSystem/Quest_Struct` (`self.ActiveQuest`)))
  (`KismetArrayLibrary.Array_Remove` _activequest_queststeps)
  (if (== (`KismetArrayLibrary.Array_Length` _activequest_queststeps) 0)
    (`self.RemoveQuest`)
    (else
      (set `self.CanChageQuest` false)
      (`self.UpdateCache`))))

(event `SelectQuest`
  (params (QuestName :type String))
  (bind _activequest_name (break `/Game/YJ/QuestSystem/Quest_Struct` (`self.ActiveQuest`)))
  (if (`KismetMathLibrary.Conv_IntToBool` (`KismetArrayLibrary.Array_Length` (`self.Quests`)))
    (if (not (`KismetStringLibrary.EqualEqual_StrStr` _activequest_name QuestName))
      (`self.ResetQuest`)
      (if (`KismetStringLibrary.EqualEqual_StrStr` QuestName)
        (bind _output_get (set `self.CurrentQusetID` 0))
        (set `self.ActiveQuest` (`|GetArrayItem` (`self.Quests`) _output_get))
        (else
          (for (_array_element _array_index) (`self.Quests`)
            (if (`KismetStringLibrary.EqualEqual_StrStr` (`.Name_6_A8C5765242A0D43E903C23BBADD40D0F` (break `/Game/YJ/QuestSystem/Quest_Struct` _array_element)) QuestName)
              (set `self.CurrentQusetID` _array_index)
              (set `self.ActiveQuest` _array_element)
              (break))))))
    (else
      (`self.ResetQuest`))))