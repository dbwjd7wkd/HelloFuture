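; Clickable apple item for the selling system that opens a purchase widget for buying apples.
; BeginPlay creates WBP_purchase and fills in the apple name and a random price, rolled once per actor.
; Clicking any of three body components toggles the widget; opening it switches to UI-only input and passes it a newly constructed BP_Apple as the inventory item.
; Hiding it here does not restore the input mode.
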(event `self.ReceiveBeginPlay`
  (bind _returnvalue (`|CreateWidget` "/Game/Oh/BP/WBP_purchase.WBP_purchase_C"))
  (set `self.Purchase UI` _returnvalue)
  ;[1 1 1] UI에 값 넘겨주기
  (set `/Game/Oh/BP/WBP_purchase.FruitName` "사과" (`self.Purchase UI`))
  (set `/Game/Oh/BP/WBP_purchase.FruitPrice` (`KismetMathLibrary.RandomIntegerInRange` 400 1000) (`self.Purchase UI`)))

(event `self.body.OnClicked`
  (params (TouchedComponent :type "PrimitiveComponent Object Reference") (ButtonPressed :type "Key Structure"))
  (if (== (`self.is Show UI`) false) :!label _label
    (`WidgetBlueprintLibrary.SetInputMode_UIOnlyEx` (`GameplayStatics.GetPlayerController` 0) null)
    (`UserWidget.AddToViewport` (`self.Purchase UI`) 0)
    (set `self.is Show UI` true)
    ;[1 1 1] 현재 아이템 종류 인벤토리에 넣기
    (bind _returnvalue (`|GenericCreateObject` "/Game/YJ/Blueprints/Inventory/BP_Apple.BP_Apple_C" (`GameplayStatics.GetPlayerPawn` 0)))
    (set `/Game/Oh/BP/WBP_purchase.InventoryItem` _returnvalue (`self.Purchase UI`))
    (else
      (`Widget.RemoveFromParent` (`self.Purchase UI`))
      (set `self.is Show UI` false))))

(event `self.Bpdy2.OnClicked`
  (params (TouchedComponent :type "PrimitiveComponent Object Reference") (ButtonPressed :type "Key Structure"))
  (goto _label))

(event `self.Bpdy1.OnClicked`
  (params (TouchedComponent :type "PrimitiveComponent Object Reference") (ButtonPressed :type "Key Structure"))
  (goto _label))

(fn `UserConstructionScript`)