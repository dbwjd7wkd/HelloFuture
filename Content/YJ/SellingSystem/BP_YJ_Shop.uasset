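; BP_YJ_Shop is a shop trigger actor that shows the selling inventory while the player character overlaps its Box.
; On entry it shows the cursor, sets Game and UI input, then creates a new WBP_Selling_Inventory, so the focus target precedes that widget.
; On exit it restores game-only input and removes the widget, but leaves the cursor flag on.
; A dialogue-completed debug handler exists, but its binding never runs.
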(event `self.ReceiveBeginPlay`)

(event `self.Box.OnComponentBeginOverlap`
  (params (OverlappedComponent :type "PrimitiveComponent Object Reference") (OtherActor :type "Actor Object Reference") (OtherComp :type "PrimitiveComponent Object Reference") (OtherBodyIndex :type Integer) (bFromSweep :type Boolean) (SweepResult :type "HitResult Structure (by ref)"))
  (bind _returnvalue (`GameplayStatics.GetPlayerController` 0))
  (cast `HelloFutureCharacter` OtherActor)
  (set `PlayerController.bShowMouseCursor` true _returnvalue)
  (`WidgetBlueprintLibrary.SetInputMode_GameAndUIEx` _returnvalue (`self.SellingInventoryUI`))
  (bind _returnvalue_2 (`|CreateWidget` "/Game/YJ/SellingSystem/WBP_Selling_Inventory.WBP_Selling_Inventory_C"))
  (set `self.SellingInventoryUI` _returnvalue_2)
  (`UserWidget.AddToViewport` (`self.SellingInventoryUI`) 0)
  (`UserWidget.SetDesiredSizeInViewport` (`self.SellingInventoryUI`) (0.0 0.0)))

(event `self.Box.OnComponentEndOverlap`
  (params (OverlappedComponent :type "PrimitiveComponent Object Reference") (OtherActor :type "Actor Object Reference") (OtherComp :type "PrimitiveComponent Object Reference") (OtherBodyIndex :type Integer))
  (cast `HelloFutureCharacter` OtherActor)
  (`WidgetBlueprintLibrary.SetInputMode_GameOnly` (`GameplayStatics.GetPlayerController` 0))
  (`Widget.RemoveFromParent` (`self.SellingInventoryUI`)))

(event `OnDialogueCompleted_Event_0`
  (`KismetSystemLibrary.PrintString` "Hello"))

(fn `UserConstructionScript`)