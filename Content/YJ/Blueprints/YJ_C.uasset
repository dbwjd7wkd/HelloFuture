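; YJ_C is a player character that handles inventory, NPC dialogue, quests and seed planting.
; Tab and quest-list inputs toggle their UI through FlipFlops, while Tick creates the HUD once when IsPlaying is set.
; Camera line traces trigger NPC interaction and interface messages for planting or activation, with numpad keys stepping a clamped seed index.
; AskForQuest shows an NPC's first quest, and HUD acceptance moves it to OHQuestComponent.
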(event `Key|Tab`
  (params (Key :type "Key Structure"))
  (bind _returnvalue (`GameplayStatics.GetPlayerController` 0))
  ;[1 1 1] Inventory System UI 띄우기
  (:`Pressed`
    (`/Engine/EditorBlueprintResources/StandardMacros.FlipFlop`
      (:`A`
        (bind _returnvalue_2 (`|CreateWidget` "/Game/YJ/UI/Inventory/WBP_Inventory.WBP_Inventory_C" (`GameplayStatics.GetPlayerController` 0)))
        (`UserWidget.AddToViewport` _returnvalue_2 0)
        (`UserWidget.SetDesiredSizeInViewport` _returnvalue_2 (0.0 0.0))
        (set `PlayerController.bShowMouseCursor` true _returnvalue)
        (`WidgetBlueprintLibrary.SetInputMode_GameAndUIEx` _returnvalue null))
      (:`B`
        (`WidgetBlueprintLibrary.SetInputMode_GameOnly` (`GameplayStatics.GetPlayerController` 0))
        (`Widget.RemoveFromParent` _returnvalue_2)))))

(event `InputAction|Interact`
  (params (Key :type "Key Structure"))
  (bind _followcamera (`self.FollowCamera`))
  (bind _returnvalue (`SceneComponent.K2_GetComponentLocation` _followcamera))
  ;[1 1 1] 다이얼로그 시스템(삭제 예정)
  (:`Pressed`
    (bind (_outhit _returnvalue_2) (`KismetSystemLibrary.LineTraceSingle` :`Start` _returnvalue :`End` (+ _returnvalue (* (`SceneComponent.GetForwardVector` _followcamera) 1000.0)) :`TraceChannel` "TraceTypeQuery1" :`DrawDebugType` "ForDuration"))
    (if _returnvalue_2
      (bind _asbp_oh_npc_master (cast `/Game/Oh/NPC/BP_OH_NPC_Master` (`.HitActor` (`GameplayStatics.BreakHitResult` _outhit))))
      (`/Game/Oh/NPC/BP_OH_NPC_Interface.Interact` _asbp_oh_npc_master))))

(event `InputAction|Interact`
  (params (Key :type "Key Structure"))
  ;[1 1 1] 다이얼로그 시스템(삭제 예정)
  (:`Pressed`
    (if (> (`KismetArrayLibrary.Array_Length` (`self.InteractablesInRange`)) 0)
      _)))

(event `Ask For Quest`
  (params (NPC :type "/Game/Oh/NPC/BP_OH_NPC_Quest Object Reference (by ref)"))
  (bind _output_get (set `self.NPC Quest` NPC))
  (bind _quests_quests (break `/Game/Oh/Quest/Oh_NPC_Quest_Holder` (`/Game/Oh/NPC/BP_OH_NPC_Quest.Quests` _output_get)))
  (bind (_output_name _output_description) (break `/Game/Oh/Quest/OH_NPC_Quest` (`|GetArrayItem` _quests_quests)))
  (`/Game/Oh/Quest/WBP_OH_HUD.Open Info` (`self.HUD`) false _output_name _output_description))

(event `InputAction|Open Quest List`
  (params (Key :type "Key Structure"))
  (bind _hud (`self.HUD`))
  (:`Pressed`
    (`/Engine/EditorBlueprintResources/StandardMacros.FlipFlop`
      (:`A`
        (`/Game/Oh/Quest/WBP_OH_HUD.Open Quest List` _hud false))
      (:`B`
        (`/Game/Oh/Quest/WBP_OH_HUD.Open Quest List` _hud true)))))

(event `self.ReceiveBeginPlay`)

(event `self.ReceiveTick`
  (params (DeltaSeconds :type "Float (single-precision)"))
  (if (`self.isPlaying`)
    (`WidgetBlueprintLibrary.SetInputMode_GameAndUIEx` (`GameplayStatics.GetPlayerController` 0) null)
    (bind _returnvalue (`|CreateWidget` "/Game/Oh/Quest/WBP_OH_HUD.WBP_OH_HUD_C" null self))
    (bind _output_get (set `self.HUD` _returnvalue))
    (`UserWidget.AddToViewport` _output_get 0)
    (add `/Game/Oh/Quest/WBP_OH_HUD.Accept Quest` _output_get (delegate `Accept Quest`))
    (set `self.isPlaying` false)))

(event `Accept Quest`
  (bind _quests_quests (break `/Game/Oh/Quest/Oh_NPC_Quest_Holder` (`/Game/Oh/NPC/BP_OH_NPC_Quest.Quests` (`self.NPC Quest`))))
  (bind _quests_quests_2 (break `/Game/Oh/Quest/Oh_NPC_Quest_Holder` (`/Game/Oh/NPC/BP_OH_NPC_Quest.Quests` (`self.NPC Quest`))))
  (`/Game/Oh/Quest/OH_Quest_Component.Add Quests` (`self.OH_Quest_Component`) (`|GetArrayItem` _quests_quests_2))
  (`KismetArrayLibrary.Array_Remove` _quests_quests))

(event `Key|P`
  (params (Key :type "Key Structure"))
  (bind _followcamera (`self.FollowCamera`))
  (bind _returnvalue (`SceneComponent.K2_GetComponentLocation` _followcamera))
  ;[1 1 1] Comment
  (:`Pressed`
    (bind _outhit (`KismetSystemLibrary.LineTraceSingle` _returnvalue (+ _returnvalue (* (`KismetMathLibrary.GetForwardVector` (`SceneComponent.K2_GetComponentRotation` _followcamera)) 2000.0)) "TraceTypeQuery1"))
    (message `/Game/Minsu/Farm/BPI_PlantSeed.BPI_PlantSeed` (`.HitActor` (`GameplayStatics.BreakHitResult` _outhit)))))

(event `Key|NumPadTwo`
  (params (Key :type "Key Structure"))
  ;[1 1 1] Comment
  (:`Pressed`
    (bind _result (`/Engine/EditorBlueprintResources/StandardMacros.IncrementInt` (`self.Seed`))
      (:`  `
        (set `self.Seed` (`KismetMathLibrary.Clamp` _result 0 2))))))

(event `Key|NumPadEight`
  (params (Key :type "Key Structure"))
  ;[1 1 1] Comment
  (:`Pressed`
    (bind _result (`/Engine/EditorBlueprintResources/StandardMacros.DecrementInt` (`self.Seed`))
      (:`  `
        (set `self.Seed` (`KismetMathLibrary.Clamp` _result 0 2))))))

(event `Key|O`
  (params (Key :type "Key Structure"))
  (bind _followcamera (`self.FollowCamera`))
  (bind _returnvalue (`SceneComponent.K2_GetComponentLocation` _followcamera))
  ;[1 1 1] Comment
  (:`Pressed`
    (bind _outhit (`KismetSystemLibrary.LineTraceSingle` _returnvalue (+ _returnvalue (* (`KismetMathLibrary.GetForwardVector` (`SceneComponent.K2_GetComponentRotation` _followcamera)) 2000.0)) "TraceTypeQuery1"))
    (message `/Game/Minsu/Farm/BPI_Activate.BPI_Activate` (`.HitActor` (`GameplayStatics.BreakHitResult` _outhit)))))

(fn `UserConstructionScript`)