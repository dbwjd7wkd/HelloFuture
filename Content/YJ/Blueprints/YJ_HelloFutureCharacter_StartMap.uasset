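; Player character Blueprint for the start map, handling keyboard input for inventory, quest log, saving and seed planting.
; Tab toggles the inventory widget and input mode, 0 saves, and K/L or numpad keys step a clamped seed index.
; P and O line trace from the follow camera and send plant-seed or activate interface messages to the hit actor.
; The quest log input creates or clears its widget, but the add-to-canvas nodes are disconnected.
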(event `Key|Tab`
  (params (Key :type "Key Structure"))
  (bind _returnvalue (`GameplayStatics.GetPlayerController` 0))
  ;[1 1 1] Inventory System UI 띄우기
  (:`Pressed`
    (`/Engine/EditorBlueprintResources/StandardMacros.FlipFlop`
      (:`A`
        (bind _returnvalue_2 (`|CreateWidget` "/Game/YJ/UI/Inventory/WBP_Inventory.WBP_Inventory_C" (`GameplayStatics.GetPlayerController` 0)))
        (`UserWidget.AddToViewport` _returnvalue_2 0)
        (`UserWidget.SetDesiredSizeInViewport` _returnvalue_2 (0.0 0.0))
        (set `PlayerController.bShowMouseCursor` true _returnvalue)
        (`WidgetBlueprintLibrary.SetInputMode_GameAndUIEx` _returnvalue null))
      (:`B`
        (`WidgetBlueprintLibrary.SetInputMode_GameOnly` (`GameplayStatics.GetPlayerController` 0))
        (`Widget.RemoveFromParent` _returnvalue_2)))))

(event `InputAction|QuestLog`
  (params (Key :type "Key Structure"))
  (:`Pressed`
    (bind _questlogui (`self.QuestLogUI`)
      (:`then`
        (`Widget.RemoveFromParent` _questlogui)
        (set `self.QuestLogUI` null))
      (:`else`
        (bind _returnvalue (`|CreateWidget` "/Game/Oh/RealQuest/QuestUI/QuestLog_UI.QuestLog_UI_C"))
        (set `self.QuestLogUI` _returnvalue)
        (cast `/Game/YJ/Blueprints/BP_YJ_GameModeBase` (`GameplayStatics.GetGameMode`))))))

(event `Key|Zero`
  (params (Key :type "Key Structure"))
  ;[1 1 1] 게임 저장하기
  (:`Pressed`
    (`self.SaveGame_0`)))

(event `Key|P`
  (params (Key :type "Key Structure"))
  (bind _followcamera (`self.FollowCamera`))
  (bind _returnvalue (`SceneComponent.K2_GetComponentLocation` _followcamera))
  ;[1 1 1] Comment
  (:`Pressed`
    (bind _outhit (`KismetSystemLibrary.LineTraceSingle` _returnvalue (+ _returnvalue (* (`KismetMathLibrary.GetForwardVector` (`SceneComponent.K2_GetComponentRotation` _followcamera)) 1000.0)) "TraceTypeQuery1"))
    (message `/Game/Minsu/Farm/BPI_PlantSeed.BPI_PlantSeed` (`.HitActor` (`GameplayStatics.BreakHitResult` _outhit)))))

(event `Key|NumPadTwo`
  (params (Key :type "Key Structure"))
  ;[1 1 1] Comment
  (:`Pressed`
    (bind _result (`/Engine/EditorBlueprintResources/StandardMacros.IncrementInt` (`self.Seed`) :!label _label)
      (:`  `
        (set `self.Seed` (`KismetMathLibrary.Clamp` _result 0 3))))))

(event `Key|K`
  (params (Key :type "Key Structure"))
  ;[1 1 1] Comment
  (:`Pressed`
    (goto _label)))

(event `Key|L`
  (params (Key :type "Key Structure"))
  ;[1 1 1] Comment
  (:`Pressed`
    (bind _result (`/Engine/EditorBlueprintResources/StandardMacros.DecrementInt` (`self.Seed`) :!label _label_2)
      (:`  `
        (set `self.Seed` (`KismetMathLibrary.Clamp` _result 0 3))))))

(event `Key|NumPadEight`
  (params (Key :type "Key Structure"))
  ;[1 1 1] Comment
  (:`Pressed`
    (goto _label_2)))

(event `self.ReceiveBeginPlay`)

(event `Key|O`
  (params (Key :type "Key Structure"))
  (bind _followcamera (`self.FollowCamera`))
  (bind _returnvalue (`SceneComponent.K2_GetComponentLocation` _followcamera))
  ;[1 1 1] Comment
  (:`Pressed`
    (bind _outhit (`KismetSystemLibrary.LineTraceSingle` _returnvalue (+ _returnvalue (* (`KismetMathLibrary.GetForwardVector` (`SceneComponent.K2_GetComponentRotation` _followcamera)) 1000.0)) "TraceTypeQuery1"))
    (message `/Game/Minsu/Farm/BPI_Activate.BPI_Activate` (`.HitActor` (`GameplayStatics.BreakHitResult` _outhit)))))

(fn `UserConstructionScript`)