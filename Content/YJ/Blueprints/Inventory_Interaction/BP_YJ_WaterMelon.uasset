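; BP_YJ_WaterMelon is a watermelon shop item that opens a purchase widget when clicked.
; BeginPlay creates WBP_purchase, sets its fruit label to the watermelon name and price, and hides component "1".
; Collision overlap shows that component, and leaving hides it again.
; Clicking any of three body components toggles the widget, switching input to UI-only on open without restoring it on close.
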(event `self.ReceiveBeginPlay`
  (`SceneComponent.SetVisibility` (`self.1`) false false)
  (bind _returnvalue (`|CreateWidget` "/Game/Oh/BP/WBP_purchase.WBP_purchase_C"))
  (bind _output_get (set `self.PurchaseUI` _returnvalue))
  (set `/Game/Oh/BP/WBP_purchase.FruitName` "수박 1000" _output_get))

(event `self.collision.OnComponentBeginOverlap`
  (params (OverlappedComponent :type "PrimitiveComponent Object Reference") (OtherActor :type "Actor Object Reference") (OtherComp :type "PrimitiveComponent Object Reference") (OtherBodyIndex :type Integer) (bFromSweep :type Boolean) (SweepResult :type "HitResult Structure (by ref)"))
  (`SceneComponent.SetVisibility` (`self.1`) true false))

(event `self.collision.OnComponentEndOverlap`
  (params (OverlappedComponent :type "PrimitiveComponent Object Reference") (OtherActor :type "Actor Object Reference") (OtherComp :type "PrimitiveComponent Object Reference") (OtherBodyIndex :type Integer))
  (`SceneComponent.SetVisibility` (`self.1`) false false))

(event `self.body.OnClicked`
  (params (TouchedComponent :type "PrimitiveComponent Object Reference") (ButtonPressed :type "Key Structure"))
  (if (== (`self.is Show UI`) false) :!label _label
    (`WidgetBlueprintLibrary.SetInputMode_UIOnlyEx` (`GameplayStatics.GetPlayerController` 0) null)
    (`UserWidget.AddToViewport` (`self.PurchaseUI`) 0)
    (set `self.is Show UI` true)
    (else
      (`Widget.RemoveFromParent` (`self.PurchaseUI`))
      (set `self.is Show UI` false))))

(event `self.Body2.OnClicked`
  (params (TouchedComponent :type "PrimitiveComponent Object Reference") (ButtonPressed :type "Key Structure"))
  (goto _label))

(event `self.Body1.OnClicked`
  (params (TouchedComponent :type "PrimitiveComponent Object Reference") (ButtonPressed :type "Key Structure"))
  (goto _label))

(fn `UserConstructionScript`)