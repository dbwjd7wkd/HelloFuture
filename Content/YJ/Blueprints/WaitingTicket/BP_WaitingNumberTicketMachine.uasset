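; Waiting-number ticket machine actor that shows its ticket UI while the player character stands in its Box trigger.
; On begin overlap it creates and adds WBP_NumberTicketMachine to the viewport, focuses it in Game and UI input mode, and shows the mouse cursor.
; On end overlap it removes the widget and hides the cursor, without restoring the input mode.
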(event `self.Box.OnComponentBeginOverlap`
  (params (OverlappedComponent :type "PrimitiveComponent Object Reference") (OtherActor :type "Actor Object Reference") (OtherComp :type "PrimitiveComponent Object Reference") (OtherBodyIndex :type Integer) (bFromSweep :type Boolean) (SweepResult :type "HitResult Structure (by ref)"))
  ;[1 1 1] 플레이어가 overlap 되면 UI가 뜨고, overlap 이 끝나면 UI가 없어진다.
  (cast `HelloFutureCharacter` OtherActor)
  (bind _returnvalue (`|CreateWidget` "/Game/YJ/UI/WaitingTicket/WBP_NumberTicketMachine.WBP_NumberTicketMachine_C" (`GameplayStatics.GetPlayerController` 0)))
  (`UserWidget.AddToViewport` _returnvalue 0)
  (`WidgetBlueprintLibrary.SetInputMode_GameAndUIEx` (`GameplayStatics.GetPlayerController` 0) _returnvalue)
  (set `PlayerController.bShowMouseCursor` true (`GameplayStatics.GetPlayerController` 0)))

(event `self.Box.OnComponentEndOverlap`
  (params (OverlappedComponent :type "PrimitiveComponent Object Reference") (OtherActor :type "Actor Object Reference") (OtherComp :type "PrimitiveComponent Object Reference") (OtherBodyIndex :type Integer))
  ;[1 1 1] 플레이어가 overlap 되면 UI가 뜨고, overlap 이 끝나면 UI가 없어진다.
  (cast `HelloFutureCharacter` OtherActor)
  (`Widget.RemoveFromParent` (stale `self.Box.OnComponentBeginOverlap` _returnvalue))
  (set `PlayerController.bShowMouseCursor` false (`GameplayStatics.GetPlayerController` 0)))

(fn `UserConstructionScript`)