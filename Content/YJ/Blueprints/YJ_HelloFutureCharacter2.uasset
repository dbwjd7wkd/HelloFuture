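; Player character for a farming and quest game, handling interaction, UI toggles and farm-tile input.
; Interaction overlaps attach a prompt widget, whose owner's attached quest actors feed dialogue widgets into the GameMode's HUD; other inputs toggle inventory and quest log.
; Keys cycle a clamped seed index, and camera line traces send plant, activate or fertilize interface messages.
; Shift's sprint handlers zero walk speed while held, mirroring changes locally and in server-intended events.
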(event `Key|LeftShift`
  (params (Key :type "Key Structure"))
  (bind _charactermovement (`self.CharacterMovement`))
  ;[1 1 1] 서버 연동 예
  ;;[1 1 1] 로컬 클라이언트 코드를 바꿈
  (:`Pressed`
    (`self.StartSprinting`)
    (set `CharacterMovementComponent.MaxWalkSpeed` 0.0 _charactermovement))
  (:`Released`
    (`self.StopSprintting`)
    (set `CharacterMovementComponent.MaxWalkSpeed` 1000.0 _charactermovement)))

(event `self.Interaction.OnComponentBeginOverlap`
  (params (OverlappedComponent :type "PrimitiveComponent Object Reference") (OtherActor :type "Actor Object Reference") (OtherComp :type "PrimitiveComponent Object Reference") (OtherBodyIndex :type Integer) (bFromSweep :type Boolean) (SweepResult :type "HitResult Structure (by ref)"))
  (bind _returnvalue (`AddComponent|NODE_AddWidgetComponent-0`))
  (set `self.InteractMessage` _returnvalue)
  (`SceneComponent.K2_AttachToComponent` _returnvalue OtherComp "None" "KeepRelative" "KeepRelative" "KeepRelative" true))

(event `StartSprinting`
  ;[1 1 1] 서버 연동 예
  ;;[1 1 1] 서버 코드만 바꿈
  (set `CharacterMovementComponent.MaxWalkSpeed` 0.0 (`self.CharacterMovement`)))

(event `self.Interaction.OnComponentEndOverlap`
  (params (OverlappedComponent :type "PrimitiveComponent Object Reference") (OtherActor :type "Actor Object Reference") (OtherComp :type "PrimitiveComponent Object Reference") (OtherBodyIndex :type Integer))
  (bind _interactmessage (`self.InteractMessage`)
    (:`then`
      (`ActorComponent.K2_DestroyComponent` _interactmessage)
      (set `self.InteractMessage` null))
    (:`else`)))

(event `StopSprintting`
  ;[1 1 1] 서버 연동 예
  ;;[1 1 1] 서버 코드만 바꿈
  (set `CharacterMovementComponent.MaxWalkSpeed` 1000.0 (`self.CharacterMovement`)))

(event `InputAction|Interact`
  (params (Key :type "Key Structure"))
  (:`Pressed`
    (bind _interactmessage (`self.InteractMessage`)
      (:`then`
        (for _array_element (`self.GetAttachedActors` (`ActorComponent.GetOwner` (`SceneComponent.GetAttachParent` _interactmessage)) true)
          (bind _asoh_real_quest (cast `/Game/Oh/RealQuest/Quests/OH_RealQuest` _array_element))
          (bind _returnvalue (`|CreateWidget` "/Game/Oh/RealQuest/QuestUI/Quset__UI.Quset__UI_C" null _asoh_real_quest))
          (bind _asbp_hello_future_game_mode (cast `/Game/BP_HelloFutureGameMode` (`GameplayStatics.GetGameMode`)))
          (bind _returnvalue_2 (`CanvasPanel.AddChildToCanvas` (`/Game/Oh/RealQuest/QuestUI/HUD_UI.QuestDialogue_Holder` (`/Game/BP_HelloFutureGameMode.HUD_Widget` _asbp_hello_future_game_mode)) _returnvalue))
          (`CanvasPanelSlot.SetAutoSize` _returnvalue_2 true)))
      (:`else`))))

(event `Key|Tab`
  (params (Key :type "Key Structure"))
  (bind _returnvalue (`GameplayStatics.GetPlayerController` 0))
  ;[1 1 1] Inventory System UI 띄우기
  (:`Pressed`
    (`/Engine/EditorBlueprintResources/StandardMacros.FlipFlop`
      (:`A`
        (bind _returnvalue_2 (`|CreateWidget` "/Game/YJ/UI/Inventory/WBP_Inventory.WBP_Inventory_C" (`GameplayStatics.GetPlayerController` 0)))
        (`UserWidget.AddToViewport` _returnvalue_2 0)
        (`UserWidget.SetDesiredSizeInViewport` _returnvalue_2 (0.0 0.0))
        (set `PlayerController.bShowMouseCursor` true _returnvalue)
        (`WidgetBlueprintLibrary.SetInputMode_GameAndUIEx` _returnvalue null))
      (:`B`
        (`WidgetBlueprintLibrary.SetInputMode_GameOnly` (`GameplayStatics.GetPlayerController` 0))
        (`Widget.RemoveFromParent` _returnvalue_2)))))

(event `InputAction|QuestLog`
  (params (Key :type "Key Structure"))
  ;[1 1 1] Quest UI Input
  (:`Pressed`
    (bind _questlogui (`self.QuestLogUI`)
      (:`then`
        (`Widget.RemoveFromParent` _questlogui)
        (set `self.QuestLogUI` null))
      (:`else`
        (bind _returnvalue (`|CreateWidget` "/Game/Oh/RealQuest/QuestUI/QuestLog_UI.QuestLog_UI_C"))
        (set `self.QuestLogUI` _returnvalue)
        (bind _asbp_hello_future_game_mode (cast `/Game/BP_HelloFutureGameMode` (`GameplayStatics.GetGameMode`)))
        (bind _returnvalue_2 (`CanvasPanel.AddChildToCanvas` (`/Game/BP_HelloFutureGameMode.HUD Canvas` _asbp_hello_future_game_mode) (`self.QuestLogUI`)))
        (`CanvasPanelSlot.SetAnchors` _returnvalue_2 (make `Anchors` (0.0 0.0) (1.0 1.0)))))))

(event `self.ReceiveBeginPlay`)

(event `Key|P`
  (params (Key :type "Key Structure"))
  (bind _followcamera (`self.FollowCamera`))
  (bind _returnvalue (`SceneComponent.K2_GetComponentLocation` _followcamera))
  ;[1 1 1] Comment
  (:`Pressed`
    (bind _outhit (`KismetSystemLibrary.LineTraceSingle` _returnvalue (+ _returnvalue (* (`KismetMathLibrary.GetForwardVector` (`SceneComponent.K2_GetComponentRotation` _followcamera)) 1000.0)) "TraceTypeQuery1"))
    (message `/Game/Minsu/Farm/BPI_PlantSeed.BPI_PlantSeed` (`.HitActor` (`GameplayStatics.BreakHitResult` _outhit)))))

(event `Key|NumPadTwo`
  (params (Key :type "Key Structure"))
  ;[1 1 1] Comment
  (:`Pressed`
    (bind _result (`/Engine/EditorBlueprintResources/StandardMacros.IncrementInt` (`self.Seed`) :!label _label)
      (:`  `
        (set `self.Seed` (`KismetMathLibrary.Clamp` _result 0 3))))))

(event `Key|K`
  (params (Key :type "Key Structure"))
  ;[1 1 1] Comment
  (:`Pressed`
    (goto _label)))

(event `Key|L`
  (params (Key :type "Key Structure"))
  ;[1 1 1] Comment
  (:`Pressed`
    (bind _result (`/Engine/EditorBlueprintResources/StandardMacros.DecrementInt` (`self.Seed`) :!label _label_2)
      (:`  `
        (set `self.Seed` (`KismetMathLibrary.Clamp` _result 0 3))))))

(event `Key|NumPadEight`
  (params (Key :type "Key Structure"))
  ;[1 1 1] Comment
  (:`Pressed`
    (goto _label_2)))

(event `Key|O`
  (params (Key :type "Key Structure"))
  (bind _followcamera (`self.FollowCamera`))
  (bind _returnvalue (`SceneComponent.K2_GetComponentLocation` _followcamera))
  ;[1 1 1] Comment
  (:`Pressed`
    (bind _outhit (`KismetSystemLibrary.LineTraceSingle` _returnvalue (+ _returnvalue (* (`KismetMathLibrary.GetForwardVector` (`SceneComponent.K2_GetComponentRotation` _followcamera)) 1000.0)) "TraceTypeQuery1"))
    (bind (_bblockinghit _binitialoverlap _time _distance _location _impactpoint _normal _impactnormal _physmat _hitactor) (`GameplayStatics.BreakHitResult` _outhit))
    (if (`/Game/Minsu/Farm/BP/BP_FarmTile.IsSomethingPlanted?` (cast `/Game/Minsu/Farm/BP/BP_FarmTile` _hitactor :!pure true))
      (message `/Game/Minsu/Farm/BPI_Activate.BPI_Activate` _hitactor)
      (else
        (message `/Game/Minsu/Farm/BPI_Fertilizer.BPI_Fertilizer` _hitactor)))))

(fn `UserConstructionScript`)