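; Bank teller actor that opens a consultation start screen when a player walks up on their turn.
; On Box overlap by a HelloFutureCharacter, it asks YJ_GameModeBase through CheckMyOrder whether that character is next in the consultation order.
; If so, it adds WBP_BankTeller_Start to the viewport for player controller 0, switches input to Game and UI focused on the widget, and shows the cursor.
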(event `self.Box.OnComponentBeginOverlap`
  (params (OverlappedComponent :type "PrimitiveComponent Object Reference") (OtherActor :type "Actor Object Reference") (OtherComp :type "PrimitiveComponent Object Reference") (OtherBodyIndex :type Integer) (bFromSweep :type Boolean) (SweepResult :type "HitResult Structure (by ref)"))
  ;[1 1 1] overlap 된게 플레이어면 진행
  (bind _ashello_future_character (cast `HelloFutureCharacter` OtherActor))
  ;[1 1 1] 상담 순서가 맞으면 진행
  (bind _asyj_game_mode_base (cast `YJ_GameModeBase` (`GameplayStatics.GetGameMode`)))
  (bind _returnvalue (`YJ_GameModeBase.CheckMyOrder` _asyj_game_mode_base _ashello_future_character))
  (if _returnvalue
    ;[1 1 1] 상담 시작 UI 뜨기
    (bind _returnvalue_2 (`|CreateWidget` "/Game/YJ/UI/WBP_BankTeller_Start.WBP_BankTeller_Start_C" (`GameplayStatics.GetPlayerController` 0)))
    (`UserWidget.AddToViewport` _returnvalue_2 0)
    (`WidgetBlueprintLibrary.SetInputMode_GameAndUIEx` (`GameplayStatics.GetPlayerController` 0) _returnvalue_2)
    (set `PlayerController.bShowMouseCursor` true (`GameplayStatics.GetPlayerController` 0))))

(fn `UserConstructionScript`)