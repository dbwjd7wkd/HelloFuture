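; BP_NPC is an NPC that shows the bank dialog widget WBP_BankNPC while the player is near, in a DialogueSystem folder marked for deletion.
; Capsule begin overlap by a HelloFutureCharacter creates the widget, switches input to Game and UI focused on it, and shows the mouse cursor.
; End overlap restores game-only input and removes the widget, but leaves the cursor flag set.
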(event `self.CapsuleComponent.OnComponentBeginOverlap`
  (params (OverlappedComponent :type "PrimitiveComponent Object Reference") (OtherActor :type "Actor Object Reference") (OtherComp :type "PrimitiveComponent Object Reference") (OtherBodyIndex :type Integer) (bFromSweep :type Boolean) (SweepResult :type "HitResult Structure (by ref)"))
  ;[1 1 1] overlap 된게 플레이어면 진행
  (cast `HelloFutureCharacter` OtherActor)
  ;[1 1 1] UI 띄우기
  (bind _returnvalue (`|CreateWidget` "/Game/YJ/UI/BackNPC/WBP_BankNPC.WBP_BankNPC_C" (`GameplayStatics.GetPlayerController` 0)))
  (`UserWidget.AddToViewport` _returnvalue 0)
  (`WidgetBlueprintLibrary.SetInputMode_GameAndUIEx` (`GameplayStatics.GetPlayerController` 0) _returnvalue)
  (set `PlayerController.bShowMouseCursor` true (`GameplayStatics.GetPlayerController` 0)))

(event `self.CapsuleComponent.OnComponentEndOverlap`
  (params (OverlappedComponent :type "PrimitiveComponent Object Reference") (OtherActor :type "Actor Object Reference") (OtherComp :type "PrimitiveComponent Object Reference") (OtherBodyIndex :type Integer))
  (cast `HelloFutureCharacter` OtherActor)
  (`/Engine/EditorBlueprintResources/StandardMacros.IsValid` (stale `self.CapsuleComponent.OnComponentBeginOverlap` _returnvalue)
    (:`Is Valid`
      (`WidgetBlueprintLibrary.SetInputMode_GameOnly` (`GameplayStatics.GetPlayerController` 0))
      (`Widget.RemoveFromParent` (stale `self.CapsuleComponent.OnComponentBeginOverlap` _returnvalue)))))

(fn `UserConstructionScript`)