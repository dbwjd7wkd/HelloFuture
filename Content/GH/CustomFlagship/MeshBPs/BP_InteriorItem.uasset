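; BP_InteriorItem is a clickable furniture actor for the custom flagship interior that is removed by a double-click.
; Mesh clicks raise a counter and restart a timer, which Tick uses to clear the count after half a second without another click.
; A second click within that window calls DestroyFurniture, which destroys whichever actor a cursor visibility trace hits rather than referencing itself.
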(event `self.ReceiveTick`
  (params (DeltaSeconds :type "Float (single-precision)"))
  (if (>= (`self.clickedNum`) 1)
    (set `self.currentTime` (+ DeltaSeconds (`self.currentTime`)))
    (if (and (> (`self.currentTime`) 0.5) (>= (`self.clickedNum`) 1))
      (set `self.clickedNum` 0)
      (set `self.currentTime` 0.0))))

(event `self.StaticMesh.OnClicked`
  (params (TouchedComponent :type "PrimitiveComponent Object Reference") (ButtonPressed :type "Key Structure"))
  (set `self.currentTime` 0.0)
  (set `self.clickedNum` (+ (`self.clickedNum`) 1))
  (if (>= (`self.clickedNum`) 2)
    (`self.DestroyFurniture`)))

(event `DestroyFurniture`
  (`self.K2_DestroyActor` (`.HitActor` (`GameplayStatics.BreakHitResult` (`PlayerController.GetHitResultUnderCursorByChannel` (`GameplayStatics.GetPlayerController` 0) "TraceTypeQuery1" true))))
  (set `self.clickedNum` 0))

(fn `UserConstructionScript`)