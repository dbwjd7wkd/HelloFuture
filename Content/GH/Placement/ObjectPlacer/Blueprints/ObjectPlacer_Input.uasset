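; Actor that controls interactive object placement: begin, rotate by yaw snap, cancel or finish, with a live preview object and floor indicator.
; BeginPlacing spawns the given class at BP_Floor's location and selects the ground or wall engine from its placement type.
; While placing, Tick runs that engine, moves the preview to its computed location, fits the indicator and shows blocked or unblocked state.
; Finishing requires a valid spot; cancelling destroys the preview.
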(event `Rotation +`
  ;[0.9453 1 0] Rotation
  (if (`self.IsPlacing`)
    (bind _objectplacer_actor (`self.ObjectPlacer Actor`)
      (:`then`
        (`/Game/GH/Placement/ObjectPlacer/Blueprints/ObjectPlacer_Actor.Rotate Z` _objectplacer_actor (`self.Yaw Rotation Snap`)))
      (:`else`))))

(event `Rotation -`
  ;[0.9453 1 0] Rotation
  (if (`self.IsPlacing`)
    (bind _objectplacer_actor (`self.ObjectPlacer Actor`)
      (:`then`
        (`/Game/GH/Placement/ObjectPlacer/Blueprints/ObjectPlacer_Actor.Rotate Z` _objectplacer_actor (* (`self.Yaw Rotation Snap`) -1.0)))
      (:`else`))))

(event `self.ReceiveBeginPlay`
  (`|ExecutionSequence`
    (:`then_0`
      (set `self.Player Camera Manager` (`GameplayStatics.GetPlayerCameraManager` 0)))
    (:`then_1`
      (bind _returnvalue (`|SpawnActorFromClass` "/Game/GH/Placement/ObjectPlacer/Blueprints/ObjectPlacer_FloorIndicator.ObjectPlacer_FloorIndicator_C" (`KismetMathLibrary.MakeTransform` (0.0 0.0 0.0)) "Undefined" "OverrideRootScale" null null))
      (set `self.Floor Indicator` _returnvalue)
      (`KismetSystemLibrary.PrintString` "Hello"))))

(event `Update Indicator Transform Tick`
  (bind (_mesh_pivot_offset_x _mesh_pivot_offset_y) (`KismetMathLibrary.BreakVector` (`/Game/GH/Placement/ObjectPlacer/Blueprints/ObjectPlacer_Engine_Base.Mesh Pivot Offset` (`self.ObjectPlacer_WorkingEngine`))))
  (bind (_returnvalue_x _returnvalue_y _returnvalue_z) (`KismetMathLibrary.BreakVector` (* (`/Game/GH/Placement/ObjectPlacer/Blueprints/ObjectPlacer_Engine_Base.Box Half Size` (`self.ObjectPlacer_WorkingEngine`)) 0.02)))
  (bind (_returnvalue_x_2 _returnvalue_y_2) (`KismetMathLibrary.BreakVector` (* (`/Game/GH/Placement/ObjectPlacer/Blueprints/ObjectPlacer_Engine_Base.Box Half Size` (`self.ObjectPlacer_WorkingEngine`)) 0.02)))
  (bind (_relativerotation_roll _relativerotation_pitch _relativerotation_yaw) (`KismetMathLibrary.BreakRotator` (`SceneComponent.RelativeRotation` (`/Game/GH/Placement/ObjectPlacer/Blueprints/ObjectPlacer_Actor.MeshesRoot` (`self.ObjectPlacer Actor`)))))
  (`|ExecutionSequence`
    (:`then_0`
      (`self.K2_AttachToActor` (`self.Floor Indicator`) (`self.ObjectPlacer Actor`) "None" "KeepWorld" "KeepWorld" "KeepWorld" true))
    (:`then_1`
      (switch `/Game/GH/Placement/ObjectPlacer/Blueprints/EObjectPlacementType` (`self.ObjectPlacement Type`)
        (:`NewEnumerator0`
          (`self.K2_SetActorRelativeLocation` (`self.Floor Indicator`) (`KismetMathLibrary.MakeVector` _mesh_pivot_offset_x _mesh_pivot_offset_y (.z (`/Game/GH/Placement/ObjectPlacer/Blueprints/ObjectPlacer_Actor.Get Box Bound Vector` (`self.ObjectPlacer Actor`)))) false false)
          (`self.SetActorRelativeScale3D` (`self.Floor Indicator`) (`KismetMathLibrary.MakeVector` _returnvalue_x_2 _returnvalue_y_2 1.0)))
        (:`NewEnumerator1`
          (`self.K2_SetActorRelativeTransform` (`self.Floor Indicator`) (`KismetMathLibrary.MakeTransform` (0.0 0.0 0.0) (`KismetMathLibrary.MakeRotator` 0.0 -90.0 _relativerotation_yaw) (`KismetMathLibrary.MakeVector` _returnvalue_z _returnvalue_y 1.0)) false false))))))

(event `Begin Placing`
  (params (Class :type "/Game/GH/Placement/ObjectPlacer/Blueprints/ObjectPlacer_Actor Class Reference"))
  ;[0 1 0.3203] Control
  (`self.Player Camera Manager`
    (:`then`
      (if (`KismetSystemLibrary.IsValidClass` Class)
        (if (not (`self.IsPlacing`))
          (`|ExecutionSequence`
            (:`then_0`
              (bind _returnvalue (`GameplayStatics.GetActorOfClass` "/Game/GH/Flagship/BP_Floor.BP_Floor_C"))
              (bind _output_get (set `self.location` (`SceneComponent.K2_GetComponentLocation` (`/Game/GH/Flagship/BP_Floor.DefaultSceneRoot` _returnvalue))))
              (`KismetSystemLibrary.PrintString` (`KismetStringLibrary.Conv_VectorToString` _output_get) true true (struct :`G` 0.66 :`B` 1.0 :`A` 1.0) 20.0))
            (:`then_1`
              (bind _returnvalue_2 (`|SpawnActorFromClass` Class (`KismetMathLibrary.MakeTransform` (`self.location`)) "Undefined" "OverrideRootScale" (`self.GetOwner`) null))
              (set `self.ObjectPlacer Actor` _returnvalue_2))
            (:`then_2`
              (`|ExecutionSequence`
                (:`then_0`
                  (`self.K2_SetActorRelativeTransform` (`self.Floor Indicator`) (`KismetMathLibrary.MakeTransform` (`self.location`)) false false))
                (:`then_1`
                  (set `self.ObjectPlacement Type` (`/Game/GH/Placement/ObjectPlacer/Blueprints/ObjectPlacer_Actor.Object Placement Type` (`self.ObjectPlacer Actor`)))
                  (switch `/Game/GH/Placement/ObjectPlacer/Blueprints/EObjectPlacementType` (`self.ObjectPlacement Type`)
                    (:`NewEnumerator0`
                      (set `self.ObjectPlacer_WorkingEngine` (`self.ObjectPlacer_Engine_Ground`)))
                    (:`NewEnumerator1`
                      (set `self.ObjectPlacer_WorkingEngine` (`self.ObjectPlacer_Engine_Wall`)))))
                (:`then_2`
                  (`/Game/GH/Placement/ObjectPlacer/Blueprints/ObjectPlacer_Engine_Base.Setup Parameters` (`self.ObjectPlacer_WorkingEngine`)))
                (:`then_3`
                  (`/Game/GH/Placement/ObjectPlacer/Blueprints/ObjectPlacer_Actor.Preview Mode` (`self.ObjectPlacer Actor`)))
                (:`then_4`
                  (`self.SetActorTickEnabled` true)
                  (set `self.IsPlacing` true))
                (:`then_5`
                  (`/Game/GH/Placement/ObjectPlacer/Blueprints/ObjectPlacer_FloorIndicator.Show` (`self.Floor Indicator`)))))))))
    (:`else`)))

(event `self.ReceiveTick`
  (params (DeltaSeconds :type "Float (single-precision)"))
  (`|ExecutionSequence`
    (:`then_0`
      (`/Game/GH/Placement/ObjectPlacer/Blueprints/ObjectPlacer_Engine_Base.Engine Tick` (`self.ObjectPlacer_WorkingEngine`)))
    (:`then_1`
      (`|ExecutionSequence`
        (:`then_0`
          (`self.Update Indicator Transform Tick`))
        (:`then_1`
          (if (`/Game/GH/Placement/ObjectPlacer/Blueprints/ObjectPlacer_Engine_Base.Spot is Valid` (`self.ObjectPlacer_WorkingEngine`))
            (bind _objectplacer_actor (`self.ObjectPlacer Actor`)
              (:`then`
                (`/Game/GH/Placement/ObjectPlacer/Blueprints/ObjectPlacer_Actor.Preview Unblocked` _objectplacer_actor)
                (`/Game/GH/Placement/ObjectPlacer/Blueprints/ObjectPlacer_FloorIndicator.Unblocked` (`self.Floor Indicator`)))
              (:`else`))
            (else
              (bind _objectplacer_actor_2 (`self.ObjectPlacer Actor`)
                (:`then`
                  (`/Game/GH/Placement/ObjectPlacer/Blueprints/ObjectPlacer_Actor.Preview Blocked` _objectplacer_actor_2)
                  (`/Game/GH/Placement/ObjectPlacer/Blueprints/ObjectPlacer_FloorIndicator.Blocked` (`self.Floor Indicator`)))
                (:`else`)))))
        (:`then_2`
          (bind _objectplacer_actor_3 (`self.ObjectPlacer Actor`)
            (:`then`
              (`SceneComponent.K2_SetWorldLocation` (`Actor.RootComponent` _objectplacer_actor_3) (`/Game/GH/Placement/ObjectPlacer/Blueprints/ObjectPlacer_Engine_Base.Final Placement Location` (`self.ObjectPlacer_WorkingEngine`)) false false))
            (:`else`)))))))

(event `Cancel Place`
  ;[0 1 0.3203] Control
  (if (`self.IsPlacing`)
    (`|ExecutionSequence`
      (:`then_0`
        (bind _objectplacer_actor (`self.ObjectPlacer Actor`)
          (:`then`
            (`self.K2_DestroyActor` _objectplacer_actor))
          (:`else`)))
      (:`then_1`
        (`self.SetActorTickEnabled` false)
        (set `self.IsPlacing` false))
      (:`then_2`
        (`/Game/GH/Placement/ObjectPlacer/Blueprints/ObjectPlacer_FloorIndicator.Hide` (`self.Floor Indicator`))))))

(event `Finish Placing`
  ;[0 1 0.3203] Control
  (if (`self.IsPlacing`)
    (if (`/Game/GH/Placement/ObjectPlacer/Blueprints/ObjectPlacer_Engine_Base.Spot is Valid` (`self.ObjectPlacer_WorkingEngine`))
      (`|ExecutionSequence`
        (:`then_0`
          (bind _objectplacer_actor (`self.ObjectPlacer Actor`)
            (:`then`
              (`/Game/GH/Placement/ObjectPlacer/Blueprints/ObjectPlacer_Actor.Placed Mode` _objectplacer_actor)
              (set `self.ObjectPlacer Actor` null))
            (:`else`)))
        (:`then_1`
          (`self.SetActorTickEnabled` false)
          (set `self.IsPlacing` false))
        (:`then_2`
          (`/Game/GH/Placement/ObjectPlacer/Blueprints/ObjectPlacer_FloorIndicator.Hide` (`self.Floor Indicator`)))))))

(fn `UserConstructionScript`
  (`|ExecutionSequence`))