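; Math helper function library for the ObjectPlacer placement system, covering rounding, sign and axis utilities for floats and vectors.
; Custom rounding snaps values to multiples of a given size, stepping up or down by flag or by the value's sign, with the vector version working per component.
; Other helpers round toward or away from zero, pick the smaller non-zero magnitude, find maximum elements and extract per-component signs.
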(fn `Custom Round Float`
  (params (A :type "Float (double-precision)") (Size :type "Float (double-precision)") (bRoundUp :type Boolean))
  (returns (ReturnValue :type "Float (double-precision)"))
  (locals (`Temporary Integer` :type Integer))
  (bind (_remainder _returnvalue) (`KismetMathLibrary.FMod` A Size))
  (bind _temporary_integer (`local.Temporary Integer`))
  (set `local.Temporary Integer` _returnvalue)
  (`|ExecutionSequence`
    (:`then_0`
      (if (!= _remainder 0.0)
        (if bRoundUp
          (`/Engine/EditorBlueprintResources/StandardMacros.IncrementInt` _temporary_integer)
          (else
            (`/Engine/EditorBlueprintResources/StandardMacros.DecrementInt` _temporary_integer)))))
    (:`then_1`
      (return (* (`local.Temporary Integer`) Size)))))

(fn `Custom Round Float Sign`
  (params (A :type "Float (double-precision)") (Size :type "Float (double-precision)"))
  (returns (ReturnValue :type "Float (double-precision)"))
  (return (`self.Custom Round Float` A Size (> (`KismetMathLibrary.SignOfFloat` A) 0.0))))

(fn `Custom Round Vector`
  (params (A :type "Vector Structure") (Size :type "Float (double-precision)") (bRoundUp :type Boolean))
  (returns (ReturnValue :type "Vector Structure"))
  (return (`KismetMathLibrary.MakeVector` (`self.Custom Round Float` (.x A) Size bRoundUp) (`self.Custom Round Float` (.y A) Size bRoundUp) (`self.Custom Round Float` (.z A) Size bRoundUp))))

(fn `Get Abs Min Except Zero`
  (params (A :type "Float (double-precision)") (B :type "Float (double-precision)"))
  (returns (ReturnValue :type "Float (double-precision)"))
  (if (`KismetMathLibrary.NearlyEqual_FloatFloat` A 0.0 0.001)
    (return B)
    (elif (`KismetMathLibrary.NearlyEqual_FloatFloat` B 0.0 0.001)
      (return A)
      (else
        (return (select `bool` (> (`KismetMathLibrary.Abs` A) (`KismetMathLibrary.Abs` B)) :`false` A :`true` B))))))

(fn `Get Max Element+`
  (params (A :type "Vector Structure"))
  (returns (`Return Value` :type "Float (double-precision)") (Axis :type Byte))
  (bind _returnvalue (`KismetMathLibrary.GetMaxElement` A))
  (return _returnvalue (select `bool` (== _returnvalue (.x A)) :`false` (select `bool` (== _returnvalue (.y A)) :!type "Byte"))))

(fn `Get Vector Element by Max Element Of Sample`
  (params (Sample :type "Vector Structure") (Target :type "Vector Structure"))
  (returns (`Return Value` :type "Float (double-precision)"))
  (return (select `byte` (`.Axis` (`self.Get Max Element+` Sample)) :`0` 0.0 :`1` 0.0 :`2` 0.0 :!type "Float (single-precision)")))

(fn `Get Vector Sign with 0`
  (params (A :type "Vector Structure"))
  (returns (`Return Value` :type "Vector Structure"))
  (return (`KismetMathLibrary.MakeVector` (`KismetMathLibrary.SignOfFloat` A_X) (`KismetMathLibrary.SignOfFloat` A_Y) (`KismetMathLibrary.SignOfFloat` A_Z))))

(fn `Round Float Sign`
  (params (A :type "Float (double-precision)") (Inverse :type Boolean))
  (returns (ReturnValue :type "Float (double-precision)"))
  (return (`KismetMathLibrary.Conv_IntToDouble` (select `bool` Inverse :`false` (select `bool` (> A 0.0) :`false` (`KismetMathLibrary.FFloor` A) :`true` (`KismetMathLibrary.FCeil` A)) :`true` (select `bool` (> A 0.0) :`false` (`KismetMathLibrary.FCeil` A) :`true` (`KismetMathLibrary.FFloor` A))))))