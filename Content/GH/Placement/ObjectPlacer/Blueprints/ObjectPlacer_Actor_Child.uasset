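; Child Blueprint of an object placer actor that changes its static mesh's look between preview and placed states.
; It overrides the preview and placed mode implementation events to assign materials to the mesh's two slots.
; The first slot gets the same material in both modes, while the second differs in preview and matches the first once placed.
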(event `self.Preview Mode Implementation`
  (bind _staticmesh (`self.StaticMesh`))
  (`PrimitiveComponent.SetMaterial` _staticmesh 0 "/Game/Assets/DELIVERY/01_-_Default.01_-_Default")
  (`PrimitiveComponent.SetMaterial` _staticmesh 1 "/Game/Assets/Train/rail/14_-_Default.14_-_Default"))

(event `self.Placed Mode Implementation`
  (bind _staticmesh (`self.StaticMesh`))
  (`PrimitiveComponent.SetMaterial` _staticmesh 0 "/Game/Map/Asset/01_-_Default.01_-_Default")
  (`PrimitiveComponent.SetMaterial` _staticmesh 1 "/Game/Assets/Train/Train/01_-_Default.01_-_Default"))

(fn `UserConstructionScript`
  (`parent.UserConstructionScript`))