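; Floor indicator Blueprint for the object placer, showing whether a placement spot is blocked.
; Show and Hide events toggle the FloorIndicator component's visibility.
; Blocked and Unblocked events recolor it by setting the material's Emissive Color vector parameter to red or green.
; BeginPlay, Tick and the construction script are empty, so all changes come through these events.
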(event `self.ReceiveBeginPlay`)

(event `self.ReceiveTick`
  (params (DeltaSeconds :type "Float (single-precision)")))

(event `Show`
  (`SceneComponent.SetVisibility` (`self.FloorIndicator`) true false))

(event `Hide`
  (`SceneComponent.SetVisibility` (`self.FloorIndicator`) false false))

(event `Unblocked`
  (`MeshComponent.SetVectorParameterValueOnMaterials` (`self.FloorIndicator`) "Emissive Color" (0.0 1.0 0.0)))

(event `Blocked`
  (`MeshComponent.SetVectorParameterValueOnMaterials` (`self.FloorIndicator`) "Emissive Color" (1.0 0.0 0.0)))

(fn `UserConstructionScript`)