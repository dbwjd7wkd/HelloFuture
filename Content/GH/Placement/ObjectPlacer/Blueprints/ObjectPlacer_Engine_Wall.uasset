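; Wall variant of the ObjectPlacer engine that overrides placement setup and tracing for objects standing on the ground.
; Setup resets pivot offsets, assumes an upward surface normal and marks the spot valid.
; Camera hits are checked for flat ground, with downward fallback traces for non-ground hits and misses.
; Direction helpers map the two working axes to X and Y, and surface-normal rotation of the trace box is disabled.
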(event `self.ReceiveBeginPlay`
  (`parent.ReceiveBeginPlay`))

(event `self.ReceiveTick`
  (params (DeltaSeconds :type "Float (single-precision)"))
  (`parent.ReceiveTick` DeltaSeconds))

(fn `Camera Trace Result Function`
  (params (`Out Hit` :type "HitResult Structure"))
  (bind (_bblockinghit _binitialoverlap _time _distance _location _impactpoint _normal _impactnormal _physmat _hitactor _hitcomponent _hitbonename _hititem _faceindex _tracestart _traceend) (`GameplayStatics.BreakHitResult` `Out Hit`))
  (bind _returnvalue (+ _impactpoint (* _impactnormal 1.0)))
  (if _bblockinghit
    (if (`KismetMathLibrary.NearlyEqual_FloatFloat` (.z _impactnormal) 1.0 0.01)
      ;[1 0 0.1406] If the camera trace hit gound, set [Box Trace Location] location to the hit location.
      (`|ExecutionSequence`
        (:`then_0`)
        (:`then_1`
          (`KismetArrayLibrary.Array_AddUnique` (`self.Actors to Ignore`) _hitactor)))
      (else
        ;[1 0.1172 0] If the camera trace doesn't hit ground, add Z trace to ground.
        (bind _outhit (`self.Camera Line Trace Function` _returnvalue (+ _returnvalue (0.0 0.0 -2500.0)) false (`self.Actors to Ignore`)))
        (if (`GameplayStatics.BreakHitResult` _outhit)
          (`|ExecutionSequence`))))
    (else
      ;[0.7578 1 0] If the camera trace doesn't hit, use another line trace for tracing floor
      (bind _outhit_2 (`self.Camera Line Trace Function` _traceend (- _traceend (`KismetMathLibrary.MakeVector` 0.0 0.0 (`self.Z Extra Trace Length`))) false (`self.Actors to Ignore`)))
      (if (`GameplayStatics.BreakHitResult` _outhit_2)
        (`|ExecutionSequence`)))))

(fn `Direction 1 - Assign Float to Vector`
  (params (Float :type "Float (double-precision)"))
  (returns (`Return Value` :type "Vector Structure"))
  (return (`KismetMathLibrary.MakeVector` Float)))

(fn `Direction 1 - Split Vector to Float`
  (params (Vector :type "Vector Structure"))
  (returns (`Return Value` :type "Float (double-precision)"))
  (return Vector_X))

(fn `Direction 1 - Trace Box Working Axis`
  (returns (Direction :type "Vector Structure"))
  (return (0.0 0.0 0.0)))

(fn `Direction 1 - Trace Box Working Axis - Float to Vector`
  (params (A :type "Float (double-precision)"))
  (returns (`Return Value` :type "Vector Structure"))
  (return (`KismetMathLibrary.MakeVector` A)))

(fn `Direction 1 - Trace Box Working Axis - Vector to Float`
  (params (Vector :type "Vector Structure"))
  (returns (`Return Value` :type "Float (double-precision)"))
  (return Vector_X))

(fn `Direction 2 - Assign Float to Vector`
  (params (Float :type "Float (double-precision)"))
  (returns (`Return Value` :type "Vector Structure"))
  (return (`KismetMathLibrary.MakeVector` 0.0 Float)))

(fn `Direction 2 - Split Vector to Float`
  (params (Vector :type "Vector Structure"))
  (returns (`Return Value` :type "Float (double-precision)"))
  (return Vector_Y))

(fn `Direction 2 - Trace Box Working Axis`
  (returns (Direction :type "Vector Structure"))
  (return (0.0 0.0 0.0)))

(fn `Direction 2 - Trace Box Working Axis - Float to Vector`
  (params (A :type "Float (double-precision)"))
  (returns (`Return Value` :type "Vector Structure"))
  (return (`KismetMathLibrary.MakeVector` 0.0 A)))

(fn `Direction 2 - Trace Box Working Axis - Vector to Float`
  (params (Vector :type "Vector Structure"))
  (returns (`Return Value` :type "Float (double-precision)"))
  (return Vector_Y))

(fn `Setup Variables`
  (`self.Object Placer Actor`
    (:`then`
      (`|ExecutionSequence`
        (:`then_0`
          (if (`self.Snap to Grid`)
            ;[1 0.6797 0] Add [Box half Size] of [ObjectPlacer Actor] to simulate the object position.
            (`|ExecutionSequence`)
            (else
              (`|ExecutionSequence`
                (:`then_0`
                  (set `self.Mesh Pivot Offset` (`KismetMathLibrary.MakeVector` 0.0 0.0 (.z (0.0 0.0 0.0)))))
                (:`then_1`
                  (set `self.Box Half Size` (0.0 0.0 0.0)))))))
        (:`then_1`
          (set `self.Box Trace Location` (+ (`self.Mesh Pivot Offset`) (`self.Box Trace Location`))))
        (:`then_2`
          (set `self.Placement Mesh Pivot Offset` (`KismetMathLibrary.MakeVector` 0.0 0.0 (.z (0.0 0.0 0.0)))))
        (:`then_3`
          (set `self.Camera Trace Surface Normal` (0.0 0.0 1.0))
          (set `self.Spot is Valid` true))))
    (:`else`)))

(fn `Trace Box - Rotate according to the surface normal`
  (returns (`Return Value` :type Boolean))
  (return false))