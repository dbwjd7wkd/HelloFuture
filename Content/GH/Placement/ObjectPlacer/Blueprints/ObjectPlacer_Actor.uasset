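; Base placeable object (furniture) actor that switches between preview and placed modes by toggling box collision and calling empty implementation hooks, including blocked/unblocked preview states.
; It fits BoxBound to the combined bounds of MeshesRoot's children on construction and after Ground-type yaw rotation.
; A Tick-timed double-click on the mesh calls DestroyFurniture, which is empty here.
; A separate custom event destroys the actor under the cursor.
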(event `self.ReceiveTick`
  (params (DeltaSeconds :type "Float (single-precision)"))
  ;[1 1 1] 더블클릭이 들어오는지 확인
  (if (>= (`self.clickedNum`) 1)
    (set `self.currentTime` (+ DeltaSeconds (`self.currentTime`)))
    (if (and (> (`self.currentTime`) 0.5) (>= (`self.clickedNum`) 1))
      (set `self.clickedNum` 0)
      (set `self.currentTime` 0.0))))

(event `self.ReceiveBeginPlay`
  (if (`self.Placed Mode On BeginPlay`)
    (`self.Placed Mode`)
    (else
      (`self.Preview Mode`))))

(event `self.StaticMesh.OnClicked`
  (params (TouchedComponent :type "PrimitiveComponent Object Reference") (ButtonPressed :type "Key Structure"))
  ;[1 1 1] 더블클릭이 들어오는지 확인
  (set `self.currentTime` 0.0)
  (set `self.clickedNum` (+ (`self.clickedNum`) 1))
  (if (>= (`self.clickedNum`) 2)
    (`self.DestroyFurniture`)))

(event `CustomEvent_1`
  ;[1 1 1] 더블클릭시 삭제
  (`self.K2_DestroyActor` (`.HitActor` (`GameplayStatics.BreakHitResult` (`PlayerController.GetHitResultUnderCursorByChannel` (`GameplayStatics.GetPlayerController` 0) "TraceTypeQuery1" true))))
  (set `self.clickedNum` 0))

(event `Preview Mode Implementation`)

(event `Preview Mode Blocked Implementation`)

(event `Placed Mode Implementation`)

(event `Preview Mode Unblocked Implementation`)

(fn `DestroyFurniture`)

(fn `Get Box Bound`
  (returns (Origin :type "Vector Structure") (Size :type "Vector Structure"))
  (return (`self.Origin`) (`self.Size`)))

(fn `Get Box Bound Vector`
  (returns (`Min Vector` :type "Vector Structure") (`Max Vector` :type "Vector Structure"))
  (return (`self.Min Vector`) (`self.Max Vector`)))

(fn `Lerp (Vector) +`
  (params (A :type "Vector Structure") (B :type "Vector Structure") (Alpha :type "Vector Structure"))
  (returns (ReturnValue :type "Vector Structure"))
  (return (`KismetMathLibrary.MakeVector` (`KismetMathLibrary.Lerp` (.x A) (.x B) (.x Alpha)) (`KismetMathLibrary.Lerp` (.y A) (.y B) (.y Alpha)) (`KismetMathLibrary.Lerp` (.z A) (.z B) (.z Alpha)))))

(fn `Placed Mode`
  (`|ExecutionSequence`
    (:`then_0`
      (`PrimitiveComponent.SetCollisionEnabled` (`self.BoxBound`) "QueryAndPhysics"))
    (:`then_2`
      (`self.Placed Mode Implementation`))))

(fn `Preview Blocked`
  (`self.Preview Mode Blocked Implementation`))

(fn `Preview Mode`
  (`|ExecutionSequence`
    (:`then_0`
      (`PrimitiveComponent.SetCollisionEnabled` (`self.BoxBound`) "NoCollision"))
    (:`then_1`
      (`self.Preview Mode Implementation`))))

(fn `Preview Unblocked`
  (`self.Preview Mode Unblocked Implementation`))

(fn `Rotate Z`
  (params (`Yaw Rotation Offset` :type "Float (double-precision)"))
  (switch `/Game/GH/Placement/ObjectPlacer/Blueprints/EObjectPlacementType` (`self.Object Placement Type`)
    (:`NewEnumerator0`
      (`SceneComponent.K2_AddRelativeRotation` (`self.MeshesRoot`) (`KismetMathLibrary.MakeRotator` 0.0 0.0 `Yaw Rotation Offset`) false false)
      (`|ExecutionSequence`
        (:`then_0`
          (`self.Update Virtual Box Bound`))
        (:`then_1`
          (`self.Update Box Bound`))))))

(fn `Update Box Bound`
  (`BoxComponent.SetBoxExtent` (`self.BoxBound`) (`self.Size`) true)
  (`SceneComponent.K2_SetRelativeLocation` (`self.BoxBound`) (`self.Origin`) false false))

(fn `Update Virtual Box Bound`
  (`|ExecutionSequence`
    (:`then_0`
      (set `self.Min Vector` (0.0 0.0 0.0))
      (set `self.Max Vector` (0.0 0.0 0.0)))
    (:`then_1`
      (for _array_element (`SceneComponent.GetChildrenComponents` (`self.MeshesRoot`) true)
        (bind _asprimitive_component (cast `PrimitiveComponent` _array_element))
        (`|ExecutionSequence`
          (:`then_0`
            (bind (_origin _boxextent) (`KismetSystemLibrary.GetComponentBounds` _asprimitive_component))
            (bind _returnvalue (/ (`KismetMathLibrary.InverseTransformLocation` (`SceneComponent.K2_GetComponentToWorld` (`self.RootComponent`)) _origin) _boxextent))
            (set `self.Max Vector` (`KismetMathLibrary.Vector_ComponentMax` (`self.Max Vector`) (* _boxextent (`self.Lerp (Vector) +` (1.0 1.0 1.0) (2.0 2.0 2.0) _returnvalue)))))
          (:`then_1`
            (set `self.Min Vector` (`KismetMathLibrary.Vector_ComponentMin` (`self.Min Vector`) (* _boxextent (`self.Lerp (Vector) +` (1.0 1.0 1.0) (0.0 0.0 0.0) _returnvalue) (-1.0 -1.0 -1.0))))))))
    (:`then_2`
      (set `self.Size` (/ (- (`self.Max Vector`) (`self.Min Vector`)) 2.0))
      (set `self.Origin` (/ (+ (`self.Max Vector`) (`self.Min Vector`)) 2.0)))))

(fn `UserConstructionScript`
  (`|ExecutionSequence`
    (:`then_0`
      (`|ExecutionSequence`
        (:`then_0`
          (`self.Update Virtual Box Bound`))
        (:`then_1`
          (`self.Update Box Bound`))))
    (:`then_1`
      (if (`self.Placed Mode On BeginPlay`)
        (`self.Placed Mode`)
        (else
          (`self.Preview Mode`))))))