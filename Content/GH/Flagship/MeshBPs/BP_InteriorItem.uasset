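; BP_InteriorItem is an interior furniture actor that the player deletes by double-clicking it.
; Clicks on its StaticMesh increment a counter and restart a timer, which Tick uses to clear the count after half a second.
; A second click within that window runs DestroyFurniture, which destroys whatever actor a Visibility trace finds under player 0's cursor, rather than explicitly destroying itself.
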(event `self.ReceiveTick`
  (params (DeltaSeconds :type "Float (single-precision)"))
  ;[1 1 1] 더블클릭이 들어오는지 확인
  (if (>= (`self.clickedNum`) 1)
    (set `self.currentTime` (+ DeltaSeconds (`self.currentTime`)))
    (if (and (> (`self.currentTime`) 0.5) (>= (`self.clickedNum`) 1))
      (set `self.clickedNum` 0)
      (set `self.currentTime` 0.0))))

(event `self.StaticMesh.OnClicked`
  (params (TouchedComponent :type "PrimitiveComponent Object Reference") (ButtonPressed :type "Key Structure"))
  ;[1 1 1] 더블클릭이 들어오는지 확인
  (set `self.currentTime` 0.0)
  (set `self.clickedNum` (+ (`self.clickedNum`) 1))
  (if (>= (`self.clickedNum`) 2)
    (`self.DestroyFurniture`)))

(event `DestroyFurniture`
  ;[1 1 1] 더블클릭시 삭제
  (`self.K2_DestroyActor` (`.HitActor` (`GameplayStatics.BreakHitResult` (`PlayerController.GetHitResultUnderCursorByChannel` (`GameplayStatics.GetPlayerController` 0) "TraceTypeQuery1" true))))
  (set `self.clickedNum` 0))

(fn `UserConstructionScript`)