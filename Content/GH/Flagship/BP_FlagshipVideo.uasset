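; BP_FlagshipVideo is a trigger actor that shows a Hall_Video widget while a HelloFutureCharacter stands inside its Box.
; On overlap it creates the widget, adds it to the viewport, also assigns it to the URLHall widget component and focuses it with game-and-UI input.
; On exit it removes the widget from its parent and restores game-only input.
; Browser URL clearing and mouse-cursor nodes are present but never run.
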(event `self.Box.OnComponentBeginOverlap`
  (params (OverlappedComponent :type "PrimitiveComponent Object Reference") (OtherActor :type "Actor Object Reference") (OtherComp :type "PrimitiveComponent Object Reference") (OtherBodyIndex :type Integer) (bFromSweep :type Boolean) (SweepResult :type "HitResult Structure (by ref)"))
  (cast `HelloFutureCharacter` OtherActor)
  (bind _returnvalue (`|CreateWidget` "/Game/Minsu/Hall/Hall_Video.Hall_Video_C"))
  (`UserWidget.AddToViewport` _returnvalue 0)
  (`WidgetComponent.SetWidget` (`self.URLHall`) _returnvalue)
  (`WidgetBlueprintLibrary.SetInputMode_GameAndUIEx` (`GameplayStatics.GetPlayerController` 0) _returnvalue))

(event `self.Box.OnComponentEndOverlap`
  (params (OverlappedComponent :type "PrimitiveComponent Object Reference") (OtherActor :type "Actor Object Reference") (OtherComp :type "PrimitiveComponent Object Reference") (OtherBodyIndex :type Integer))
  (cast `HelloFutureCharacter` OtherActor)
  (`Widget.RemoveFromParent` (stale `self.Box.OnComponentBeginOverlap` _returnvalue))
  (`WidgetBlueprintLibrary.SetInputMode_GameOnly` (`GameplayStatics.GetPlayerController` 0)))

(fn `UserConstructionScript`)