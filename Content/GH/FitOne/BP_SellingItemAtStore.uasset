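; Store display actor for a clothing item for sale, highlighted with an outline while the cursor is over its box.
; BeginPlay copies the item's skeletal mesh to a hidden outline component using the Clicked_M_Inst material.
; Overlap events set the arrow mesh's spin rate and apply one yaw step each.
; Click handling is empty; the buy/already-bought widget logic is disconnected, and the BeginPlay ownership check has no effect.
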(event `self.ReceiveBeginPlay`
  (bind _outlineskeletal (`self.outlineSkeletal`))
  (`|ExecutionSequence`
    (:`then_0`
      (bind _asyj_hello_future_character (cast `/Game/Map/YJ_HelloFutureCharacter` (`GameplayStatics.GetPlayerCharacter` 0)))
      (bind _returnvalue (`HelloFutureCharacter.GetBoughtClothes` _asyj_hello_future_character (`self.name`)))
      (if _returnvalue
        _))
    (:`then_1`
      (`SkinnedMeshComponent.SetSkinnedAssetAndUpdate` _outlineskeletal (`SkinnedMeshComponent.SkeletalMesh` (`self.SellingItem`)) true)
      (for (_ _array_index) (`MeshComponent.GetMaterials` _outlineskeletal)
        (`PrimitiveComponent.SetMaterial` (`self.outlineSkeletal`) _array_index "/Game/GH/FitOne/Clicked_M_Inst.Clicked_M_Inst")
        (`SceneComponent.SetVisibility` (`self.outlineSkeletal`) false false)))))

(event `self.Box.OnClicked`
  (params (TouchedComponent :type "PrimitiveComponent Object Reference") (ButtonPressed :type "Key Structure")))

(event `SetInvisibleDia`
  (`SceneComponent.SetVisibility` (`self.StaticMesh`) false false))

(event `self.StaticMesh.OnComponentBeginOverlap`
  (params (OverlappedComponent :type "PrimitiveComponent Object Reference") (OtherActor :type "Actor Object Reference") (OtherComp :type "PrimitiveComponent Object Reference") (OtherBodyIndex :type Integer) (bFromSweep :type Boolean) (SweepResult :type "HitResult Structure (by ref)"))
  ;[1 1 1] 화살표 모션
  (bind _output_get (set `self.rotatePerSec` 45.0 :!label _label))
  (`SceneComponent.K2_AddLocalRotation` (`self.StaticMesh`) (`KismetMathLibrary.MakeRotator` 0.0 0.0 (* (`GameplayStatics.GetWorldDeltaSeconds`) _output_get)) false false))

(event `self.Box.OnComponentBeginOverlap`
  (params (OverlappedComponent :type "PrimitiveComponent Object Reference") (OtherActor :type "Actor Object Reference") (OtherComp :type "PrimitiveComponent Object Reference") (OtherBodyIndex :type Integer) (bFromSweep :type Boolean) (SweepResult :type "HitResult Structure (by ref)"))
  ;[1 1 1] 화살표 모션
  (goto _label))

(event `self.Box.OnComponentEndOverlap`
  (params (OverlappedComponent :type "PrimitiveComponent Object Reference") (OtherActor :type "Actor Object Reference") (OtherComp :type "PrimitiveComponent Object Reference") (OtherBodyIndex :type Integer))
  ;[1 1 1] 화살표 모션
  (bind _output_get (set `self.rotatePerSec` 0.0 :!label _label_2))
  (`SceneComponent.K2_AddLocalRotation` (`self.StaticMesh`) (`KismetMathLibrary.MakeRotator` 0.0 0.0 (* (`GameplayStatics.GetWorldDeltaSeconds`) _output_get)) false false))

(event `self.StaticMesh.OnComponentEndOverlap`
  (params (OverlappedComponent :type "PrimitiveComponent Object Reference") (OtherActor :type "Actor Object Reference") (OtherComp :type "PrimitiveComponent Object Reference") (OtherBodyIndex :type Integer))
  ;[1 1 1] 화살표 모션
  (goto _label_2))

(event `self.Box.OnBeginCursorOver`
  (params (TouchedComponent :type "PrimitiveComponent Object Reference"))
  (`SceneComponent.SetVisibility` (`self.outlineSkeletal`) true false))

(event `self.Box.OnEndCursorOver`
  (params (TouchedComponent :type "PrimitiveComponent Object Reference"))
  (`SceneComponent.SetVisibility` (`self.outlineSkeletal`) false false))

(event `CreateOutline`)

(event `deleteOutline`)

(fn `UserConstructionScript`)