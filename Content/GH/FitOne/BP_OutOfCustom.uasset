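; BP_OutOfCustom is an exit trigger that sends the player back to the level stored in the character's PreLevelName.
; Overlapping or clicking its Box caches that name and clears it on the HelloFutureCharacter.
; Only the overlap path calls SaveGame; both paths then share a five-second delay before opening the cached level by name.
; Debug strings print on overlap and cursor hover.
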(event `self.Box.OnComponentBeginOverlap`
  (params (OverlappedComponent :type "PrimitiveComponent Object Reference") (OtherActor :type "Actor Object Reference") (OtherComp :type "PrimitiveComponent Object Reference") (OtherBodyIndex :type Integer) (bFromSweep :type Boolean) (SweepResult :type "HitResult Structure (by ref)"))
  (bind _ashello_future_character (cast `HelloFutureCharacter` OtherActor))
  (bind _output_get (set `self.SavedPreLevelName` (`HelloFutureCharacter.preLevelName` _ashello_future_character)))
  (`KismetSystemLibrary.PrintString` _output_get)
  (bind _output_get_2 (set `HelloFutureCharacter.preLevelName` "" _ashello_future_character))
  (`KismetSystemLibrary.PrintString` _output_get_2)
  (`HelloFutureCharacter.SaveGame` _ashello_future_character)
  (`KismetSystemLibrary.Delay` 5.0 :!label _label)
  (`GameplayStatics.OpenLevel` (`KismetStringLibrary.Conv_StringToName` (`self.SavedPreLevelName`))))

(event `self.Box.OnClicked`
  (params (TouchedComponent :type "PrimitiveComponent Object Reference") (ButtonPressed :type "Key Structure"))
  (bind _ashello_future_character (cast `HelloFutureCharacter` (`GameplayStatics.GetPlayerCharacter` 0)))
  (set `self.SavedPreLevelName` (`HelloFutureCharacter.preLevelName` _ashello_future_character))
  (set `HelloFutureCharacter.preLevelName` "" _ashello_future_character)
  (goto _label))

(event `self.Box.OnBeginCursorOver`
  (params (TouchedComponent :type "PrimitiveComponent Object Reference"))
  (`KismetSystemLibrary.PrintString` "Hello"))

(fn `UserConstructionScript`)