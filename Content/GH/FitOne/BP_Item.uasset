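; Clickable item Blueprint that applies its own skeletal mesh and materials to a FitCategory slot through the FitOneController.
; BeginPlay caches the controller and flags whether the mesh has multiple materials.
; Clicking the Box sends category, mesh, materials and object name to the controller's single- or multi-material change function.
; Toggle-off and double-click removal logic remains in the graph but is disconnected.
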(event `self.ReceiveBeginPlay`
  (bind _asfit_one_controller (cast `/Game/GH/FitOne/FitOneController` (`GameplayStatics.GetPlayerController` 0)))
  (set `self.FitOneController` _asfit_one_controller)
  ;[1 1 1] 클릭한 아이템이 여러개의 머터리얼인지 확인
  (if (> (`KismetArrayLibrary.Array_Length` (`MeshComponent.GetMaterials` (`self.SkeletalMesh`))) 1)
    (set `self.isMulti` true)))

(event `self.Box.OnBeginCursorOver`
  (params (TouchedComponent :type "PrimitiveComponent Object Reference")))

(event `self.Box.OnClicked`
  (params (TouchedComponent :type "PrimitiveComponent Object Reference") (ButtonPressed :type "Key Structure"))
  (bind _skeletalmesh (`self.SkeletalMesh`))
  (bind _fitcategory (`self.FitCategory`))
  (bind _fitonecontroller (`self.FitOneController`))
  (bind _returnvalue (`MeshComponent.GetMaterials` _skeletalmesh))
  (bind _returnvalue_2 (`KismetSystemLibrary.GetObjectName` self))
  (bind _skeletalmesh_2 (`SkinnedMeshComponent.SkeletalMesh` _skeletalmesh))
  (`GameplayStatics.GetActorOfClass` "/Game/GH/FitOne/BP_PrettyBoneActor.BP_PrettyBoneActor_C")
  (if (`self.isMulti`)
    (`/Game/GH/FitOne/FitOneController.CTR_FitOneChangeMultiMat` _fitonecontroller _fitcategory _returnvalue _skeletalmesh_2 false _returnvalue_2)
    (else
      (`/Game/GH/FitOne/FitOneController.CTR_FitOne_Change` _fitonecontroller _fitcategory (`|GetArrayItem` _returnvalue) _skeletalmesh_2 true _returnvalue_2))))

(fn `UserConstructionScript`)