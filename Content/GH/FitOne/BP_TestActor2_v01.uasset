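; Modular character test actor for fitting body parts, clothing and accessories as separate skeletal mesh components.
; The construction script makes the head the master pose component for all other parts, so they share its pose.
; ChangeFitMeshAndMat switches on category but handles only Nose, calling mesh and material setters with no values connected, leaving the event's mesh and material inputs unused.
; An unreachable default-set chain holds a preset nose mesh and material.
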(event `ChangeFitMeshAndMat`
  (params (ChangeCategory :type "/Game/GH/FitOne/EFitCategory Enum" :default "NewEnumerator0") (ChageMaterial :type "MaterialInterface Object Reference") (ChangeMesh :type "SkeletalMesh Object Reference") (state :type Boolean))
  (bind _actor_nose (`self.actor_nose`))
  (switch `/Game/GH/FitOne/EFitCategory` ChangeCategory
    (:`NewEnumerator3`
      (`SkinnedMeshComponent.SetSkinnedAssetAndUpdate` _actor_nose null true)
      (`PrimitiveComponent.SetMaterial` _actor_nose 0 null))))

(fn `UserConstructionScript`
  (`SkinnedMeshComponent.SetLeaderPoseComponent` (`self.actor_hand`) (`self.actor_head`) false)
  (`SkinnedMeshComponent.SetLeaderPoseComponent` (`self.actor_under`) (`self.actor_head`) false)
  (`SkinnedMeshComponent.SetLeaderPoseComponent` (`self.actor_nose`) (`self.actor_head`) false)
  (`SkinnedMeshComponent.SetLeaderPoseComponent` (`self.actor_hair`) (`self.actor_head`) false)
  (`SkinnedMeshComponent.SetLeaderPoseComponent` (`self.actor_torso`) (`self.actor_head`) false)
  (`SkinnedMeshComponent.SetLeaderPoseComponent` (`self.actor_wholeclothes`) (`self.actor_head`) false)
  (`SkinnedMeshComponent.SetLeaderPoseComponent` (`self.actor_glasses`) (`self.actor_head`) false)
  (`SkinnedMeshComponent.SetLeaderPoseComponent` (`self.actor_hat`) (`self.actor_head`) false)
  (`SkinnedMeshComponent.SetLeaderPoseComponent` (`self.actor_bag`) (`self.actor_head`) false)
  (`SkinnedMeshComponent.SetLeaderPoseComponent` (`self.actor_watch`) (`self.actor_head`) false))