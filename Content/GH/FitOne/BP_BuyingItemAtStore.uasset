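; BP_BuyingItemAtStore is a clickable store actor representing a named, priced clothing item for purchase.
; Clicking its Box asks YJ_HelloFutureCharacter whether the item is already bought, then switches input to Game and UI.
; Owned items only create WBP_AlreadyBought without adding it to the viewport, while unowned items display WBP_BuyingClothes filled with name and price.
; Hovering the cursor over the Box prints the item name.
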(event `self.Box.OnClicked`
  (params (TouchedComponent :type "PrimitiveComponent Object Reference") (ButtonPressed :type "Key Structure"))
  (bind _asyj_hello_future_character (cast `/Game/Map/YJ_HelloFutureCharacter` (`GameplayStatics.GetPlayerCharacter` 0)))
  (bind _returnvalue (`HelloFutureCharacter.GetBoughtClothes` _asyj_hello_future_character (`self.name`)))
  (if _returnvalue
    (`WidgetBlueprintLibrary.SetInputMode_GameAndUIEx` (`GameplayStatics.GetPlayerController` 0) null)
    (`|CreateWidget` "/Game/GH/FitOne/WBP_AlreadyBought.WBP_AlreadyBought_C")
    (else
      (`WidgetBlueprintLibrary.SetInputMode_GameAndUIEx` (`GameplayStatics.GetPlayerController` 0) null)
      (bind _returnvalue_2 (`|CreateWidget` "/Game/GH/FitOne/WBP_BuyingClothes.WBP_BuyingClothes_C"))
      (bind _output_get (set `self.BuyingClothesUI` _returnvalue_2))
      (set `/Game/GH/FitOne/WBP_BuyingClothes.clotheName` (`self.name`) _output_get)
      (set `/Game/GH/FitOne/WBP_BuyingClothes.price` (`self.price`) _output_get)
      (`UserWidget.AddToViewport` _output_get 0))))

(event `self.Box.OnBeginCursorOver`
  (params (TouchedComponent :type "PrimitiveComponent Object Reference"))
  (`KismetSystemLibrary.PrintString` (`self.name`)))

(fn `UserConstructionScript`)