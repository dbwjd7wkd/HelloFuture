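; BP_PrettyBone is a modular character that swaps skeletal meshes and materials per fitting category, such as hair, clothes and accessories.
; ChangeFitMeshAndMat sets one material on slot 0, changing only the material for the head, while ChangeFitMeshAndMatMulti applies a material array by slot index.
; The construction script makes ActorHead the master pose for most parts, excluding upper and under clothes.
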(event `ChangeFitMeshAndMat`
  (params (ChangeCategory :type "/Game/GH/FitOne/EFitCategory Enum" :default "NewEnumerator0") (ChageMaterial :type "MaterialInterface Object Reference") (ChangeMesh :type "SkeletalMesh Object Reference") (state :type Boolean))
  (bind _actor_hair (`self.actor_hair`))
  (bind _actor_nose (`self.actor_nose`))
  (bind _actor_bag (`self.actor_bag`))
  (bind _actor_upperclothes (`self.actor_upperclothes`))
  (switch `/Game/GH/FitOne/EFitCategory` ChangeCategory
    (:`NewEnumerator1`
      (`PrimitiveComponent.SetMaterial` (`self.actor_head`) 0 ChageMaterial))
    (:`NewEnumerator2`
      (`SkinnedMeshComponent.SetSkinnedAssetAndUpdate` _actor_hair ChangeMesh true)
      (`PrimitiveComponent.SetMaterial` _actor_hair 0 ChageMaterial))
    (:`NewEnumerator3`
      (`SkinnedMeshComponent.SetSkinnedAssetAndUpdate` _actor_nose ChangeMesh true)
      (`PrimitiveComponent.SetMaterial` _actor_nose 0 ChageMaterial))
    (:`NewEnumerator11`
      (`SkinnedMeshComponent.SetSkinnedAssetAndUpdate` _actor_upperclothes ChangeMesh true)
      (`PrimitiveComponent.SetMaterial` _actor_upperclothes 0 ChageMaterial))
    (:`NewEnumerator9`
      (`SkinnedMeshComponent.SetSkinnedAssetAndUpdate` _actor_bag ChangeMesh true)
      (`PrimitiveComponent.SetMaterial` _actor_bag 0 ChageMaterial))))

(event `ChangeFitMeshAndMatMulti`
  (params (ChangeCategory :type "/Game/GH/FitOne/EFitCategory Enum" :default "NewEnumerator0") (ChageMaterial :type "Array of MaterialInterface Object Reference") (ChangeMesh :type "SkeletalMesh Object Reference") (state :type Boolean))
  (bind _actor_hair (`self.actor_hair`))
  (bind _actor_wholeclothes (`self.actor_wholeclothes`))
  (bind _actor_underclothes (`self.actor_underclothes`))
  (bind _actor_watch (`self.actor_watch`))
  (bind _actor_hat (`self.actor_hat`))
  (bind _actor_glasses (`self.actor_glasses`))
  (switch `/Game/GH/FitOne/EFitCategory` ChangeCategory
    (:`NewEnumerator2`
      (`SkinnedMeshComponent.SetSkinnedAssetAndUpdate` _actor_hair ChangeMesh true)
      (for (_array_element _array_index) ChageMaterial
        (`PrimitiveComponent.SetMaterial` _actor_hair _array_index _array_element)))
    (:`NewEnumerator12`
      (`SkinnedMeshComponent.SetSkinnedAssetAndUpdate` _actor_underclothes ChangeMesh true)
      (for (_array_element_2 _array_index_2) ChageMaterial
        (`PrimitiveComponent.SetMaterial` _actor_underclothes _array_index_2 _array_element_2)))
    (:`NewEnumerator13`
      (`SkinnedMeshComponent.SetSkinnedAssetAndUpdate` _actor_wholeclothes ChangeMesh true)
      (for (_array_element_3 _array_index_3) ChageMaterial
        (`PrimitiveComponent.SetMaterial` _actor_wholeclothes _array_index_3 _array_element_3)))
    (:`NewEnumerator6`
      (`SkinnedMeshComponent.SetSkinnedAssetAndUpdate` _actor_glasses ChangeMesh true)
      (for (_array_element_4 _array_index_4) ChageMaterial
        (`PrimitiveComponent.SetMaterial` _actor_glasses _array_index_4 _array_element_4)))
    (:`NewEnumerator7`
      (`SkinnedMeshComponent.SetSkinnedAssetAndUpdate` _actor_hat ChangeMesh true)
      (for (_array_element_5 _array_index_5) ChageMaterial
        (`PrimitiveComponent.SetMaterial` _actor_hat _array_index_5 _array_element_5)))
    (:`NewEnumerator8`
      (`SkinnedMeshComponent.SetSkinnedAssetAndUpdate` _actor_watch ChangeMesh true)
      (for (_array_element_6 _array_index_6) ChageMaterial
        (`PrimitiveComponent.SetMaterial` _actor_watch _array_index_6 _array_element_6)))))

(fn `UserConstructionScript`
  (`SkinnedMeshComponent.SetLeaderPoseComponent` (`self.actor_nose`) (`self.actor_head`) false)
  (`SkinnedMeshComponent.SetLeaderPoseComponent` (`self.actor_hair`) (`self.actor_head`) false)
  (`SkinnedMeshComponent.SetLeaderPoseComponent` (`self.actor_wholeclothes`) (`self.actor_head`) false)
  (`SkinnedMeshComponent.SetLeaderPoseComponent` (`self.actor_glasses`) (`self.actor_head`) false)
  (`SkinnedMeshComponent.SetLeaderPoseComponent` (`self.actor_hat`) (`self.actor_head`) false)
  (`SkinnedMeshComponent.SetLeaderPoseComponent` (`self.actor_bag`) (`self.actor_head`) false)
  (`SkinnedMeshComponent.SetLeaderPoseComponent` (`self.actor_watch`) (`self.actor_head`) false))