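; Modular dress-up character whose skeletal-mesh parts follow the body through master pose.
; Initialization applies InitialParts; change events swap meshes and single or multiple materials by category, resolving hat, hair, accessory and clothing conflicts.
; Initialization resets ABP_LastClicked and some multi-material changes record to it; MovetoAnotherLevel saves the outfit through the game instance.
; The Whole Clothes case only clears upper and under clothes, as its mesh-apply nodes are unconnected.
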(event `Initialize_CustomActor`
  (bind _actor_hair (`self.actor_hair`))
  (bind _actor_nose (`self.actor_nose`))
  (bind _actor_upperclothes (`self.actor_upperclothes`))
  (bind _actor_underclothes (`self.actor_underclothes`))
  (bind _actor_wholeclothes (`self.actor_wholeclothes`))
  (bind _actor_glasses (`self.actor_glasses`))
  (bind _actor_hat (`self.actor_hat`))
  (bind _actor_bag (`self.actor_bag`))
  (bind _actor_watch (`self.actor_watch`))
  (bind _actor_hathair (`self.actor_hathair`))
  (bind _actor_hair_acc2_rabbitband (`self.actor_hair_acc2_rabbitband`))
  (bind _actor_hair_acc1_ribborn (`self.actor_hair_acc1_ribborn`))
  (bind (_initbody _initfacem _inithairstyle _inithairstylem _initnose _initnosem _initupperclothes _inituppperclothesm _initunderclothes _initunderclothesm _initwholeclothes _initwholeclothesm _initglasses _initglassesm _inithat _inithatm _initbag _initbagm _initwatch _initwatchm _inithathair _inithairacc1 _inithairacc2 _inithathairm _inithairacc1m _inithairacc2m) (break `/Game/GH/FitOne/S_InitialParts` (`self.InitialParts`)))
  ;[1 1 1] 초기화
  (`|ExecutionSequence`
    (:`then_0`
      (`PrimitiveComponent.SetMaterial` (`self.actor_body`) 0 _initfacem)
      (bind _returnvalue (`GameplayStatics.GetActorOfClass` "/Game/GH/FitOne/ABP_LastClicked.ABP_LastClicked_C" :!label _label))
      (`GH_LastClickedTMap.InitLastClickedItem` _returnvalue))
    (:`then_1`
      (`SkinnedMeshComponent.SetSkinnedAssetAndUpdate` _actor_hair _inithairstyle true)
      (for (_array_element _array_index) _inithairstylem
        (`PrimitiveComponent.SetMaterial` _actor_hair _array_index _array_element)
        (goto _label)))
    (:`then_2`
      (`SkinnedMeshComponent.SetSkinnedAssetAndUpdate` _actor_nose _initnose true)
      (`PrimitiveComponent.SetMaterial` _actor_nose 0 _initnosem)
      (goto _label))
    (:`then_3`
      (`SkinnedMeshComponent.SetSkinnedAssetAndUpdate` _actor_upperclothes _initupperclothes true)
      (for (_array_element_2 _array_index_2) _inituppperclothesm
        (`PrimitiveComponent.SetMaterial` _actor_upperclothes _array_index_2 _array_element_2)
        (goto _label)))
    (:`then_4`
      (`SkinnedMeshComponent.SetSkinnedAssetAndUpdate` _actor_underclothes _initunderclothes true)
      (for (_array_element_3 _array_index_3) _initunderclothesm
        (`PrimitiveComponent.SetMaterial` _actor_underclothes _array_index_3 _array_element_3)
        (goto _label)))
    (:`then_5`
      (`SkinnedMeshComponent.SetSkinnedAssetAndUpdate` _actor_wholeclothes _initwholeclothes true)
      (for (_array_element_4 _array_index_4) _initwholeclothesm
        (`PrimitiveComponent.SetMaterial` _actor_wholeclothes _array_index_4 _array_element_4)
        (goto _label)))
    (:`then_6`
      (`SkinnedMeshComponent.SetSkinnedAssetAndUpdate` _actor_glasses _initglasses true)
      (for (_array_element_5 _array_index_5) _initglassesm
        (`PrimitiveComponent.SetMaterial` _actor_glasses _array_index_5 _array_element_5)
        (goto _label)))
    (:`then_7`
      (`SkinnedMeshComponent.SetSkinnedAssetAndUpdate` _actor_hat _inithat true)
      (for (_array_element_6 _array_index_6) _inithatm
        (`PrimitiveComponent.SetMaterial` _actor_hat _array_index_6 _array_element_6)
        (goto _label)))
    (:`then_8`
      (`SkinnedMeshComponent.SetSkinnedAssetAndUpdate` _actor_bag _initbag true)
      (for (_array_element_7 _array_index_7) _initbagm
        (`PrimitiveComponent.SetMaterial` _actor_bag _array_index_7 _array_element_7)
        (goto _label)))
    (:`then_9`
      (`SkinnedMeshComponent.SetSkinnedAssetAndUpdate` _actor_watch _initwatch true)
      (for (_array_element_8 _array_index_8) _initwatchm
        (`PrimitiveComponent.SetMaterial` _actor_watch _array_index_8 _array_element_8)
        (goto _label)))
    (:`then_10`
      (`SkinnedMeshComponent.SetSkinnedAssetAndUpdate` _actor_hathair _inithathair true)
      (for (_array_element_9 _array_index_9) _inithathairm
        (`PrimitiveComponent.SetMaterial` _actor_hathair _array_index_9 _array_element_9)))
    (:`then_11`
      (`SkinnedMeshComponent.SetSkinnedAssetAndUpdate` _actor_hair_acc1_ribborn _inithairacc1 true)
      (for (_array_element_10 _array_index_10) _inithairacc1m
        (`PrimitiveComponent.SetMaterial` _actor_hair_acc1_ribborn _array_index_10 _array_element_10)))
    (:`then_12`
      (`SkinnedMeshComponent.SetSkinnedAssetAndUpdate` _actor_hair_acc2_rabbitband _inithairacc2 true)
      (for (_array_element_11 _array_index_11) _inithairacc2m
        (`PrimitiveComponent.SetMaterial` _actor_hair_acc2_rabbitband _array_index_11 _array_element_11)))))

(event `ChangeFitMeshAndMat`
  (params (ChangeCategory :type "/Game/GH/FitOne/EFitCategory Enum" :default "NewEnumerator0") (ChageMaterial :type "MaterialInterface Object Reference") (ChangeMesh :type "SkeletalMesh Object Reference") (state :type Boolean) (clickedName :type String))
  (bind _actor_nose (`self.actor_nose`))
  (bind _actor_underclothes (`self.actor_underclothes`))
  (bind _actor_bag (`self.actor_bag`))
  (bind _actor_upperclothes (`self.actor_upperclothes`))
  (bind _actor_hair (`self.actor_hair`))
  ;[1 1 1] Single Material
  (set `self.Change Category` ChangeCategory)
  (set `self.Chage Material` ChageMaterial)
  (set `self.Change Mesh` ChangeMesh)
  (switch `/Game/GH/FitOne/EFitCategory` (`self.Change Category`)
    (:`NewEnumerator1`
      (`PrimitiveComponent.SetMaterial` (`self.actor_body`) 0 (`self.Chage Material`)))
    (:`NewEnumerator2`
      (bind _output_get (set `self.hasHat` (> (`KismetArrayLibrary.Array_Length` (`MeshComponent.GetMaterials` (`self.actor_hat`))) 0)))
      (if _output_get
        (bind _output_get_2 (set `self.isBald` (< (`KismetArrayLibrary.Array_Length` (`MeshComponent.GetMaterials` (`self.actor_hathair`))) 1)))
        (if _output_get_2
          (`SkinnedMeshComponent.SetSkinnedAssetAndUpdate` (`self.actor_hathair`) "/Game/GH/Assets/RealMeshs/OtherswthDiffBone/mc_trimhair_03.mc_trimhair_03" true)
          (`PrimitiveComponent.SetMaterial` (`self.actor_hathair`) 0 (`self.Chage Material`))
          (else
            (`PrimitiveComponent.SetMaterial` (`self.actor_hathair`) 0 (`self.Chage Material`))))
        (else
          (`SkinnedMeshComponent.SetSkinnedAssetAndUpdate` _actor_hair (`self.Change Mesh`) true)
          (`PrimitiveComponent.SetMaterial` _actor_hair 0 (`self.Chage Material`)))))
    (:`NewEnumerator3`
      (`SkinnedMeshComponent.SetSkinnedAssetAndUpdate` _actor_nose (`self.Change Mesh`) true)
      (`PrimitiveComponent.SetMaterial` _actor_nose 0 (`self.Chage Material`)))
    (:`NewEnumerator11`
      (`SkinnedMeshComponent.SetSkinnedAssetAndUpdate` (`self.actor_wholeclothes`) null true)
      (`SkinnedMeshComponent.SetSkinnedAssetAndUpdate` _actor_upperclothes (`self.Change Mesh`) true)
      (`PrimitiveComponent.SetMaterial` _actor_upperclothes 0 (`self.Chage Material`)))
    (:`NewEnumerator12`
      (`SkinnedMeshComponent.SetSkinnedAssetAndUpdate` (`self.actor_wholeclothes`) null true)
      (`SkinnedMeshComponent.SetSkinnedAssetAndUpdate` _actor_underclothes (`self.Change Mesh`) true)
      (`PrimitiveComponent.SetMaterial` _actor_underclothes 0 (`self.Chage Material`)))
    (:`NewEnumerator9`
      (`KismetSystemLibrary.PrintString` (`KismetSystemLibrary.GetObjectName` ChageMaterial))
      (`SkinnedMeshComponent.SetSkinnedAssetAndUpdate` _actor_bag (`self.Change Mesh`) true)
      (`KismetSystemLibrary.PrintString` (`KismetSystemLibrary.GetObjectName` ChangeMesh))
      (`PrimitiveComponent.SetMaterial` _actor_bag 0 (`self.Chage Material`)))
    (:`NewEnumerator15`
      (bind _output_get_3 (set `self.hasHat` (> (`KismetArrayLibrary.Array_Length` (`MeshComponent.GetMaterials` (`self.actor_hat`))) 0)))
      (if _output_get_3
        (`SkinnedMeshComponent.SetSkinnedAssetAndUpdate` (`self.actor_hat`) null true))
      (`SkinnedMeshComponent.SetSkinnedAssetAndUpdate` (`self.actor_hair_acc2_rabbitband`) (`self.Change Mesh`) true)
      (`PrimitiveComponent.SetMaterial` (`self.actor_hair_acc2_rabbitband`) 0 (`self.Chage Material`)))))

(event `ChangeFitMeshAndMatMulti`
  (params (ChangeCategory :type "/Game/GH/FitOne/EFitCategory Enum" :default "NewEnumerator0") (ChageMaterial :type "Array of MaterialInterface Object Reference") (ChangeMesh :type "SkeletalMesh Object Reference") (state :type Boolean) (clickedName :type String))
  (bind _actor_wholeclothes (`self.actor_wholeclothes`))
  (bind _actor_watch (`self.actor_watch`))
  (bind _actor_hair (`self.actor_hair`))
  (bind _returnvalue (`MeshComponent.GetMaterials` (`self.actor_hair`)))
  ;[1 1 1] Multi Materials
  (set `self.Change Category` ChangeCategory)
  (bind _output_get (set `self.Chage Materials` ChageMaterial))
  (set `self.Chage Material` (`|GetArrayItem` _output_get 1))
  (set `self.Change Mesh` ChangeMesh)
  (switch `/Game/GH/FitOne/EFitCategory` (`self.Change Category`)
    (:`NewEnumerator2`
      (bind _output_get_2 (set `self.hasHat` (> (`KismetArrayLibrary.Array_Length` (`MeshComponent.GetMaterials` (`self.actor_hat`))) 0)))
      (if _output_get_2
        (set `self.isBald` (< (`KismetArrayLibrary.Array_Length` (`MeshComponent.GetMaterials` (`self.actor_hathair`))) 1))
        (if true
          (`SkinnedMeshComponent.SetSkinnedAssetAndUpdate` (`self.actor_hathair`) "/Game/GH/Assets/RealMeshs/OtherswthDiffBone/mc_trimhair_03.mc_trimhair_03" true)
          (`PrimitiveComponent.SetMaterial` (`self.actor_hathair`) 0 (`self.Chage Material`))
          (else
            (`PrimitiveComponent.SetMaterial` (`self.actor_hathair`) 0 (`self.Chage Material`))))
        (else
          (`SkinnedMeshComponent.SetSkinnedAssetAndUpdate` _actor_hair (`self.Change Mesh`) true)
          (for (_array_element _array_index) (`self.Chage Materials`)
            (`PrimitiveComponent.SetMaterial` _actor_hair _array_index _array_element)
            (bind _returnvalue_2 (`GameplayStatics.GetActorOfClass` "/Game/GH/FitOne/ABP_LastClicked.ABP_LastClicked_C" :!label _label_2))
            (`GH_LastClickedTMap.SetLastClickedItem` _returnvalue_2 (`|GetEnumeratorNameAsString` (`self.Change Category`)) clickedName)))))
    (:`NewEnumerator11`
      (`SkinnedMeshComponent.SetSkinnedAssetAndUpdate` _actor_wholeclothes null true)
      (`SkinnedMeshComponent.SetSkinnedAssetAndUpdate` (`self.actor_upperclothes`) (`self.Change Mesh`) true)
      (for (_array_element_2 _array_index_2) (`self.Chage Materials`)
        (`PrimitiveComponent.SetMaterial` (`self.actor_upperclothes`) _array_index_2 _array_element_2)
        (goto _label_2)))
    (:`NewEnumerator12`
      (`SkinnedMeshComponent.SetSkinnedAssetAndUpdate` _actor_wholeclothes null true)
      (`SkinnedMeshComponent.SetSkinnedAssetAndUpdate` (`self.actor_underclothes`) (`self.Change Mesh`) true)
      (for (_array_element_3 _array_index_3) (`self.Chage Materials`)
        (`PrimitiveComponent.SetMaterial` (`self.actor_underclothes`) _array_index_3 _array_element_3)
        (goto _label_2)))
    (:`NewEnumerator13`
      (`SkinnedMeshComponent.SetSkinnedAssetAndUpdate` (`self.actor_upperclothes`) null true)
      (`SkinnedMeshComponent.SetSkinnedAssetAndUpdate` (`self.actor_underclothes`) null true))
    (:`NewEnumerator6`
      (`SkinnedMeshComponent.SetSkinnedAssetAndUpdate` (`self.actor_glasses`) (`self.Change Mesh`) true)
      (for (_array_element_4 _array_index_4) (`self.Chage Materials`)
        (`PrimitiveComponent.SetMaterial` (`self.actor_glasses`) _array_index_4 _array_element_4)
        (goto _label_2)))
    (:`NewEnumerator7`
      (`SkinnedMeshComponent.SetSkinnedAssetAndUpdate` (`self.actor_hair_acc1_ribborn`) null true)
      (`SkinnedMeshComponent.SetSkinnedAssetAndUpdate` (`self.actor_hair_acc2_rabbitband`) null true)
      (if (> (`KismetArrayLibrary.Array_Length` _returnvalue) 0)
        (set `self.isBald` false)
        (set `self.hairColor` (`|GetArrayItem` _returnvalue (`KismetArrayLibrary.Array_LastIndex` _returnvalue)))
        (`SkinnedMeshComponent.SetSkinnedAssetAndUpdate` (`self.actor_hair`) null true)
        (else
          (set `self.isBald` true)))
      (`SkinnedMeshComponent.SetSkinnedAssetAndUpdate` (`self.actor_hat`) (`self.Change Mesh`) true)
      (for (_array_element_5 _array_index_5) (`self.Chage Materials`)
        (`PrimitiveComponent.SetMaterial` (`self.actor_hat`) _array_index_5 _array_element_5)
        (if (not (`self.isBald`))
          (`SkinnedMeshComponent.SetSkinnedAssetAndUpdate` (`self.actor_hathair`) "/Game/GH/Assets/RealMeshs/OtherswthDiffBone/mc_trimhair_03.mc_trimhair_03" true)
          (`PrimitiveComponent.SetMaterial` (`self.actor_hathair`) 0 (`self.hairColor`)))))
    (:`NewEnumerator8`
      (`SkinnedMeshComponent.SetSkinnedAssetAndUpdate` _actor_watch (`self.Change Mesh`) true)
      (for (_array_element_6 _array_index_6) (`self.Chage Materials`)
        (`PrimitiveComponent.SetMaterial` _actor_watch _array_index_6 _array_element_6)
        (goto _label_2)))
    (:`NewEnumerator16`
      (bind _output_get_3 (set `self.hasHat` (> (`KismetArrayLibrary.Array_Length` (`MeshComponent.GetMaterials` (`self.actor_hat`))) 0)))
      (if _output_get_3
        (`SkinnedMeshComponent.SetSkinnedAssetAndUpdate` (`self.actor_hat`) null true))
      (`SkinnedMeshComponent.SetSkinnedAssetAndUpdate` (`self.actor_hair_acc1_ribborn`) (`self.Change Mesh`) true)
      (for (_array_element_7 _array_index_7) (`self.Chage Materials`)
        (`PrimitiveComponent.SetMaterial` (`self.actor_hair_acc1_ribborn`) _array_index_7 _array_element_7)))))

(event `Move toAnotherLevel`
  (bind _selectedparts (`self.Get Customed Data`))
  (bind _asreal_char_game_instance (cast `/Game/Map/realCharGameInstance` (`GameplayStatics.GetGameInstance`)))
  (`/Game/Map/realCharGameInstance.SaveCustomParts` _asreal_char_game_instance _selectedparts))

(fn `Get Customed Data`
  (returns (SelectedParts :type "/Game/GH/FitOne/S_FitSavedGameParts Structure"))
  (bind _actor_hair (`self.actor_hair`))
  (bind _actor_glasses (`self.actor_glasses`))
  (bind _actor_bag (`self.actor_bag`))
  (bind _actor_watch (`self.actor_watch`))
  (bind _actor_hair_acc1_ribborn (`self.actor_hair_acc1_ribborn`))
  (bind _actor_hair_acc2_rabbitband (`self.actor_hair_acc2_rabbitband`))
  (bind _actor_upperclothes (`self.actor_upperclothes`))
  (bind _actor_underclothes (`self.actor_underclothes`))
  (bind _actor_wholeclothes (`self.actor_wholeclothes`))
  (bind _actor_hat (`self.actor_hat`))
  (bind _actor_hathair (`self.actor_hathair`))
  (setmembers `/Game/GH/FitOne/S_FitSavedGameParts` :`StructRef` (`self.fitParts`) :`FaceM` (`PrimitiveComponent.GetMaterial` (`self.actor_body`) 0) :`FitHair` (`SkinnedMeshComponent.SkeletalMesh` _actor_hair) :`HairM` (`MeshComponent.GetMaterials` _actor_hair) :`FitNose` (`SkinnedMeshComponent.SkeletalMesh` (`self.actor_nose`)) :`FitUpperClothes` (`SkinnedMeshComponent.SkeletalMesh` _actor_upperclothes) :`UppperClothesM` (`MeshComponent.GetMaterials` _actor_upperclothes) :`FitUnderClothes` (`SkinnedMeshComponent.SkeletalMesh` _actor_underclothes) :`UnderClothesM` (`MeshComponent.GetMaterials` _actor_underclothes) :`FitWholeClothes` (`SkinnedMeshComponent.SkeletalMesh` _actor_wholeclothes) :`WholeClothesM` (`MeshComponent.GetMaterials` _actor_wholeclothes) :`FitHat` (`SkinnedMeshComponent.SkeletalMesh` _actor_hat) :`FitHatM` (`MeshComponent.GetMaterials` _actor_hat) :`HatHair` (`SkinnedMeshComponent.SkeletalMesh` _actor_hathair) :`HatHairM` (`PrimitiveComponent.GetMaterial` _actor_hathair 0) :`FitGlasses` (`SkinnedMeshComponent.SkeletalMesh` _actor_glasses) :`FitGlassesM` (`MeshComponent.GetMaterials` _actor_glasses) :`FitBag` (`SkinnedMeshComponent.SkeletalMesh` _actor_bag) :`FitBagM` (`PrimitiveComponent.GetMaterial` _actor_bag 0) :`FitWatch` (`SkinnedMeshComponent.SkeletalMesh` _actor_watch) :`FitWatchM` (`MeshComponent.GetMaterials` _actor_watch) :`HairAcc1` (`SkinnedMeshComponent.SkeletalMesh` _actor_hair_acc1_ribborn) :`HairAcc1M` (`MeshComponent.GetMaterials` _actor_hair_acc1_ribborn) :`HairAcc2` (`SkinnedMeshComponent.SkeletalMesh` _actor_hair_acc2_rabbitband) :`HairAcc2M` (`MeshComponent.GetMaterials` _actor_hair_acc2_rabbitband)))

(fn `UserConstructionScript`
  (`SkinnedMeshComponent.SetLeaderPoseComponent` (`self.actor_nose`) (`self.actor_body`) false)
  (`SkinnedMeshComponent.SetLeaderPoseComponent` (`self.actor_hair`) (`self.actor_body`) false)
  (`SkinnedMeshComponent.SetLeaderPoseComponent` (`self.actor_wholeclothes`) (`self.actor_body`) false)
  (`SkinnedMeshComponent.SetLeaderPoseComponent` (`self.actor_glasses`) (`self.actor_body`) false)
  (`SkinnedMeshComponent.SetLeaderPoseComponent` (`self.actor_hat`) (`self.actor_body`) false)
  (`SkinnedMeshComponent.SetLeaderPoseComponent` (`self.actor_bag`) (`self.actor_body`) false)
  (`SkinnedMeshComponent.SetLeaderPoseComponent` (`self.actor_watch`) (`self.actor_body`) false)
  (`SkinnedMeshComponent.SetLeaderPoseComponent` (`self.actor_upperclothes`) (`self.actor_body`) false)
  (`SkinnedMeshComponent.SetLeaderPoseComponent` (`self.actor_underclothes`) (`self.actor_body`) false)
  (`SkinnedMeshComponent.SetLeaderPoseComponent` (`self.actor_foot_left`) (`self.actor_body`) false)
  (`SkinnedMeshComponent.SetLeaderPoseComponent` (`self.actor_foot_right`) (`self.actor_body`) false)
  (`SkinnedMeshComponent.SetLeaderPoseComponent` (`self.actor_hathair`) (`self.actor_body`) false)
  (`SkinnedMeshComponent.SetLeaderPoseComponent` (`self.actor_hair_acc1_ribborn`) (`self.actor_body`) false)
  (`SkinnedMeshComponent.SetLeaderPoseComponent` (`self.actor_hair_acc2_rabbitband`) (`self.actor_body`) false))