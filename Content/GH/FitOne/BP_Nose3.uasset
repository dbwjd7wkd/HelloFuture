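; BP_Nose3 is a clickable character-customization item that toggles its own skeletal mesh on or off for a FitCategory through the FitOneController.
; It caches the FitOneController from player 0 on BeginPlay.
; Box clicks alternate via FlipFlop between sending the category with mesh, first material and true state, and sending only the category.
; Hover and equip debug prints refer to a jacket, despite the nose name.
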(event `self.ReceiveBeginPlay`
  (bind _asfit_one_controller (cast `/Game/GH/FitOne/FitOneController` (`GameplayStatics.GetPlayerController` 0)))
  (set `self.FitOneController` _asfit_one_controller))

(event `self.Box.OnBeginCursorOver`
  (params (TouchedComponent :type "PrimitiveComponent Object Reference"))
  (`KismetSystemLibrary.PrintString` "hovered on jacket"))

(event `self.Box.OnClicked`
  (params (TouchedComponent :type "PrimitiveComponent Object Reference") (ButtonPressed :type "Key Structure"))
  (bind _skeletalmesh (`self.SkeletalMesh`))
  (bind _fitonecontroller (`self.FitOneController`))
  (bind _fitcategory (`self.FitCategory`))
  (`/Engine/EditorBlueprintResources/StandardMacros.FlipFlop`
    (:`A`
      (`KismetSystemLibrary.PrintString` "clicked a jacket")
      (`/Game/GH/FitOne/FitOneController.CTR_FitOne_Change` _fitonecontroller _fitcategory (`|GetArrayItem` (`MeshComponent.GetMaterials` _skeletalmesh)) (`SkinnedMeshComponent.SkeletalMesh` _skeletalmesh) true))
    (:`B`
      (`/Game/GH/FitOne/FitOneController.CTR_FitOne_Change` _fitonecontroller _fitcategory null null false))))

(fn `UserConstructionScript`)