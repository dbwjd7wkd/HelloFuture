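; Clickable fitting item that applies its skeletal mesh and materials to its FitCategory through FitOneController.
; BeginPlay caches the controller and flags meshes with more than one material, selecting the multi- or single-material change call.
; On a box click, it compares its object name to the category's last-clicked item from ABP_LastClicked.
; A match calls RemoveWhenDoubleClicked once per InitialSettings entry; otherwise the item is applied.
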(event `self.ReceiveBeginPlay`
  (bind _asfit_one_controller (cast `/Game/GH/FitOne/FitOneController` (`GameplayStatics.GetPlayerController` 0)))
  (set `self.FitOneController` _asfit_one_controller)
  (if (> (`KismetArrayLibrary.Array_Length` (`MeshComponent.GetMaterials` (`self.SkeletalMesh`))) 1)
    (set `self.isMulti` true)))

(event `self.Box.OnBeginCursorOver`
  (params (TouchedComponent :type "PrimitiveComponent Object Reference")))

(event `self.Box.OnClicked`
  (params (TouchedComponent :type "PrimitiveComponent Object Reference") (ButtonPressed :type "Key Structure"))
  (bind _skeletalmesh (`self.SkeletalMesh`))
  (bind _fitcategory (`self.FitCategory`))
  (bind _fitonecontroller (`self.FitOneController`))
  (bind _returnvalue (`MeshComponent.GetMaterials` _skeletalmesh))
  (bind _skeletalmesh_2 (`SkinnedMeshComponent.SkeletalMesh` _skeletalmesh))
  (bind _returnvalue_2 (`GameplayStatics.GetActorOfClass` "/Game/GH/FitOne/ABP_LastClicked.ABP_LastClicked_C"))
  (bind _returnvalue_3 (`GH_LastClickedTMap.GetLastClickedItem` _returnvalue_2 (`|GetEnumeratorNameAsString` (`self.FitCategory`))))
  (if (`KismetStringLibrary.EqualEqual_StrStr` _returnvalue_3 (`KismetSystemLibrary.GetObjectName` self))
    (for _ (`self.initialSettings`)
      (`/Game/GH/FitOne/FitOneController.RemoveWhenDoubleClicked` (`self.FitOneController`) (`self.FitCategory`) (`self.isMulti`)))
    (elif (`self.isMulti`)
      (`/Game/GH/FitOne/FitOneController.CTR_FitOneChangeMultiMat` _fitonecontroller _fitcategory _returnvalue _skeletalmesh_2 false)
      (else
        (`/Game/GH/FitOne/FitOneController.CTR_FitOne_Change` _fitonecontroller _fitcategory (`|GetArrayItem` _returnvalue) _skeletalmesh_2 true)))))

(fn `UserConstructionScript`)