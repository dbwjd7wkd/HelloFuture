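; BP_HairStyle2 is a clickable fitting part, named for a hairstyle, that applies or removes its look through the FitOneController cached at BeginPlay.
; Clicks on its Box alternate via FlipFlop between applying and reverting.
; Applying sends FitCategory with its own SkeletalMesh and materials, using a separate controller call for multi-material meshes.
; Reverting sends only the category, which the author notes falls back to the default.
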(event `self.ReceiveBeginPlay`
  (bind _asfit_one_controller (cast `/Game/GH/FitOne/FitOneController` (`GameplayStatics.GetPlayerController` 0)))
  (set `self.FitOneController` _asfit_one_controller))

(event `self.Box.OnBeginCursorOver`
  (params (TouchedComponent :type "PrimitiveComponent Object Reference")))

(event `self.Box.OnClicked`
  (params (TouchedComponent :type "PrimitiveComponent Object Reference") (ButtonPressed :type "Key Structure"))
  (bind _skeletalmesh (`self.SkeletalMesh`))
  (bind _fitonecontroller (`self.FitOneController`))
  (bind _fitcategory (`self.FitCategory`))
  (bind _returnvalue (`MeshComponent.GetMaterials` _skeletalmesh))
  (bind _skeletalmesh_2 (`SkinnedMeshComponent.SkeletalMesh` _skeletalmesh))
  (`/Engine/EditorBlueprintResources/StandardMacros.FlipFlop`
    (:`A`
      (if (> (`KismetArrayLibrary.Array_Length` _returnvalue) 1)
        ;[1 1 1] material 여러개일때
        (`/Game/GH/FitOne/FitOneController.CTR_FitOneChangeMultiMat` _fitonecontroller _fitcategory _returnvalue _skeletalmesh_2 false)
        (else
          (`/Game/GH/FitOne/FitOneController.CTR_FitOne_Change` _fitonecontroller _fitcategory (`|GetArrayItem` _returnvalue) _skeletalmesh_2 true))))
    (:`B`
      ;[1 1 1] 안받으면 자동으로 기본으로 들어가도록  처리
      (`/Game/GH/FitOne/FitOneController.CTR_FitOne_Change` _fitonecontroller _fitcategory null null false))))

(fn `UserConstructionScript`)