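; BP_Nose1 is a clickable nose part in the FitOne part-fitting feature.
; On BeginPlay it caches the first player controller as a FitOneController.
; Clicks on its Box alternate through a FlipFlop, calling CTRFitOneChange on that controller with the part's FitCategory.
; The first click sends the part's own skeletal mesh and first material with State true; the next sends the hardcoded Nose_01 and PhongE32, leaving State at its default.
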(event `self.ReceiveBeginPlay`
  (bind _asfit_one_controller (cast `/Game/GH/FitOne/FitOneController` (`GameplayStatics.GetPlayerController` 0)))
  (set `self.FitOneController` _asfit_one_controller))

(event `self.Box.OnBeginCursorOver`
  (params (TouchedComponent :type "PrimitiveComponent Object Reference")))

(event `self.Box.OnClicked`
  (params (TouchedComponent :type "PrimitiveComponent Object Reference") (ButtonPressed :type "Key Structure"))
  (bind _skeletalmesh (`self.SkeletalMesh`))
  (bind _fitonecontroller (`self.FitOneController`))
  (bind _fitcategory (`self.FitCategory`))
  (`/Engine/EditorBlueprintResources/StandardMacros.FlipFlop`
    (:`A`
      (`/Game/GH/FitOne/FitOneController.CTR_FitOne_Change` _fitonecontroller _fitcategory (`|GetArrayItem` (`MeshComponent.GetMaterials` _skeletalmesh)) (`SkinnedMeshComponent.SkeletalMesh` _skeletalmesh) true ""))
    (:`B`
      ;[1 1 1] 안받으면 자동으로 기본으로 들어가도록  처리
      (`/Game/GH/FitOne/FitOneController.CTR_FitOne_Change` _fitonecontroller _fitcategory "/Game/Assets/Unreal_Export_Test/Nose/phongE32.phongE32" "/Game/Assets/Unreal_Export_Test/Nose/nose_01.nose_01" false ""))))

(fn `UserConstructionScript`)