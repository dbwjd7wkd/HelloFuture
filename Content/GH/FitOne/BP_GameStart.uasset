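; Clickable box that exits the FitOne customization level and returns the player to the map they came from.
; On click it calls SaveCustom on FitOneController and copies SavedCustomParts from the game instance.
; It then reads PreLevelName from the player character, falls back to HouseMap when that is "None", and opens the level after a short delay.
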(event `self.Box.OnClicked`
  (params (TouchedComponent :type "PrimitiveComponent Object Reference") (ButtonPressed :type "Key Structure"))
  ;[1 1 1] 나갈 때-게임인스턴스에 정보 저장하고
  (bind _asfit_one_controller (cast `/Game/GH/FitOne/FitOneController` (`GameplayStatics.GetPlayerController` 0)))
  (`/Game/GH/FitOne/FitOneController.SaveCustom` _asfit_one_controller)
  (bind _asreal_char_game_instance (cast `/Game/Map/realCharGameInstance` (`GameplayStatics.GetGameInstance`)))
  (set `self.Saved Custom Parts` (`/Game/Map/realCharGameInstance.SavedCustomParts` _asreal_char_game_instance))
  ;[1 1 1] 저장했던 이전 맵 이름을 들고옴
  (bind _ashello_future_character (cast `HelloFutureCharacter` (`GameplayStatics.GetPlayerCharacter` 0)))
  (bind _prelevelname (`HelloFutureCharacter.preLevelName` _ashello_future_character))
  (if (== _prelevelname "None")
    (set `self.SavedPreLevelName` "HouseMap")
    (else
      (set `self.SavedPreLevelName` _prelevelname)))
  (`KismetSystemLibrary.Delay` 1.0)
  (`GameplayStatics.OpenLevel` (`self.SavedPreLevelName`)))

(event `self.Box.OnBeginCursorOver`
  (params (TouchedComponent :type "PrimitiveComponent Object Reference")))

(event `self.Box.OnComponentBeginOverlap`
  (params (OverlappedComponent :type "PrimitiveComponent Object Reference") (OtherActor :type "Actor Object Reference") (OtherComp :type "PrimitiveComponent Object Reference") (OtherBodyIndex :type Integer) (bFromSweep :type Boolean) (SweepResult :type "HitResult Structure (by ref)")))

(fn `UserConstructionScript`)