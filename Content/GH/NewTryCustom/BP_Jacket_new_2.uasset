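; Clickable jacket actor for character customization that toggles its garment through the custom character player controller.
; On BeginPlay it caches that controller, and hovering over its Box only prints a debug message.
; Box clicks alternate via FlipFlop: one sends the clothing category, skeletal mesh and first material to CTRChange with State true.
; The next sends only the category, leaving the other inputs at their defaults.
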(event `self.ReceiveBeginPlay`
  (bind _asnew_try_real_bp_custom_char_controller (cast `/Game/GH/NewTryCustom/newTryRealBP_CustomCharController` (`GameplayStatics.GetPlayerController` 0)))
  (set `self.NewTryRealBPCustomCharController` _asnew_try_real_bp_custom_char_controller))

(event `self.Box.OnBeginCursorOver`
  (params (TouchedComponent :type "PrimitiveComponent Object Reference"))
  (`KismetSystemLibrary.PrintString` "hovered on jacket"))

(event `self.Box.OnClicked`
  (params (TouchedComponent :type "PrimitiveComponent Object Reference") (ButtonPressed :type "Key Structure"))
  (bind _skeletalmesh (`self.SkeletalMesh`))
  (bind _clothescategoryofsm (`self.ClothesCategoryOfSM`))
  (bind _newtryrealbpcustomcharcontroller (`self.NewTryRealBPCustomCharController`))
  (`/Engine/EditorBlueprintResources/StandardMacros.FlipFlop`
    (:`A`
      (`KismetSystemLibrary.PrintString` "clicked a jacket")
      (`/Game/GH/NewTryCustom/newTryRealBP_CustomCharController.CTR_Change` _newtryrealbpcustomcharcontroller _clothescategoryofsm (`|GetArrayItem` (`MeshComponent.GetMaterials` _skeletalmesh)) (`SkinnedMeshComponent.SkeletalMesh` _skeletalmesh) true))
    (:`B`
      (`/Game/GH/NewTryCustom/newTryRealBP_CustomCharController.CTR_Change` _newtryrealbpcustomcharcontroller _clothescategoryofsm null null false))))

(fn `UserConstructionScript`)