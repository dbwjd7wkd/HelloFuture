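; Player controller for the character customisation screen, which opens the W_BuildChar widget in UI-only input with the mouse cursor shown.
; On BeginPlay it caches the CharGameInstance and finds the CustomCharacter actor in the level.
; Its events forward clothing, hair, accessory and part-update requests to that character.
; Saving tells the character to save its data, then after a short delay stores the saved parts in the game instance.
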(event `self.ReceiveBeginPlay`
  (bind _aschar_game_instance (cast `/Game/GH/Custom/CharGameInstance` (`GameplayStatics.GetGameInstance`))
    (:`then`
      (set `self.GameInstance` _aschar_game_instance)
      (`|ExecutionSequence`
        (:`then_0`
          (bind _returnvalue (`|CreateWidget` "/Game/GH/Custom/W_BuildChar.W_BuildChar_C"))
          (bind _output_get (set `self.CharBuildWidget` _returnvalue))
          (`UserWidget.AddToViewport` _output_get 0)
          (`WidgetBlueprintLibrary.SetInputMode_UIOnlyEx` self (`self.CharBuildWidget`))
          (set `self.bShowMouseCursor` true))
        (:`then_1`
          (bind _outactors (`GameplayStatics.GetAllActorsOfClass` "/Game/GH/Custom/CustomCharacter.CustomCharacter_C"))
          (for _array_element _outactors
            (set `self.CustomChar` _array_element)))))
    (:`CastFailed`
      (`KismetSystemLibrary.PrintString` "Failed"))))

(event `AddJacket`
  (params (State :type Boolean))
  (`/Game/GH/Custom/CustomCharacter.AddJacket` (`self.CustomChar`) State))

(event `AddPants`
  (params (State :type Boolean))
  (`/Game/GH/Custom/CustomCharacter.AddPants` (`self.CustomChar`) State))

(event `AddHairStyle1`
  (params (State :type Boolean))
  (`/Game/GH/Custom/CustomCharacter.AddHair` (`self.CustomChar`) State "/Game/GH/SCK_Casual01/Models/MESH_A_02.MESH_A_02"))

(event `AddHairStyle2`
  (params (State :type Boolean))
  (`/Game/GH/Custom/CustomCharacter.AddHair` (`self.CustomChar`) State "/Game/GH/SCK_Casual01/Models/MESH_A_03.MESH_A_03"))

(event `AddSunglasses`
  (params (State :type Boolean))
  (`/Game/GH/Custom/CustomCharacter.AddSunglasses` (`self.CustomChar`) State))

(event `AddBeard`
  (params (State :type Boolean))
  (`/Game/GH/Custom/CustomCharacter.AddBeard` (`self.CustomChar`) State))

(event `UpdateCharPart`
  (params (UpdatePart :type "/Game/GH/Custom/E_CurrentCharacterPart Enum" :default "NewEnumerator0"))
  (`/Game/GH/Custom/CustomCharacter.UpdateCharPart` (`self.CustomChar`) UpdatePart))

(event `SaveSelectedChar`
  (bind _customchar (`self.CustomChar`))
  (`/Game/GH/Custom/CustomCharacter.SaveCharData` _customchar)
  (`KismetSystemLibrary.Delay` 0.2)
  (bind _savedpartsdata (`/Game/GH/Custom/CustomCharacter.GetSavedParts` _customchar))
  (`/Game/GH/Custom/CharGameInstance.StoreSavedParts` (`self.GameInstance`) _savedpartsdata))

(fn `UserConstructionScript`)