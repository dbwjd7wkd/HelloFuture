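; BP_Video is a networked video player controller with playback, playlist, five-second seek and volume controls.
; Each control event passes through a Server-named event to a Client-named event that drives the media player or sound target.
; Play resumes when IsPause is set and otherwise opens the playlist.
; Both seek controls currently add five seconds, including the backward one, and all OnRep functions are empty.
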(event `self.ReceiveBeginPlay`)

(event `Play_Video`
  ;[1 1 1] 비디오 플레이
  (`self.VideoPlay_Server1` (`self.Media`) (`self.In Playlist`) (`self.Is Pause`)))

(event `Back_Video`
  ;[1 1 1] 비디오 이전영상
  (`self.VideoBack_Server1` (`self.Media`)))

(event `SoundUp_Video`
  ;[1 1 1] 볼륨업
  (`self.SoundUp_Server1` null (`self.Volume Multiplier Up`)))

(event `SoundDown_Video`
  ;[1 1 1] 볼륨다운
  (`self.SoundDown_Server1` null (`self.Volume Multiplier Down`)))

(event `SoundMute_Video`
  ;[1 1 1] 볼륨 뮤트
  (`self.SoundMute_Server1` null (`self.Volume Multiplier Mute`)))

(event `Next_Video`
  ;[1 1 1] 비디오 다음영상
  (`self.VideoNext_Server1` (`self.Media`)))

(event `PausePlay_Video`
  ;[1 1 1] 일시정지 후 재생
  (`self.VideoPausePlay_Server1` (`self.Media`)))

(event `Pause_Video`
  ;[1 1 1] 일시정지
  (`self.VideoPause_Server1` (`self.Media`)))

(event `VideoPlay_Server1`
  (params (Target :type "MediaPlayer Object Reference") (InPlaylist :type "MediaPlaylist Object Reference") (Condition :type Boolean))
  ;[1 1 1] 비디오 플레이
  (`self.VideoPlay_Client1` Target InPlaylist Condition))

(event `SoundMute_Server1`
  (params (Target :type "MediaPlayer Object Reference") (Volume :type "Float (double-precision)"))
  ;[1 1 1] 볼륨 뮤트
  (`self.SoundMute_Client1` Target Volume))

(event `VideoBack_Server1`
  (params (Target :type "MediaPlayer Object Reference"))
  ;[1 1 1] 비디오 이전영상
  (`self.VideoBack_Client1` Target))

(event `SoundUp_Server1`
  (params (Target :type "SynthComponent Object Reference") (VolumeMultiplier :type "Float (double-precision)"))
  ;[1 1 1] 볼륨업
  (`self.SoundUp_Client1` Target VolumeMultiplier))

(event `SoundDown_Server1`
  (params (Target :type "MediaPlayer Object Reference") (Volume :type "Float (double-precision)"))
  ;[1 1 1] 볼륨다운
  (`self.SoundDown_Client1` Target Volume))

(event `VideoPausePlay_Server1`
  (params (Target :type "MediaPlayer Object Reference"))
  ;[1 1 1] 일시정지 후 재생
  (`self.VideoPausePlay_Client1` Target))

(event `VideoPause_Server1`
  (params (Target :type "MediaPlayer Object Reference"))
  ;[1 1 1] 일시정지
  (`self.VideoPause_Client1` Target))

(event `VideoNext_Server1`
  (params (Target :type "MediaPlayer Object Reference"))
  ;[1 1 1] 비디오 다음영상
  (`self.VideoNext_Client1` Target))

(event `VideoPlay_Client1`
  (params (Target :type "MediaPlayer Object Reference") (InPlaylist :type "MediaPlaylist Object Reference") (Condition :type Boolean))
  ;[1 1 1] 비디오 플레이
  (if Condition
    (`MediaPlayer.PlayAndSeek` Target)
    (set `self.Is Pause` false)
    (else
      (`MediaPlayer.OpenPlaylist` Target InPlaylist))))

(event `SoundDown_Client1`
  (params (Target :type "MediaPlayer Object Reference") (Volume :type "Float (double-precision)"))
  ;[1 1 1] 볼륨다운
  (`MediaPlayer.SetNativeVolume` Target Volume))

(event `SoundMute_Client1`
  (params (Target :type "MediaPlayer Object Reference") (Volume :type "Float (double-precision)"))
  ;[1 1 1] 볼륨 뮤트
  (`MediaPlayer.SetNativeVolume` Target Volume))

(event `VideoPause_Client1`
  (params (Target :type "MediaPlayer Object Reference"))
  ;[1 1 1] 일시정지
  (`MediaPlayer.Pause` Target)
  (set `self.Is Pause` true))

(event `SoundUp_Client1`
  (params (Target :type "SynthComponent Object Reference") (VolumeMultiplier :type "Float (double-precision)"))
  ;[1 1 1] 볼륨업
  (`SynthComponent.SetVolumeMultiplier` Target VolumeMultiplier))

(event `VideoPausePlay_Client1`
  (params (Target :type "MediaPlayer Object Reference"))
  ;[1 1 1] 일시정지 후 재생
  (`MediaPlayer.PlayAndSeek` Target)
  (set `self.Is Pause` false))

(event `VideoBack_Client1`
  (params (Target :type "MediaPlayer Object Reference"))
  ;[1 1 1] 비디오 이전영상
  (`MediaPlayer.Previous` Target))

(event `VideoNext_Client1`
  (params (Target :type "MediaPlayer Object Reference"))
  ;[1 1 1] 비디오 다음영상
  (`MediaPlayer.Next` Target))

(event `5SecondsUp`
  ;[1 1 1] 5초 이후
  (`self.5SecondsUp_Server` (`self.Media`)))

(event `5SecondsDown`
  ;[1 1 1] 5초이전
  (`self.5SecondsDown_Server` (`self.Media`)))

(event `5SecondsUp_Server`
  (params (Target :type "MediaPlayer Object Reference"))
  ;[1 1 1] 5초 이후
  (`self.5SecondsUp_Client` Target))

(event `5SecondsDown_Server`
  (params (Target :type "MediaPlayer Object Reference"))
  ;[1 1 1] 5초이전
  (`self.5SecondsDown_Client` Target))

(event `5SecondsUp_Client`
  (params (Target :type "MediaPlayer Object Reference"))
  (bind (_returnvalue_days _returnvalue_hours _returnvalue_minutes _returnvalue_seconds) (`KismetMathLibrary.BreakTimespan` (`MediaPlayer.GetTime` Target)))
  ;[1 1 1] 5초 이후
  (`MediaPlayer.Seek` Target (`KismetMathLibrary.MakeTimespan` 0 0 0 (+ _returnvalue_seconds 5))))

(event `5SecondsDown_Client`
  (params (Target :type "MediaPlayer Object Reference"))
  (bind (_returnvalue_days _returnvalue_hours _returnvalue_minutes _returnvalue_seconds) (`KismetMathLibrary.BreakTimespan` (`MediaPlayer.GetTime` Target)))
  ;[1 1 1] 5초이전
  (`MediaPlayer.Seek` Target (`KismetMathLibrary.MakeTimespan` 0 0 0 (+ _returnvalue_seconds 5))))

(fn `OnRep_In Playlist`)

(fn `OnRep_Is Pause`)

(fn `OnRep_Media`)

(fn `OnRep_Media Source`)

(fn `OnRep_MediaSoundComp`)

(fn `OnRep_Target`)

(fn `OnRep_Target_0`)

(fn `OnRep_Volume Multiplier Down`)

(fn `OnRep_Volume Multiplier Mute`)

(fn `OnRep_Volume Multiplier Up`)

(fn `UserConstructionScript`)

(fn `VideoPlay_Client`
  (params (Target1 :type "MediaPlayer Object Reference") (MediaSource1 :type "MediaSource Object Reference")))